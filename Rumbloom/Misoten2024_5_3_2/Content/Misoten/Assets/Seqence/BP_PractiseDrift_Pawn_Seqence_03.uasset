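; BP_PractiseDrift_Pawn_Seqence_03 is a pawn, apparently for a drift-practice sequence, with a Human rider and a vehicle Mesh.
; Its DriftLeft event plays the same non-looping left-drift animation on both components.
; AKIRA, BeginPlay, Tick and the construction script are empty.
; Throttled decal spawning, Akira animations and particle spawn-rate resets remain as disconnected logic that never runs.
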(event Custom|DriftLeft
  (Utilities|FlowControl|Sequence
    (:then_0
      (Components|Animation|PlayAnimation (Variables|Default|GetHuman) "/Game/Misoten/Assets/Models/Proto_CharaAssets/Chara_Animation_WileyDrift/Anim_Bat_01_DriftLeft_Loop.Anim_Bat_01_DriftLeft_Loop" false))
    (:then_1
      (Components|Animation|PlayAnimation (Variables|Character|GetMesh) "/Game/Misoten/Assets/Models/Proto_CharaAssets/Chara_Animation_WileyDrift/Anim_Bat_01_DriftLeft_Loop.Anim_Bat_01_DriftLeft_Loop" false))))

(event Custom|AKIRA)

(event EventBeginPlay)

(event EventTick
  (params (DeltaSeconds :type Float%20%28single-precision%29)))

(fn ConstructionScript)