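; Actor Blueprint for a background building plane mesh that stays hidden until a stage of the drift practice is reached.
; BeginPlay hides the static mesh component.
; Each Tick casts the player controller to BP_PractiseDrift_PlayerCon and, when its SplineFlg equals 2, makes the mesh visible once through a DoOnce.
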(event EventBeginPlay
  (Rendering|SetVisibility (Variables|Debug|GetStaticMeshComponent) false false))

(event Collision|EventActorBeginOverlap
  (params (OtherActor :type Actor%20Object%20Reference)))

(event EventTick
  (params (DeltaSeconds :type Float%20%28single-precision%29))
  (bind _asbp_practise_drift_player_con (Utilities|Casting|CastToBP_PractiseDrift_PlayerCon (Game|GetPlayerController 0)))
  (if (== (Variables|/Game/Misoten/BP/BP_PractiseDrift_PlayerCon.BP_PractiseDrift_PlayerCon_C|GetSplineFlg _asbp_practise_drift_player_con) 2)
    (Utilities|FlowControl|DoOnce false
      (:Completed
        (Rendering|SetVisibility (Variables|Debug|GetStaticMeshComponent) true false)))))

(fn ConstructionScript)