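; Background building actor made of four static mesh parts (A to D) that stays hidden until a player progress flag is reached.
; BeginPlay hides all four meshes and disables actor collision.
; Tick polls SplineFlg on BP_PractiseDrift_PlayerCon, and when it equals 2 a DoOnce makes the meshes visible and re-enables collision.
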(event EventBeginPlay
  (Rendering|SetVisibility (Variables|Default|GetSM_Building_A_SM_Building_AF) false false)
  (Rendering|SetVisibility (Variables|Default|GetSM_Building_B_SM_Building_BE) false false)
  (Rendering|SetVisibility (Variables|Default|GetSM_Building_C_SM_Building_CF) false false)
  (Rendering|SetVisibility (Variables|Default|GetSM_Building_D_SM_Building_DE) false false)
  (Collision|SetActorEnableCollision false))

(event Collision|EventActorBeginOverlap
  (params (OtherActor :type Actor%20Object%20Reference)))

(event EventTick
  (params (DeltaSeconds :type Float%20%28single-precision%29))
  (bind _asbp_practise_drift_player_con (Utilities|Casting|CastToBP_PractiseDrift_PlayerCon (Game|GetPlayerController 0)))
  (if (== (Variables|/Game/Misoten/BP/BP_PractiseDrift_PlayerCon.BP_PractiseDrift_PlayerCon_C|GetSplineFlg _asbp_practise_drift_player_con) 2)
    (Utilities|FlowControl|DoOnce false
      (:Completed
        (Collision|SetActorEnableCollision true)
        (Rendering|SetVisibility (Variables|Default|GetSM_Building_A_SM_Building_AF) true false)
        (Rendering|SetVisibility (Variables|Default|GetSM_Building_B_SM_Building_BE) true false)
        (Rendering|SetVisibility (Variables|Default|GetSM_Building_C_SM_Building_CF) true false)
        (Rendering|SetVisibility (Variables|Default|GetSM_Building_D_SM_Building_DE) true false)))))

(fn ConstructionScript)