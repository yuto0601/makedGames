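; BP_DecalScratch_Piller is a background scratch decal actor, apparently for pillars, that varies its look at spawn.
; On BeginPlay it creates a dynamic material instance on its decal and sets a randomly chosen scratch texture from an array.
; Its sphere overlap detects BP_DecalScratch actors, then calls a collision duplication event and prints a debug message.
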(event OnComponentBeginOverlap(Sphere)
  (params (OverlappedComponent :type Primitive%20Component%20Object%20Reference) (OtherActor :type Actor%20Object%20Reference) (OtherComp :type Primitive%20Component%20Object%20Reference) (OtherBodyIndex :type Integer) (bFromSweep :type Boolean) (SweepResult :type Hit%20Result%20Structure%20%28by%20ref%29))
  (bind _asbp_decal_scratch (Utilities|Casting|CastToBP_DecalScratch OtherActor))
  (Default|CallCollisionDuplicationEvent)
  (Development|PrintString "重なっとる"))

(event EventBeginPlay
  (bind _returnvalue (Rendering|Material|CreateDynamicMaterialInstance (Variables|Default|GetDecal) :!class /Script/Engine.DecalComponent))
  (Rendering|Material|SetTextureParameterValue _returnvalue "ScratchTexture" (Utilities|Array|Get(acopy) (Variables|Default|GetTexture) (Math|Random|RandomInteger 5))))

(event EventTick
  (params (DeltaSeconds :type Float%20%28single-precision%29)))

(fn ConstructionScript)