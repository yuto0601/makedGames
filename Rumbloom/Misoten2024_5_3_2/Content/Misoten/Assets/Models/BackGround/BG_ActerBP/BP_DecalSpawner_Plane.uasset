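; Background actor that scatters scratch decals within its box volume when play begins.
; BeginPlay calls a DecalSpawn event that spawns 40 BP_DecalScratch actors at random points inside the Box component's bounds.
; Only X scale varies randomly between the Min and Max variables; as wired, Y always equals Min and Z always equals Max.
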(event Custom|DecalSpawn]
  (params (NewParam :type Integer))
  (bind _box (Variables|Default|GetBox))
  (bind _min (Variables|Default|GetMin))
  (bind _max (Variables|Default|GetMax))
  (for _index (range 1 NewParam)
    (Game|SpawnActorfromClass "/Game/Misoten/Assets/Models/BackGround/BG_ActerBP/BP_DecalScratch.BP_DecalScratch_C" (Math|Transform|MakeTransform (Math|Random|RandomPointinBoundingBox (Transformation|GetWorldLocation _box) (Variables|/Script/Engine.BoxComponent|GetBoxExtent _box)) (Math|Rotator|MakeRotator 0.0 0.0 0.0) (Math|Vector|MakeVector (Math|Random|RandomFloatinRange _min _max) (Math|Random|RandomFloatinRange _min _min) (Math|Random|RandomFloatinRange _max _max))) "Undefined" "OverrideRootScale" 0 0)))

(event EventBeginPlay
  (CallFunction|DecalSpawn] 40))

(event Collision|EventActorBeginOverlap
  (params (OtherActor :type Actor%20Object%20Reference)))

(event EventTick
  (params (DeltaSeconds :type Float%20%28single-precision%29)))

(fn ConstructionScript)