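; Background floor actor that scatters scratch decals over its surface when play begins.
; BeginPlay calls the DecalSpawn custom event, which loops to spawn BP_DecalScratch actors at random points inside the Box collision's bounds.
; Each decal gets a random yaw and random per-axis scale, so the wear pattern differs on every run.
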(event Custom|DecalSpawn
  (params (NewParam :type Integer))
  (bind _box (Variables|Default|GetBox))
  ;[1 1 1] Boxコリジョン内のランダム位置に傷デカールを生成
  (for _index (range 1 NewParam)
    (Game|SpawnActorfromClass "/Game/Misoten/Assets/Models/BackGround/BG_ActerBP/BP_DecalScratch.BP_DecalScratch_C" (Math|Transform|MakeTransform (Math|Random|RandomPointinBoundingBox (Transformation|GetWorldLocation _box) (Variables|/Script/Engine.BoxComponent|GetBoxExtent _box)) (Math|Rotator|MakeRotator 0.0 0.0 (Math|Random|RandomFloatinRange 0.0 7.2e+02)) (Math|Vector|MakeVector (Math|Random|RandomFloatinRange 1.0 2.5) (Math|Random|RandomFloatinRange 1.0 2.5) (Math|Random|RandomFloatinRange 1.0 2.5))) "Undefined" "OverrideRootScale" 0 0)))

(event EventBeginPlay
  ;[1 1 1] 傷デカールの生成/数指定（カスタムイベント）
  (CallFunction|DecalSpawn 80))

(event Collision|EventActorBeginOverlap
  (params (OtherActor :type Actor%20Object%20Reference)))

(event EventTick
  (params (DeltaSeconds :type Float%20%28single-precision%29)))

(fn ConstructionScript)