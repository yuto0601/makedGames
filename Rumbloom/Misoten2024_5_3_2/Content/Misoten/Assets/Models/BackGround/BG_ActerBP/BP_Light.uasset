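; BP_Light is a background light actor that animates a decal's size.
; On BeginPlay, a timeline drives the decal's uniform world scale, adding a small curve-based variation to a fixed base size.
; A random float and a SetNewTime call accompany playback, apparently to vary the timeline's phase per instance.
; A second timeline that would swing an Arrow component's pitch is left disconnected and never runs.
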(event EventBeginPlay
  (Utilities|FlowControl|Sequence
    (:then_0
      (bind _新規track_0 (Timeline|タイムライン_0 Play)
        (:Update
          (Transformation|SetWorldScale3D (Variables|Default|GetDecal) (Math|Vector|MakeVector (+ (* _新規track_0 0.1) 3.43) (+ (* _新規track_0 0.1) 3.43) (+ (* _新規track_0 0.1) 3.43))))))
    (:then_1
      (Timeline|タイムライン_0 SetNewTime))))

(event Collision|EventActorBeginOverlap
  (params (OtherActor :type Actor%20Object%20Reference)))

(event EventTick
  (params (DeltaSeconds :type Float%20%28single-precision%29)))

(fn ConstructionScript)