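; Background pillar actor that randomizes its concrete surface pattern and scatters scratch decals over itself at BeginPlay.
; It creates a dynamic material instance on the pillar mesh and randomizes three MoveUV scalar parameters, so each pillar's pattern differs.
; The DecalSpawn event then spawns scratch decal actors at random points inside DecalBox with random scale, using look-at rotations to aim them toward the pillar's root.
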(event Custom|DecalSpawn
  (params (NewParam :type Integer))
  (bind _decalbox (Variables|Default|GetDecalBox))
  (bind _defaultsceneroot (Variables|Default|GetDefaultSceneRoot))
  (bind _returnvalue (Transformation|GetWorldLocation _decalbox))
  (bind _returnvalue_2 (Transformation|GetWorldLocation _defaultsceneroot))
  (bind _boxextent (Variables|/Script/Engine.BoxComponent|GetBoxExtent _decalbox))
  (bind _returnvalue_3 (Math|Random|RandomPointinBoundingBox _returnvalue _boxextent))
  (bind _returnvalue_4 (Math|Rotator|FindLookatRotation (Math|Vector|MakeVector (.x _returnvalue_3) (.y _returnvalue_3) 0.0) (Math|Vector|MakeVector (.x _returnvalue_2) (.y _returnvalue_2) 0.0)))
  ;[1 1 1] Boxコリジョン内のランダム位置に傷デカールを生成
  (for _index (range 1 NewParam)
    (Game|SpawnActorfromClass "/Game/Misoten/Assets/Models/BackGround/BG_ActerBP/BP_DecalScratch_Piller.BP_DecalScratch_Piller_C" (Math|Transform|MakeTransform (Math|Vector|MakeVector (.x _returnvalue_3) (.y _returnvalue_3) (.z _returnvalue_3)) (Math|Rotator|MakeRotator (.roll _returnvalue_4) (.pitch _returnvalue_4) (.yaw _returnvalue_4)) (Math|Vector|MakeVector (Math|Random|RandomFloatinRange 0.5 1.0) (Math|Random|RandomFloatinRange 0.5 1.0) (Math|Random|RandomFloatinRange 0.5 1.0))) "Undefined" "OverrideRootScale" 0 0)))

(event EventBeginPlay
  (Utilities|FlowControl|Sequence
    (:then_0
      ;[1 1 1] 柱ごとの模様をランダムに生成
      (bind _returnvalue (Rendering|Material|CreateDynamicMaterialInstance (Variables|Default|GetSM_BG_Pillar) 0 "/Game/Misoten/Assets/Models/BackGround/BG_Material_Texture/MI_Concrete_01.MI_Concrete_01" "None" :!class /Script/Engine.PrimitiveComponent))
      (Rendering|Material|SetScalarParameterValue _returnvalue "MoveUV1" (Math|Random|RandomFloatinRange 0.0 1e+01) :!class /Script/Engine.MaterialInstanceDynamic)
      (Rendering|Material|SetScalarParameterValue _returnvalue "MoveUV2" (Math|Random|RandomFloatinRange 0.0 1e+01) :!class /Script/Engine.MaterialInstanceDynamic)
      (Rendering|Material|SetScalarParameterValue _returnvalue "MoveUV3" (Math|Random|RandomFloatinRange 0.0 1e+01) :!class /Script/Engine.MaterialInstanceDynamic))
    (:then_1
      ;[1 1 1] 傷デカールの生成/数指定（カスタムイベント）
      (CallFunction|DecalSpawn 30))))

(event Collision|EventActorBeginOverlap
  (params (OtherActor :type Actor%20Object%20Reference)))

(event EventTick
  (params (DeltaSeconds :type Float%20%28single-precision%29)))

(fn ConstructionScript)