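; Finish-area track mesh actor for the drift racer that randomly presents one of six speed-up floor pads, or none.
; Tick rerolls the pad when the controller's RandamFlg switches to 1, and an entry box updates the controller's object count to flag the last map.
; The active pad's box boosts a grounded player unless BP_BOSSChase's hit flags are set, using a data-table speed value.
; A timer starts the boost sound, which stops permanently once boss HP runs out.
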(event OnComponentBeginOverlap(Box2)
  (params (OverlappedComponent :type Primitive%20Component%20Object%20Reference) (OtherActor :type Actor%20Object%20Reference) (OtherComp :type Primitive%20Component%20Object%20Reference) (OtherBodyIndex :type Integer) (bFromSweep :type Boolean) (SweepResult :type Hit%20Result%20Structure%20%28by%20ref%29))
  ;[1 1 1] 加速床に当たった時の処理
  (Utilities|Casting|CastToBP_PractiseDrift_Pawn OtherActor)
  (if (== (Variables|Default|GetVsivleFlg) 2)
    (CallFunction|KasokuEvent)))

(event OnComponentBeginOverlap(Box)
  (params (OverlappedComponent :type Primitive%20Component%20Object%20Reference) (OtherActor :type Actor%20Object%20Reference) (OtherComp :type Primitive%20Component%20Object%20Reference) (OtherBodyIndex :type Integer) (bFromSweep :type Boolean) (SweepResult :type Hit%20Result%20Structure%20%28by%20ref%29))
  ;[1 1 1] 生成ナンバー作成
  (Utilities|Casting|CastToBP_PractiseDrift_Pawn OtherActor)
  (Utilities|FlowControl|DoOnce false
    (:Completed
      (bind _output_get (Variables|Default|SetMYObjectNunber (+ (Variables|/Game/Misoten/BP/BP_PractiseDrift_PlayerCon.BP_PractiseDrift_PlayerCon_C|GetObjectNunber (Variables|Default|GetPlayerController)) (Variables|Default|GetMYObjectNunber))))
      (bind _output_get_2 (Variables|/Game/Misoten/BP/BP_PractiseDrift_PlayerCon.BP_PractiseDrift_PlayerCon_C|SetObjectNunber (Variables|Default|GetPlayerController) _output_get))
      (if (== _output_get_2 13)
        (Variables|/Game/Misoten/BP/BP_PractiseDrift_PlayerCon.BP_PractiseDrift_PlayerCon_C|SetlastMapflg (Variables|Default|GetPlayerController) true)))))

(event OnComponentBeginOverlap(Box1)
  (params (OverlappedComponent :type Primitive%20Component%20Object%20Reference) (OtherActor :type Actor%20Object%20Reference) (OtherComp :type Primitive%20Component%20Object%20Reference) (OtherBodyIndex :type Integer) (bFromSweep :type Boolean) (SweepResult :type Hit%20Result%20Structure%20%28by%20ref%29))
  ;[1 1 1] 加速床に当たった時の処理
  (Utilities|Casting|CastToBP_PractiseDrift_Pawn OtherActor)
  (if (== (Variables|Default|GetVsivleFlg) 1)
    (CallFunction|KasokuEvent)))

(event OnComponentBeginOverlap(Box3)
  (params (OverlappedComponent :type Primitive%20Component%20Object%20Reference) (OtherActor :type Actor%20Object%20Reference) (OtherComp :type Primitive%20Component%20Object%20Reference) (OtherBodyIndex :type Integer) (bFromSweep :type Boolean) (SweepResult :type Hit%20Result%20Structure%20%28by%20ref%29))
  ;[1 1 1] 加速床に当たった時の処理
  (Utilities|Casting|CastToBP_PractiseDrift_Pawn OtherActor)
  (if (== (Variables|Default|GetVsivleFlg) 3)
    (CallFunction|KasokuEvent)))

(event OnAudioPlayStateChanged(MS_NomalBoost_Cue)
  (params (PlayState :type EAudioComponentPlayState%20Enum :default "Playing"))
  (switch Utilities|FlowControl|Switch|SwitchonEAudioComponentPlayState PlayState
    (:Stopped
      (Variables|Default|SetKasokuHit false)
      (Utilities|FlowControl|DoOnce false) ; enters at Reset
    )))

(event OnComponentBeginOverlap(Box4)
  (params (OverlappedComponent :type Primitive%20Component%20Object%20Reference) (OtherActor :type Actor%20Object%20Reference) (OtherComp :type Primitive%20Component%20Object%20Reference) (OtherBodyIndex :type Integer) (bFromSweep :type Boolean) (SweepResult :type Hit%20Result%20Structure%20%28by%20ref%29))
  ;[1 1 1] 加速床に当たった時の処理
  (Utilities|Casting|CastToBP_PractiseDrift_Pawn OtherActor)
  (if (== (Variables|Default|GetVsivleFlg) 4)
    (CallFunction|KasokuEvent)))

(event OnComponentBeginOverlap(Box5)
  (params (OverlappedComponent :type Primitive%20Component%20Object%20Reference) (OtherActor :type Actor%20Object%20Reference) (OtherComp :type Primitive%20Component%20Object%20Reference) (OtherBodyIndex :type Integer) (bFromSweep :type Boolean) (SweepResult :type Hit%20Result%20Structure%20%28by%20ref%29))
  ;[1 1 1] 加速床に当たった時の処理
  (Utilities|Casting|CastToBP_PractiseDrift_Pawn OtherActor)
  (if (== (Variables|Default|GetVsivleFlg) 5)
    (CallFunction|KasokuEvent)))

(event OnComponentBeginOverlap(Box6)
  (params (OverlappedComponent :type Primitive%20Component%20Object%20Reference) (OtherActor :type Actor%20Object%20Reference) (OtherComp :type Primitive%20Component%20Object%20Reference) (OtherBodyIndex :type Integer) (bFromSweep :type Boolean) (SweepResult :type Hit%20Result%20Structure%20%28by%20ref%29))
  ;[1 1 1] 加速床に当たった時の処理
  (Utilities|Casting|CastToBP_PractiseDrift_Pawn OtherActor)
  (if (== (Variables|Default|GetVsivleFlg) 6)
    (CallFunction|KasokuEvent)))

(event Custom|Playsound
  (if (Variables|Default|GetKasokuHit)
    (Utilities|FlowControl|DoOnce false
      (:Completed
        (bind _returnvalue (Actor|GetActorOfClass "/Game/Misoten/BP/Misoten_Enemy/Enemy/Boss/BP_BOSSChase.BP_BOSSChase_C"))
        (if (<= (Variables|/Game/Misoten/BP/Misoten_Enemy/Enemy/Boss/BP_BOSSChase.BP_BOSSChase_C|GetHP _returnvalue) 0.0)
          (Audio|Components|Audio|Stop (Variables|Default|GetMS_NomalBoost_Cue))
          (Variables|Default|SetKasokuHit false)
          (Variables|Default|SetSoundStopFlg true)
          (else
            (Audio|Components|Audio|Play (Variables|Default|GetMS_NomalBoost_Cue) 0.0)))))))

(event Custom|kasokuEvent
  (bind _returnvalue (Actor|GetActorOfClass "/Game/Misoten/BP/Misoten_Enemy/Enemy/Boss/BP_BOSSChase.BP_BOSSChase_C"))
  (if (not (Variables|/Game/Misoten/BP/Misoten_Enemy/Enemy/Boss/BP_BOSSChase.BP_BOSSChase_C|GetHitFlg _returnvalue))
    (if (not (Variables|/Game/Misoten/BP/Misoten_Enemy/Enemy/Boss/BP_BOSSChase.BP_BOSSChase_C|GetHit2Flg _returnvalue))
      (bind _asbp_practise_drift_pawn (Utilities|Casting|CastToBP_PractiseDrift_Pawn (Game|Player|GetPlayerPawn 0)))
      (bind _asbp_practise_drift_player_con (Utilities|Casting|CastToBP_PractiseDrift_PlayerCon (Game|GetPlayerController 0)))
      (if (Variables|/Game/Misoten/BP/BP_PractiseDrift_Pawn.BP_PractiseDrift_Pawn_C|GetIsGround _asbp_practise_drift_pawn)
        (Variables|Default|SetKasokuHit true)
        (Default|SpeedUpEvent _asbp_practise_drift_player_con (Variables|Default|GetBegineSpeedUpValue))))))

(event Collision|EventActorBeginOverlap
  (params (OtherActor :type Actor%20Object%20Reference)))

(event EventTick
  (params (DeltaSeconds :type Float%20%28single-precision%29))
  (Utilities|FlowControl|Sequence
    (:then_0
      (bind _asbp_practise_drift_player_con (Utilities|Casting|CastToBP_PractiseDrift_PlayerCon (Game|GetPlayerController 0)))
      (bind _output_get (Variables|Default|SetPlayerController _asbp_practise_drift_player_con))
      (if (!= (Variables|/Game/Misoten/BP/BP_PractiseDrift_PlayerCon.BP_PractiseDrift_PlayerCon_C|GetRandamFlg _output_get) (Variables|Default|GetKakoRandFlg))
        (if (== (Variables|/Game/Misoten/BP/BP_PractiseDrift_PlayerCon.BP_PractiseDrift_PlayerCon_C|GetRandamFlg _output_get) 1)
          (Variables|Default|SetKakoRandFlg (Variables|/Game/Misoten/BP/BP_PractiseDrift_PlayerCon.BP_PractiseDrift_PlayerCon_C|GetRandamFlg (Variables|Default|GetPlayerController)))
          (if (Variables|/Game/Misoten/BP/BP_PractiseDrift_PlayerCon.BP_PractiseDrift_PlayerCon_C|GetlastMapflg (Variables|Default|GetPlayerController))
            (if (< (Variables|/Game/Misoten/BP/BP_PractiseDrift_PlayerCon.BP_PractiseDrift_PlayerCon_C|GetCountHitFlg (Variables|Default|GetPlayerController)) 1)
              (Variables|Default|SetVsivleFlg (Math|Random|RandomIntegerinRange 0 6))
              (Variables|/Game/Misoten/BP/BP_PractiseDrift_PlayerCon.BP_PractiseDrift_PlayerCon_C|SetCountHitFlg (Variables|Default|GetPlayerController) (+ (Variables|/Game/Misoten/BP/BP_PractiseDrift_PlayerCon.BP_PractiseDrift_PlayerCon_C|GetCountHitFlg (Variables|Default|GetPlayerController)) 1))
              (else
                (Variables|Default|SetVsivleFlg (Math|Random|RandomIntegerinRange 1 6))
                (Variables|/Game/Misoten/BP/BP_PractiseDrift_PlayerCon.BP_PractiseDrift_PlayerCon_C|SetCountHitFlg (Variables|Default|GetPlayerController) 0)))
            (else
              (Variables|Default|SetVsivleFlg (Math|Random|RandomIntegerinRange 0 6))))
          ;[1 1 1] 加速装置を表示させるか判断する処理
          (switch int (Variables|Default|GetVsivleFlg)
            (:0
              (Rendering|SetVisibility (Variables|Default|GetSM_TestFloor) false true))
            (:1
              (Rendering|SetVisibility (Variables|Default|GetSM_TestFloor) true true)
              (Rendering|SetVisibility (Variables|Default|GetSM_TestFloor1) false false)
              (Rendering|SetVisibility (Variables|Default|GetSM_TestFloor2) false false)
              (Rendering|SetVisibility (Variables|Default|GetSM_TestFloor3) false false)
              (Rendering|SetVisibility (Variables|Default|GetSM_TestFloor4) false false)
              (Rendering|SetVisibility (Variables|Default|GetSM_TestFloor5) false false))
            (:2
              (Rendering|SetVisibility (Variables|Default|GetSM_TestFloor1) true true)
              (Rendering|SetVisibility (Variables|Default|GetSM_TestFloor) false false)
              (Rendering|SetVisibility (Variables|Default|GetSM_TestFloor2) false false)
              (Rendering|SetVisibility (Variables|Default|GetSM_TestFloor3) false false)
              (Rendering|SetVisibility (Variables|Default|GetSM_TestFloor4) false false)
              (Rendering|SetVisibility (Variables|Default|GetSM_TestFloor5) false false))
            (:3
              (Rendering|SetVisibility (Variables|Default|GetSM_TestFloor2) true true)
              (Rendering|SetVisibility (Variables|Default|GetSM_TestFloor) false false)
              (Rendering|SetVisibility (Variables|Default|GetSM_TestFloor1) false false)
              (Rendering|SetVisibility (Variables|Default|GetSM_TestFloor5) false false)
              (Rendering|SetVisibility (Variables|Default|GetSM_TestFloor3) false false)
              (Rendering|SetVisibility (Variables|Default|GetSM_TestFloor4) false false))
            (:4
              (Rendering|SetVisibility (Variables|Default|GetSM_TestFloor3) true true)
              (Rendering|SetVisibility (Variables|Default|GetSM_TestFloor) false false)
              (Rendering|SetVisibility (Variables|Default|GetSM_TestFloor1) false false)
              (Rendering|SetVisibility (Variables|Default|GetSM_TestFloor2) false false)
              (Rendering|SetVisibility (Variables|Default|GetSM_TestFloor4) false false)
              (Rendering|SetVisibility (Variables|Default|GetSM_TestFloor5) false false))
            (:5
              (Rendering|SetVisibility (Variables|Default|GetSM_TestFloor4) true true)
              (Rendering|SetVisibility (Variables|Default|GetSM_TestFloor) false false)
              (Rendering|SetVisibility (Variables|Default|GetSM_TestFloor1) false false)
              (Rendering|SetVisibility (Variables|Default|GetSM_TestFloor2) false false)
              (Rendering|SetVisibility (Variables|Default|GetSM_TestFloor3) false false)
              (Rendering|SetVisibility (Variables|Default|GetSM_TestFloor5) false false))
            (:6
              (Rendering|SetVisibility (Variables|Default|GetSM_TestFloor5) true true)
              (Rendering|SetVisibility (Variables|Default|GetSM_TestFloor) false false)
              (Rendering|SetVisibility (Variables|Default|GetSM_TestFloor1) false false)
              (Rendering|SetVisibility (Variables|Default|GetSM_TestFloor2) false false)
              (Rendering|SetVisibility (Variables|Default|GetSM_TestFloor3) false false)
              (Rendering|SetVisibility (Variables|Default|GetSM_TestFloor4) false false)))
          (else
            (Variables|Default|SetKakoRandFlg (Variables|/Game/Misoten/BP/BP_PractiseDrift_PlayerCon.BP_PractiseDrift_PlayerCon_C|GetRandamFlg (Variables|Default|GetPlayerController)))))))
    (:then_1
      (if (Variables|Default|GetSoundStopFlg)
        (Audio|Components|Audio|Stop (Variables|Default|GetMS_NomalBoost_Cue))))))

(event EventBeginPlay
  (bind _asbp_practise_drift_player_con (Utilities|Casting|CastToBP_PractiseDrift_PlayerCon (Game|GetPlayerController 0)))
  (Variables|Default|SetPlayerController _asbp_practise_drift_player_con)
  (Rendering|SetVisibility (Variables|Default|GetSM_TestFloor) false true)
  (Utilities|Time|SetTimerbyEvent (delegate Custom|Playsound) 0.1 true))

(fn ConstructionScript
  (bind _returnvalue (Utilities|GetDataTableRow "/Game/Misoten/BP/DataTable/GimmickStatusDataTable.GimmickStatusDataTable" "SpeedUpStand")
    (:then
      (Variables|Default|SetBegineSpeedUpValue (.BeginSpeedUpValue (Utilities|Struct|BreakGimmickStatusStruct _returnvalue)))
      (Variables|Default|SetEndSpeedUpValue (.EndSpeedUpValue (Utilities|Struct|BreakGimmickStatusStruct _returnvalue))))))