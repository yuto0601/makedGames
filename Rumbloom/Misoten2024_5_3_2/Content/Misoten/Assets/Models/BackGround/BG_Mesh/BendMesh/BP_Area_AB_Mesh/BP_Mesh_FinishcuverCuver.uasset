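; BP_Mesh_FinishcuverCuver is a background stage mesh actor that stays hidden and non-collidable until the player reaches a certain spline state.
; BeginPlay hides its stage mesh and disables actor collision.
; Tick casts the first player controller to BP_PractiseDrift_PlayerCon and polls its SplineFlg.
; When the flag equals 2, a DoOnce shows the mesh and enables collision a single time.
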(event EventBeginPlay
  (Rendering|SetVisibility (Variables|Default|GetSM_BG_Mesh_Field_Stage1_3) false false)
  (Collision|SetActorEnableCollision false))

(event Collision|EventActorBeginOverlap
  (params (OtherActor :type Actor%20Object%20Reference)))

(event EventTick
  (params (DeltaSeconds :type Float%20%28single-precision%29))
  (bind _asbp_practise_drift_player_con (Utilities|Casting|CastToBP_PractiseDrift_PlayerCon (Game|GetPlayerController 0)))
  (if (== (Variables|/Game/Misoten/BP/BP_PractiseDrift_PlayerCon.BP_PractiseDrift_PlayerCon_C|GetSplineFlg _asbp_practise_drift_player_con) 2)
    (Utilities|FlowControl|DoOnce false
      (:Completed
        (Collision|SetActorEnableCollision true)
        (Rendering|SetVisibility (Variables|Default|GetSM_BG_Mesh_Field_Stage1_3) true false)))))

(fn ConstructionScript)