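; Trigger volume actor that clears the streamed sub-levels of SplineMeshNarrowStage when the practice drift pawn enters its box.
; On box overlap by a BP_PractiseDrift_Pawn, it hides each of the hard-coded Area levels (AB, C, DE, F, G) and requests a non-blocking unload of each.
; It only unloads and never loads a level; BeginPlay, Tick and the construction script are empty.
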(event OnComponentBeginOverlap(Box)
  (params (OverlappedComponent :type Primitive%20Component%20Object%20Reference) (OtherActor :type Actor%20Object%20Reference) (OtherComp :type Primitive%20Component%20Object%20Reference) (OtherBodyIndex :type Integer) (bFromSweep :type Boolean) (SweepResult :type Hit%20Result%20Structure%20%28by%20ref%29))
  (Utilities|Casting|CastToBP_PractiseDrift_Pawn OtherActor)
  (Variables|/Script/Engine.LevelStreaming|SetbShouldBeVisible (Class|GameplayStatics|GetStreamingLevel "SplineMeshNarrowStage_Area_AB") false)
  (Class|GameplayStatics|UnloadStreamLevelbySoftObjectPtr "/Game/Misoten/Level/Stage1/SplineMeshNarrowStage_Area_AB.SplineMeshNarrowStage_Area_AB" false)
  (Variables|/Script/Engine.LevelStreaming|SetbShouldBeVisible (Class|GameplayStatics|GetStreamingLevel "SplineMeshNarrowStage_Area_C") false)
  (Class|GameplayStatics|UnloadStreamLevelbySoftObjectPtr "/Game/Misoten/Level/Stage1/SplineMeshNarrowStage_Area_C.SplineMeshNarrowStage_Area_C" false)
  (Variables|/Script/Engine.LevelStreaming|SetbShouldBeVisible (Class|GameplayStatics|GetStreamingLevel "SplineMeshNarrowStage_Area_DE") false)
  (Class|GameplayStatics|UnloadStreamLevelbySoftObjectPtr "/Game/Misoten/Level/Stage1/SplineMeshNarrowStage_Area_DE.SplineMeshNarrowStage_Area_DE" false)
  (Variables|/Script/Engine.LevelStreaming|SetbShouldBeVisible (Class|GameplayStatics|GetStreamingLevel "SplineMeshNarrowStage_Area_F") false)
  (Class|GameplayStatics|UnloadStreamLevelbySoftObjectPtr "/Game/Misoten/Level/Stage1/SplineMeshNarrowStage_Area_F.SplineMeshNarrowStage_Area_F" false)
  (Variables|/Script/Engine.LevelStreaming|SetbShouldBeVisible (Class|GameplayStatics|GetStreamingLevel "SplineMeshNarrowStage_Area_G") false)
  (Class|GameplayStatics|UnloadStreamLevelbySoftObjectPtr "/Game/Misoten/Level/SplineMeshNarrowStage_Area_G.SplineMeshNarrowStage_Area_G" false))

(event EventBeginPlay)

(event Collision|EventActorBeginOverlap
  (params (OtherActor :type Actor%20Object%20Reference)))

(event EventTick
  (params (DeltaSeconds :type Float%20%28single-precision%29)))

(fn ConstructionScript)