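; BP_BGM is the in-game background music controller, switching between the main track and the boss track.
; BeginPlay stops both audio cues, and Tick watches BGMFlg against its cached previous value.
; On a change, value 1 plays the main cue and stops the boss cue, while 2 does the reverse through custom stop events.
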(event Custom|BGMStopEvent
  (Audio|Components|Audio|Stop (Variables|Default|GetMS_Main_ver3_Cue)))

(event Custom|BOSSBGMStopEvent
  (Audio|Components|Audio|Stop (Variables|Default|GetMS_MainBossBGM_Cue)))

(event EventTick
  (params (DeltaSeconds :type Float%20%28single-precision%29))
  (if (!= (Variables|Default|GetBGMFlg) (Variables|Default|GetkakoBGMFlg))
    (Variables|Default|SetkakoBGMFlg (Variables|Default|GetBGMFlg))
    (switch int (Variables|Default|GetBGMFlg)
      (:1
        (Audio|Components|Audio|Play (Variables|Default|GetMS_Main_ver3_Cue) 0.0)
        (CallFunction|BOSSBGMStopEvent))
      (:2
        (Audio|Components|Audio|Play (Variables|Default|GetMS_MainBossBGM_Cue) 0.0)
        (CallFunction|BGMStopEvent)))))

(event EventBeginPlay
  (Audio|Components|Audio|Stop (Variables|Default|GetMS_MainBossBGM_Cue))
  (Audio|Components|Audio|Stop (Variables|Default|GetMS_Main_ver3_Cue)))

(fn ConstructionScript)