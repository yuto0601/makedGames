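; Trigger volume that switches the drift game to its final spline when the player pawn enters it.
; On Box overlap by BP_PractiseDrift_Pawn, a DoOnce sets SplineFlg on the player controller to the final spline's index.
; Tick polls SplineFlg against a cached HikakuSpline; when it changes while RisetFlg is set, it clears that flag and re-arms the DoOnce.
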(event OnComponentBeginOverlap(Box)
  (params (OverlappedComponent :type Primitive%20Component%20Object%20Reference) (OtherActor :type Actor%20Object%20Reference) (OtherComp :type Primitive%20Component%20Object%20Reference) (OtherBodyIndex :type Integer) (bFromSweep :type Boolean) (SweepResult :type Hit%20Result%20Structure%20%28by%20ref%29))
  ;[1 1 1] 最後のスプラインに変える処理
  (Utilities|Casting|CastToBP_PractiseDrift_Pawn OtherActor)
  (Utilities|FlowControl|DoOnce false
    (:Completed
      (bind _asbp_practise_drift_player_con (Utilities|Casting|CastToBP_PractiseDrift_PlayerCon (Game|GetPlayerController 0)))
      (Variables|/Game/Misoten/BP/BP_PractiseDrift_PlayerCon.BP_PractiseDrift_PlayerCon_C|SetSplineFlg _asbp_practise_drift_player_con 2))))

(event EventBeginPlay)

(event Collision|EventActorBeginOverlap
  (params (OtherActor :type Actor%20Object%20Reference)))

(event EventTick
  (params (DeltaSeconds :type Float%20%28single-precision%29))
  ;[1 1 1] 最後のスプラインに変える処理
  (bind _asbp_practise_drift_player_con (Utilities|Casting|CastToBP_PractiseDrift_PlayerCon (Game|GetPlayerController 0)))
  (if (!= (Variables|Default|GetHikakuSpline) (Variables|/Game/Misoten/BP/BP_PractiseDrift_PlayerCon.BP_PractiseDrift_PlayerCon_C|GetSplineFlg _asbp_practise_drift_player_con))
    (Variables|Default|SetHikakuSpline (Variables|/Game/Misoten/BP/BP_PractiseDrift_PlayerCon.BP_PractiseDrift_PlayerCon_C|GetSplineFlg _asbp_practise_drift_player_con))
    (if (Variables|/Game/Misoten/BP/BP_PractiseDrift_PlayerCon.BP_PractiseDrift_PlayerCon_C|GetRisetFlg _asbp_practise_drift_player_con)
      (Variables|/Game/Misoten/BP/BP_PractiseDrift_PlayerCon.BP_PractiseDrift_PlayerCon_C|SetRisetFlg _asbp_practise_drift_player_con false)
      (Utilities|FlowControl|DoOnce false) ; enters at Reset
    )))

(fn ConstructionScript)