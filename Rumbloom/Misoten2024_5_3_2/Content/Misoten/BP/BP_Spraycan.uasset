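; Spray can actor for the drift practice mode that plays a spray sound and adds spray score when the player pawn overlaps it.
; Player controller pause events toggle its custom time dilation and a flag that blocks hits.
; A DoOnce, reset by a repeating two-second Delay on Tick, throttles scoring rather than consuming the can.
; The IsHit guard is only ever set false here, so it never blocks repeat hits.
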(event OnComponentBeginOverlap(splaycan)
  (params (OverlappedComponent :type Primitive%20Component%20Object%20Reference) (OtherActor :type Actor%20Object%20Reference) (OtherComp :type Primitive%20Component%20Object%20Reference) (OtherBodyIndex :type Integer) (bFromSweep :type Boolean) (SweepResult :type Hit%20Result%20Structure%20%28by%20ref%29))
  (if (not (Variables|Default|GetIsHit))
    (if (not (Variables|Default|GetIsPause))
      (bind _asbp_practise_drift_pawn (Utilities|Casting|CastToBP_PractiseDrift_Pawn OtherActor))
      (Variables|Default|SetIsHit false)
      (Utilities|FlowControl|DoOnce false
        (:Completed
          (Audio|PlaySoundatLocation "/Game/Misoten/BP/Audio/SE/MS_Spray_Cue.MS_Spray_Cue" (Transformation|GetActorLocation) "0, 0, 0" 0.6 1.0 0.0 0 0 0 0)
          (Default|AddScoreSpray (Variables|/Game/Misoten/BP/BP_PractiseDrift_Pawn.BP_PractiseDrift_Pawn_C|GetBP_PlayerState _asbp_practise_drift_pawn)))))))

(event Custom|SetCustomTimeDilationZero
  (Variables|Default|SetCustomTimeDilation 0.0)
  (Variables|Default|SetIsPause true))

(event Custom|SetCustomTimeDilationOne
  (Variables|Default|SetCustomTimeDilation 1.0)
  (Variables|Default|SetIsPause false))

(event EventBeginPlay
  (bind _asbp_practise_drift_player_con (Utilities|Casting|CastToBP_PractiseDrift_PlayerCon (Game|GetPlayerController 0)))
  (EventDispatchers|BindEventtoStartPause _asbp_practise_drift_player_con (delegate Custom|SetCustomTimeDilationZero))
  (EventDispatchers|BindEventtoStopPause _asbp_practise_drift_player_con (delegate Custom|SetCustomTimeDilationOne)))

(event Collision|EventActorBeginOverlap
  (params (OtherActor :type Actor%20Object%20Reference)))

(event EventTick
  (params (DeltaSeconds :type Float%20%28single-precision%29))
  (Utilities|FlowControl|Delay 2.0)
  (Utilities|FlowControl|DoOnce false) ; enters at Reset
)

(fn ConstructionScript)