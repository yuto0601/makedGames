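; Base crow enemy for the drift game, killed by the player's charge hits or by being encircled, awarding score for each.
; Charge hits damage table-driven HP and smash it along a camera-relative direction; Tick moves it, mirroring off walls with growing speed until a bounce or time limit.
; Enclosure sums signed angles to the player's spline points as a winding test.
; Deaths update the parent spawner and boss enemy count.
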(event OnComponentBeginOverlap(Sphere)
  (params (OverlappedComponent :type Primitive%20Component%20Object%20Reference) (OtherActor :type Actor%20Object%20Reference) (OtherComp :type Primitive%20Component%20Object%20Reference) (OtherBodyIndex :type Integer) (bFromSweep :type Boolean) (SweepResult :type Hit%20Result%20Structure%20%28by%20ref%29))
  (Utilities|Casting|CastToBP_PractiseDrift_Pawn OtherActor)
  (Utilities|FlowControl|DoOnce false
    (:Completed
      (Audio|PlaySoundatLocation "/Game/Misoten/BP/Audio/SE/MS_Surprised.MS_Surprised" (Transformation|GetActorLocation) "0, 0, 0" 0.15 1.0 0.0 0 0 0 0)
      (Transformation|SetActorRotation (Math|Rotator|FindLookatRotation (Transformation|GetActorLocation) (Transformation|GetActorLocation (Game|GetPlayerCharacter 0))))
      (Components|Activation|SetActive (Variables|Default|GetNS_Exc) true false)
      (Utilities|Time|SetTimerbyEvent (delegate Custom|NSDrop) 1.0))))

(event OnComponentBeginOverlap(Box)
  (params (OverlappedComponent :type Primitive%20Component%20Object%20Reference) (OtherActor :type Actor%20Object%20Reference) (OtherComp :type Primitive%20Component%20Object%20Reference) (OtherBodyIndex :type Integer) (bFromSweep :type Boolean) (SweepResult :type Hit%20Result%20Structure%20%28by%20ref%29))
  (bind _returnvalue (Game|GetPlayerCameraManager 0))
  (bind _as_bp_practise_drift_pawn (Variables|Default|GetAs%20BP%20Practise%20Drift%20Pawn))
  (bind _as_bp_practise_drift_player_con (Variables|Default|GetAs%20BP%20Practise%20Drift%20Player%20Con))
  (bind _normalspeed (Variables|Default|GetNormalSpeed))
  (bind _returnvalue_2 (Transformation|GetActorUpVector _returnvalue))
  (bind _returnvalue_3 (Transformation|GetActorRotation _returnvalue))
  (bind _returnvalue_4 (Transformation|GetActorForwardVector _returnvalue))
  (bind _returnvalue_5 (Transformation|GetActorRightVector _returnvalue))
  (bind _returnvalue_6 (* _normalspeed -1.0))
  (bind _nowspeed (Variables|/Game/Misoten/BP/BP_PractiseDrift_PlayerCon.BP_PractiseDrift_PlayerCon_C|GetNowSpeed _as_bp_practise_drift_player_con))
  (bind _returnvalue_7 (Math|Rotator|FindLookatRotation _returnvalue_4 _returnvalue_2))
  (bind _returnvalue_8 (Math|Rotator|FindLookatRotation _returnvalue_4 _returnvalue_5))
  (bind _returnvalue_9 (Math|Rotator|MakeRotator (.roll _returnvalue_3) (.pitch _returnvalue_3) (.yaw _returnvalue_3)))
  (bind _returnvalue_10 (* _nowspeed _returnvalue_6))
  (bind _returnvalue_11 (* _returnvalue_9 -1.0))
  (bind _returnvalue_12 (* _returnvalue_8 -1.0))
  (bind _returnvalue_13 (* _returnvalue_7 -1.0))
  (bind _returnvalue_14 (Math|Rotator|CombineRotators _returnvalue_11 _returnvalue_13))
  (bind _asbp_practise_drift_pawn (Utilities|Casting|CastToBP_PractiseDrift_Pawn OtherActor))
  (Default|CallHitEnemy _asbp_practise_drift_pawn)
  (bind _actor (Default|GetLockonTarget _asbp_practise_drift_pawn))
  (if (== _actor self)
    (Default|LockonRelease _asbp_practise_drift_pawn))
  (bind _isdeath (CallFunction|Damage (Variables|/Game/Misoten/BP/BP_PlayerState.BP_PlayerState_C|GetChargeAttackValue (Variables|/Game/Misoten/BP/BP_PractiseDrift_Pawn.BP_PractiseDrift_Pawn_C|GetBP_PlayerState (Variables|Default|GetAs%20BP%20Practise%20Drift%20Pawn)))))
  (CallFunction|Death false _isdeath)
  (Utilities|FlowControl|DoOnce false
    (:Completed
      (bind _returnvalue_15 (Niagara|SpawnSystematLocation "/Game/Misoten/Assets/EFF/EFF_Hit_Level_Medium/NS_Hit_Level_Medium.NS_Hit_Level_Medium" (Transformation|GetActorLocation)))
      (Rendering|SetRenderCustomDepth _returnvalue_15 false)
      (Audio|PlaySoundatLocation "/Game/Misoten/BP/Audio/SE/Enemy/MS_CrowRush_Cue.MS_CrowRush_Cue" (Transformation|GetActorLocation) "0, 0, 0" 0.6 1.0 0.0 0 0 0 0)
      (CallFunction|EnemyCountDown)
      (if (Variables|/Game/Misoten/BP/BP_PractiseDrift_Pawn.BP_PractiseDrift_Pawn_C|GetIsDriftRight _as_bp_practise_drift_pawn)
        (Default|CallSmashEnemy (Math|Rotator|CombineRotators _returnvalue_11 _returnvalue_12) _returnvalue_10)
        (elif (Variables|/Game/Misoten/BP/BP_PractiseDrift_Pawn.BP_PractiseDrift_Pawn_C|GetIsDriftLeft _as_bp_practise_drift_pawn)
          (Default|CallSmashEnemy (Math|Rotator|CombineRotators (* _returnvalue_11 -1.0) _returnvalue_12) _returnvalue_10)
          (elif (Variables|/Game/Misoten/BP/BP_PractiseDrift_PlayerCon.BP_PractiseDrift_PlayerCon_C|GetIsWiley (Variables|Default|GetAs%20BP%20Practise%20Drift%20Player%20Con))
            (Default|CallSmashEnemy _returnvalue_14 _returnvalue_10)
            (else
              (Default|CallSmashEnemy _returnvalue_14 _returnvalue_10)))))
      (Default|HitStop (Variables|Default|GetAs%20BP%20Practise%20Drift%20Pawn)))))

(event Custom|LookatTarget
  (params (TargetActor :type Actor%20Object%20Reference))
  (Transformation|SetActorRotation (Math|Rotator|FindLookatRotation (Transformation|GetActorLocation) (Transformation|GetActorLocation TargetActor))))

(event Custom|HitStage_Event
  (bind _returnvalue (Game|GetPlayerCameraManager 0))
  (bind _as_bp_practise_drift_pawn (Variables|Default|GetAs%20BP%20Practise%20Drift%20Pawn))
  (bind _as_bp_practise_drift_player_con (Variables|Default|GetAs%20BP%20Practise%20Drift%20Player%20Con))
  (bind _normalspeed (Variables|Default|GetNormalSpeed))
  (bind _returnvalue_2 (Transformation|GetActorUpVector _returnvalue))
  (bind _returnvalue_3 (Transformation|GetActorRotation _returnvalue))
  (bind _returnvalue_4 (Transformation|GetActorForwardVector _returnvalue))
  (bind _returnvalue_5 (Transformation|GetActorRightVector _returnvalue))
  (bind _returnvalue_6 (* _normalspeed -1.0))
  (bind _nowspeed (Variables|/Game/Misoten/BP/BP_PractiseDrift_PlayerCon.BP_PractiseDrift_PlayerCon_C|GetNowSpeed _as_bp_practise_drift_player_con))
  (bind _returnvalue_7 (Math|Rotator|FindLookatRotation _returnvalue_4 _returnvalue_2))
  (bind _returnvalue_8 (Math|Rotator|FindLookatRotation _returnvalue_4 _returnvalue_5))
  (bind _returnvalue_9 (Math|Rotator|MakeRotator (.roll _returnvalue_3) (.pitch _returnvalue_3) (.yaw _returnvalue_3)))
  (bind _returnvalue_10 (* _nowspeed _returnvalue_6))
  (bind _returnvalue_11 (* _returnvalue_9 -1.0))
  (bind _returnvalue_12 (* _returnvalue_8 -1.0))
  (bind _returnvalue_13 (* _returnvalue_7 -1.0))
  (bind _returnvalue_14 (Math|Rotator|CombineRotators _returnvalue_11 _returnvalue_13))
  (Utilities|FlowControl|DoOnce false) ; enters at Reset
)

(event Custom|EncloseCompulsionStop
  (Variables|Default|SetEnclosed false)
  (Components|Activation|SetActive (Variables|Default|GetChargeEFF) false false))

(event Custom|Reflection
  (params (TargetActor :type Actor%20Object%20Reference))
  (Transformation|SetActorRotation (* (Math|Rotator|FindLookatRotation (Transformation|GetActorLocation) (Transformation|GetActorLocation TargetActor)) -1.0)))

(event Custom|LookatVector
  (params (Rotator :type Rotator) (SmashSpeed :type Float%20%28double-precision%29))
  (Transformation|SetActorRotation Rotator))

(event Custom|SetCustomTimeDilationZero
  (Variables|Default|SetCustomTimeDilation 0.0))

(event Custom|SetCustomTimeDilationOne
  (Variables|Default|SetCustomTimeDilation 1.0))

(event Custom|EncloseJudgeEvent
  (params (SplineObject :type Spline%20Component%20Object%20Reference))
  (if (not (Variables|Default|GetEnclosed))
    (if (<= (Math|Vector|VectorLength (- (Transformation|GetActorLocation (Variables|Default|GetAs%20BP%20Practise%20Drift%20Pawn)) (Transformation|GetActorLocation))) (Variables|Default|GetEffectiveDistance))
      (Utilities|IsValid SplineObject
        (:Is%20Valid
          (bind _resultout (CallFunction|InternalandExternalJudgments SplineObject))
          (if (>= _resultout (* (Math|Trig|GetPI) 2.0))
            (Default|AddEncloseEnemyList (Variables|Default|GetAs%20BP%20Practise%20Drift%20Player%20Con) self)
            (Variables|Default|SetEnclosed true)))))))

(event Custom|EncloseEvent
  (CallFunction|Death true true))

(event Custom|SmashEnemy_Event
  (params (Rotator :type Rotator) (SmashSpeed :type Float%20%28double-precision%29))
  (bind _maxspeed (Variables|Default|GetMaxSpeed))
  (bind _minspeed (Variables|Default|GetMinSpeed))
  (if (>= SmashSpeed _maxspeed)
    (Variables|Default|SetNowSpeed _maxspeed)
    (elif (<= SmashSpeed _minspeed)
      (Variables|Default|SetNowSpeed _minspeed)
      (else
        (Variables|Default|SetNowSpeed SmashSpeed)))))

(event Custom|EnemyCountUP
  (bind _returnvalue (Actor|GetActorOfClass "/Game/Misoten/BP/Misoten_Enemy/Enemy/Boss/BP_BOSS.BP_BOSS_C"))
  (Utilities|IsValid _returnvalue
    (:Is%20Valid
      (if (Variables|/Game/Misoten/BP/Misoten_Enemy/Enemy/Boss/BP_BOSS.BP_BOSS_C|GetBOSSStageNaw _returnvalue)
        (Variables|/Game/Misoten/BP/Misoten_Enemy/Enemy/Boss/BP_BOSS.BP_BOSS_C|SetEnemyCount _returnvalue (+ (Variables|/Game/Misoten/BP/Misoten_Enemy/Enemy/Boss/BP_BOSS.BP_BOSS_C|GetEnemyCount _returnvalue) 1.0))))))

(event Custom|EnemyCountDown
  (bind _returnvalue (Actor|GetActorOfClass "/Game/Misoten/BP/Misoten_Enemy/Enemy/Boss/BP_BOSS.BP_BOSS_C"))
  (Utilities|IsValid _returnvalue
    (:Is%20Valid
      (if (Variables|/Game/Misoten/BP/Misoten_Enemy/Enemy/Boss/BP_BOSS.BP_BOSS_C|GetBOSSStageNaw _returnvalue)
        (bind _output_get (Variables|/Game/Misoten/BP/Misoten_Enemy/Enemy/Boss/BP_BOSS.BP_BOSS_C|SetEnemyCount _returnvalue (+ (Variables|/Game/Misoten/BP/Misoten_Enemy/Enemy/Boss/BP_BOSS.BP_BOSS_C|GetEnemyCount _returnvalue) -1.0)))
        (if (== _output_get 0.0)
          (Default|SpawnEnemy _returnvalue))))))

(event Custom|NSDrop
  (Components|Activation|SetActive (Variables|Default|GetNS_Drop1) true false))

(event EventBeginPlay
  (EventDispatchers|BindEventtoSmashEnemy (delegate Custom|SmashEnemy_Event))
  (EventDispatchers|BindEventtoSmashEnemy (delegate Custom|LookatVector))
  (bind _asbp_practise_drift_pawn (Utilities|Casting|CastToBP_PractiseDrift_Pawn (Game|Player|GetPlayerPawn 0)))
  (Variables|Default|SetAs%20BP%20Practise%20Drift%20Pawn _asbp_practise_drift_pawn)
  (bind _asbp_practise_drift_player_con (Utilities|Casting|CastToBP_PractiseDrift_PlayerCon (Game|GetPlayerController 0)))
  (Variables|Default|SetAs%20BP%20Practise%20Drift%20Player%20Con _asbp_practise_drift_player_con)
  (EventDispatchers|BindEventtoHitStage (delegate Custom|HitStage_Event))
  (EventDispatchers|BindEventtoEncloseJudge (Variables|Default|GetAs%20BP%20Practise%20Drift%20Pawn) (delegate Custom|EncloseJudgeEvent))
  (EventDispatchers|BindEventtoStartPause (Variables|Default|GetAs%20BP%20Practise%20Drift%20Player%20Con) (delegate Custom|SetCustomTimeDilationZero))
  (EventDispatchers|BindEventtoStopPause (Variables|Default|GetAs%20BP%20Practise%20Drift%20Player%20Con) (delegate Custom|SetCustomTimeDilationOne)))

(event EventDestroyed
  (bind _parent (Variables|Default|Getparent))
  (if (Utilities|IsValid _parent)
    (Default|ArrayConfirm _parent)))

(event EventTick
  (params (DeltaSeconds :type Float%20%28single-precision%29))
  (bind _returnvalue (Transformation|GetActorLocation))
  (if (Variables|Default|GetIsHit)
    (bind _output_get (Variables|Default|SetHitTime (+ (Variables|Default|GetHitTime) DeltaSeconds)))
    (if (>= _output_get 3.0)
      (CallFunction|Death false true)))
  (bind _sweephitresult (Transformation|AddActorWorldOffset (* (Transformation|GetActorForwardVector) (Variables|Default|GetNowSpeed)) true))
  (bind _outhit (Collision|LineTraceByChannel _returnvalue (+ _returnvalue (* (Transformation|GetActorForwardVector) -3e+03)) "TraceTypeQuery1" true 0 "None" true "(R=1.000000,G=0.000000,B=0.000000,A=1.000000)" "(R=0.000000,G=1.000000,B=0.000000,A=1.000000)" 1.0))
  (if (and (.bBlockingHit (Collision|BreakHitResult _outhit)) (.bBlockingHit (Collision|BreakHitResult _sweephitresult)))
    (Default|CallHitStage)
    (Transformation|SetActorRotation (Math|Conversions|RotationFromXVector (Math|Vector|MirrorVectorbyNormal (Transformation|GetActorForwardVector) (.ImpactNormal (Collision|BreakHitResult _outhit)))))
    (Transformation|AddActorWorldOffset (* (Transformation|GetActorForwardVector) (Variables|Default|GetNowSpeed)) true)
    (bind _returnvalue_2 (Niagara|SpawnSystematLocation "/Game/Misoten/Assets/EFF/Toon_Shockwave/NS_ToonShockwave.NS_ToonShockwave" (Transformation|GetActorLocation) (Transformation|GetActorRotation) "3.000000,3.000000,3.000000"))
    (Rendering|SetRenderCustomDepth _returnvalue_2 false)
    (if (>= (Variables|Default|GetHitFloorNum) (Variables|Default|GetMaxHitFloorNum))
      (CallFunction|Death false true)
      (else
        (bind _output_get_2 (Variables|Default|SetHitFloorNum (+ (Variables|Default|GetHitFloorNum) 1)))
        (Variables|Default|SetNowSpeed (* _output_get_2 (Variables|Default|GetNowSpeed)))))
    (elif (.bBlockingHit (Collision|BreakHitResult _sweephitresult))
      (Transformation|AddActorWorldOffset (* (Transformation|GetActorForwardVector) (Variables|Default|GetNowSpeed))))))

(fn ConstructionScript
  (bind _returnvalue (Utilities|GetDataTableRow "/Game/Misoten/BP/DataTable/EnemyStatusDataTable.EnemyStatusDataTable" "Normal")
    (:then
      (Variables|Default|SetHP (.HP (Utilities|Struct|BreakEnemyStatusStruct _returnvalue)))
      (Variables|Default|SetNormalSpeed (.NormalSpeed (Utilities|Struct|BreakEnemyStatusStruct _returnvalue))))))

(fn Attack)

(fn Damage
  (params (Damage :type Float%20%28double-precision%29))
  (bind _asabp_crow_anim (Utilities|Casting|CastToABP_CrowAnim (Components|SkeletalMesh|GetAnimInstance (Variables|Default|GetCrow)))
    (:then
      (Default|SetDamage _asabp_crow_anim true))
    (:CastFailed
      _))
  (bind _output_get (Variables|Default|SetHP (- (Variables|Default|GetHP) Damage)))
  (Variables|Default|SetIsHit true)
  (return (<= _output_get 0.0)))

(fn InternalandExternalJudgments
  (params (Spline :type Spline%20Component%20Object%20Reference))
  (bind _returnvalue (Transformation|GetActorLocation))
  (LocalVariables|SetSplineObject Spline)
  (LocalVariables|SetResult 0.0)
  (bind _index (Utilities|FlowControl|ForLoopwithBreak 0 (- (Class|SplineComponent|GetNumberOfSplineSegments (LocalVariables|GetSplineObject)) 2) :!label _label)
    (:LoopBody
      (Utilities|IsValid (LocalVariables|GetSplineObject)
        (:Is%20Valid
          (if (< (Math|Vector|DotProduct (Math|Vector|CrossProduct (- (.Location (Spline|GetLocationandTangentatSplinePoint (LocalVariables|GetSplineObject) _index "World")) _returnvalue) (- (.Location (Spline|GetLocationandTangentatSplinePoint (LocalVariables|GetSplineObject) (+ _index 1) "World")) _returnvalue)) (Math|Vector|MakeVector 0.0 0.0 1.0)) 0.0)
            (LocalVariables|SetResult (+ (Math|Trig|Acos(Degrees) (/ (Math|Vector|DotProduct (- (.Location (Spline|GetLocationandTangentatSplinePoint (LocalVariables|GetSplineObject) _index "World")) _returnvalue) (- (.Location (Spline|GetLocationandTangentatSplinePoint (LocalVariables|GetSplineObject) (+ _index 1) "World")) _returnvalue)) (* (Math|Vector|VectorLength (- (.Location (Spline|GetLocationandTangentatSplinePoint (LocalVariables|GetSplineObject) _index "World")) _returnvalue)) (Math|Vector|VectorLength (- (.Location (Spline|GetLocationandTangentatSplinePoint (LocalVariables|GetSplineObject) (+ _index 1) "World")) _returnvalue))))) (LocalVariables|GetResult)))
            (else
              (LocalVariables|SetResult (+ (* (Math|Trig|Acos(Degrees) (/ (Math|Vector|DotProduct (- (.Location (Spline|GetLocationandTangentatSplinePoint (LocalVariables|GetSplineObject) _index "World")) _returnvalue) (- (.Location (Spline|GetLocationandTangentatSplinePoint (LocalVariables|GetSplineObject) (+ _index 1) "World")) _returnvalue)) (* (Math|Vector|VectorLength (- (.Location (Spline|GetLocationandTangentatSplinePoint (LocalVariables|GetSplineObject) _index "World")) _returnvalue)) (Math|Vector|VectorLength (- (.Location (Spline|GetLocationandTangentatSplinePoint (LocalVariables|GetSplineObject) (+ _index 1) "World")) _returnvalue))))) -1.0) (LocalVariables|GetResult))))))
        (:Is%20Not%20Valid
          (goto _label Break))))
    (:Completed
      (return (Math|Float|Absolute(Float) (LocalVariables|GetResult))))))

(fn GetIsMove
  (if (Math|Float|NearlyEqual(Float) (Variables|Default|GetNowSpeed) 0.0 1e-06)
    (return false)
    (else
      (return true))))

(fn Death
  (params (isEnclose :type Boolean) (IsDeath :type Boolean))
  (bind _returnvalue (Transformation|GetActorTransform))
  (bind _returnvalue_2 (Transformation|GetActorTransform))
  (bind _parent (Variables|Default|Getparent))
  (if IsDeath
    (if isEnclose
      (Niagara|SpawnSystematLocation "/Game/Misoten/Assets/EFF/EFF_LightningAttack/NS_LightningAttack.NS_LightningAttack" (.location _returnvalue_2) (.rotation _returnvalue_2))
      (Default|AddScoreEnclose (Variables|/Game/Misoten/BP/BP_PractiseDrift_Pawn.BP_PractiseDrift_Pawn_C|GetBP_PlayerState (Variables|Default|GetAs%20BP%20Practise%20Drift%20Pawn)))
      (else
        (Niagara|SpawnSystematLocation "/Game/Misoten/Assets/EFF/FX_Enemy_Disappearance/NS_Enemy_Disappearance.NS_Enemy_Disappearance" (.location _returnvalue) (.rotation _returnvalue) "0.200000,0.200000,0.200000")
        (Default|AddScoreCharge (Variables|/Game/Misoten/BP/BP_PractiseDrift_Pawn.BP_PractiseDrift_Pawn_C|GetBP_PlayerState (Variables|Default|GetAs%20BP%20Practise%20Drift%20Pawn)))))
    ;[1 1 1] スポナーで生成されたオブジェクトなら次のウェーブへ遷移するか確認する
    (if (Utilities|IsValid _parent)
      (Utilities|Array|RemoveIndex (Variables|/Game/Misoten/BP/Misoten_Enemy/Enemy/tutrial/wave/BP_WaveEnemySpawner.BP_WaveEnemySpawner_C|Getnow%20Enemy%20Obj _parent))
      (Default|ArrayConfirm (Variables|Default|Getparent)))
    (CallFunction|EnemyCountDown)
    (Actor|DestroyActor)
    (else
      (return))))