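; BP_CrowNormal_Burette is a projectile actor (apparently a crow enemy's normal bullet) that flies in a straight line toward where the player was at spawn.
; BeginPlay snapshots the player's location, takes its start point from BP_BOSSChase's Bullet component and its speed from that boss's OutRowThrowingSpeed, then faces the player.
; Tick makes a swept move along that fixed direction by Speed per frame, without delta-time scaling or calling parent Tick.
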(event EventBeginPlay
  (Utilities|FlowControl|Sequence
    (:then_0
      (|CallParentFunction))
    (:then_1
      (Variables|Default|SetTargetLocation (Transformation|GetActorLocation (Game|GetPlayerCharacter 0)))
      (bind _returnvalue (Actor|GetActorOfClass "/Game/Misoten/BP/Misoten_Enemy/Enemy/Boss/BP_BOSSChase.BP_BOSSChase_C"))
      (Variables|Default|SetStartLocation (Transformation|GetWorldLocation (Variables|/Game/Misoten/BP/Misoten_Enemy/Enemy/Boss/BP_BOSSChase.BP_BOSSChase_C|GetBullet _returnvalue)))
      (Variables|Default|SetSpeed (Variables|/Game/Misoten/BP/Misoten_Enemy/Enemy/Boss/BP_BOSSChase.BP_BOSSChase_C|GetOut%20Row%20Throwing%20Speed _returnvalue))
      (Transformation|SetActorRotation (Math|Rotator|FindLookatRotation (Transformation|GetActorLocation) (Transformation|GetActorLocation (Game|GetPlayerCharacter 0)))))))

(event Collision|EventActorBeginOverlap
  (params (OtherActor :type Actor%20Object%20Reference))
  (|CallParentFunction OtherActor) ; このノードは無効になっているため呼び出せません。\n機能をビルドするにはピンをドラッグしてください。
)

(event EventTick
  (params (DeltaSeconds :type Float%20%28single-precision%29))
  (Utilities|FlowControl|Sequence
    (:then_1
      (Transformation|AddActorWorldOffset (* (Math|Vector|Normalize (- (Variables|Default|GetTargetLocation) (Variables|Default|GetStartLocation))) (Variables|Default|GetSpeed)) true))))

(fn ConstructionScript
  (|CallParentFunction))