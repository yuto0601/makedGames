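; Crow enemy projectile thrown by BP_BOSS at the player, which the player can reflect back for score.
; BeginPlay sets the damage animation and marks a target led ahead by player speed; Tick moves it along the start-to-target direction at boss-defined speed.
; Reflection retargets the boss's reflection point with hit effects and camera shake.
; Overlap damages and stuns the boss after reflection, or turns the projectile into BP_CrowNormal on the floor.
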(event OnComponentBeginOverlap(Box)
  (params (OverlappedComponent :type Primitive%20Component%20Object%20Reference) (OtherActor :type Actor%20Object%20Reference) (OtherComp :type Primitive%20Component%20Object%20Reference) (OtherBodyIndex :type Integer) (bFromSweep :type Boolean) (SweepResult :type Hit%20Result%20Structure%20%28by%20ref%29))
  (Utilities|FlowControl|Sequence
    (:then_0
      (if (not (Variables|Default|GetIsThrow))
        ;[1 1 1] ボスに当たった時
        (bind _asbp_boss (Utilities|Casting|CastToBP_BOSS OtherActor))
        (Default|BulletDamage _asbp_boss)
        (Niagara|SpawnSystematLocation "/Game/Misoten/Assets/EFF/EFF_Hit_Level_High/NS_Hit_Level_High.NS_Hit_Level_High" (Transformation|GetWorldLocation (Variables|/Game/Misoten/BP/Misoten_Enemy/Enemy/Boss/BP_BOSS.BP_BOSS_C|GetReflectionLocation _asbp_boss)) "0, 0, 0" "5.000000,5.000000,5.000000")
        (Default|Stan _asbp_boss)
        (Actor|DestroyActor)))
    (:then_1
      ;[1 1 1] 床に当たった時
      (Utilities|Casting|CastToBP_BigArea_AreaF OtherActor)
      (Game|SpawnActorfromClass "/Game/Misoten/BP/Misoten_Enemy/Enemy/BP_CrowNormal.BP_CrowNormal_C" (Math|Transform|MakeTransform (Transformation|GetActorLocation) (Transformation|GetActorRotation) "1.000000,1.000000,1.000000") "Undefined" "MultiplyWithRoot" 0 0)
      (Actor|DestroyActor))))

(event Custom|Reflection
  (params (Start :type Vector))
  ;[1 1 1] 跳ね返し
  (Variables|Default|SetTargetLocation (Variables|Default|GetReflectionLocation))
  (Variables|Default|SetStartLocation Start)
  (bind _returnvalue (Actor|GetActorOfClass "/Game/Misoten/BP/BP_PractiseDrift_Pawn.BP_PractiseDrift_Pawn_C"))
  (Niagara|SpawnSystematLocation "/Game/Misoten/Assets/EFF/EFF_Hit_Level_Low/NS_Hit_Level_Low.NS_Hit_Level_Low" (Math|Vector|MakeVector (.x (Transformation|GetWorldLocation (Variables|/Game/Misoten/BP/BP_PractiseDrift_Pawn.BP_PractiseDrift_Pawn_C|GetAttackCollision _returnvalue))) (.y (Transformation|GetWorldLocation (Variables|/Game/Misoten/BP/BP_PractiseDrift_Pawn.BP_PractiseDrift_Pawn_C|GetAttackCollision _returnvalue))) (+ (.z (Transformation|GetWorldLocation (Variables|/Game/Misoten/BP/BP_PractiseDrift_Pawn.BP_PractiseDrift_Pawn_C|GetAttackCollision _returnvalue))) 1e+02)) (Math|Rotator|FindLookatRotation (Transformation|GetActorLocation) (Camera|GetCameraLocation (Game|GetPlayerCameraManager 0))) "10.000000,10.000000,10.000000")
  (Audio|PlaySoundatLocation "/Game/Misoten/BP/Audio/SE/Player/MS_NomalReflectSuccess.MS_NomalReflectSuccess" "0, 0, 0" "0, 0, 0" 0.6 1.0 0.0 0 0 0 0)
  (CameraShakes|StartCameraShake (Game|GetPlayerCameraManager 0) "/Game/Misoten/BP/Misoten_Enemy/Enemy/Boss/BP_CameraShake_Reflection.BP_CameraShake_Reflection_C" 1.0 "CameraLocal" "0, 0, 0")
  (Variables|Default|SetIsThrow false)
  (bind _asbp_practise_drift_pawn (Utilities|Casting|CastToBP_PractiseDrift_Pawn (Game|Player|GetPlayerPawn 0)))
  (Default|AddScoreReflection (Variables|/Game/Misoten/BP/BP_PractiseDrift_Pawn.BP_PractiseDrift_Pawn_C|GetBP_PlayerState _asbp_practise_drift_pawn)))

(event EventBeginPlay
  ;[1 1 1] ダメージを受けた時のアニメーション
  (bind _asabp_crow_anim (Utilities|Casting|CastToABP_CrowAnim (Components|SkeletalMesh|GetAnimInstance (Variables|Default|GetSkeletalMesh))))
  (Default|SetDamage _asabp_crow_anim true)
  ;[1 1 1] 投げる場所と狙う場所の位置を取得
  (bind _returnvalue (Actor|GetActorOfClass "/Game/Misoten/BP/Misoten_Enemy/Enemy/Boss/BP_BOSS.BP_BOSS_C"))
  (Variables|Default|SetReflectionLocation (Transformation|GetWorldLocation (Variables|/Game/Misoten/BP/Misoten_Enemy/Enemy/Boss/BP_BOSS.BP_BOSS_C|GetReflectionLocation _returnvalue)))
  (Variables|Default|SetTargetLocation (Transformation|GetActorLocation (Game|GetPlayerCharacter 0)))
  ;[1 1 1] 投げるスピードの取得
  (bind _returnvalue_2 (Actor|GetActorOfClass "/Game/Misoten/BP/Misoten_Enemy/Enemy/Boss/BP_BOSS.BP_BOSS_C"))
  (Variables|Default|SetStartLocation (Transformation|GetWorldLocation (Variables|/Game/Misoten/BP/Misoten_Enemy/Enemy/Boss/BP_BOSS.BP_BOSS_C|GetBulletLocation _returnvalue_2)))
  (Variables|Default|SetSpeed (Variables|/Game/Misoten/BP/Misoten_Enemy/Enemy/Boss/BP_BOSS.BP_BOSS_C|GetOut%20Row%20Throwing%20Speed _returnvalue_2))
  ;[1 1 1] プレイヤーのほうを向く
  (Transformation|SetActorRotation (Math|Rotator|FindLookatRotation (Transformation|GetActorLocation) (Transformation|GetActorLocation (Game|GetPlayerCharacter 0))))
  ;[1 1 1] 狙う場所をプレイヤーのちょっと前にする
  (bind _asbp_practise_drift_player_con (Utilities|Casting|CastToBP_PractiseDrift_PlayerCon (Game|GetPlayerController 0)))
  (bind _output_get (Variables|Default|SetTargetLocation (+ (* (Transformation|GetActorForwardVector _asbp_practise_drift_player_con) (* (Variables|/Game/Misoten/BP/BP_PractiseDrift_PlayerCon.BP_PractiseDrift_PlayerCon_C|GetNowSpeed _asbp_practise_drift_player_con) 45.0)) (Transformation|GetActorLocation (Game|GetPlayerCharacter 0)))))
  (Niagara|SpawnSystematLocation "/Game/Misoten/Assets/EFF/EFF_Throw_TargetPoint/NS_Throw_Target_v2.NS_Throw_Target_v2" _output_get))

(event EventTick
  (params (DeltaSeconds :type Float%20%28single-precision%29))
  ;[1 1 1] 狙った場所に移動する
  (Transformation|AddActorWorldOffset (* (Math|Vector|Normalize (- (Variables|Default|GetTargetLocation) (Variables|Default|GetStartLocation))) (Variables|Default|GetSpeed))))

(fn ConstructionScript)