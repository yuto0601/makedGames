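; Projectile for the chase boss, fired along a straight line toward one of three lanes.
; On BeginPlay it turns toward the player, reads BP_BOSSChase's throw point and randomly picks its left, middle or right target.
; Tick moves it along that direction by Speed per frame, without delta-time scaling.
; Overlapping a BP_Mesh_Finish spawns a BP_BOSSChase_Bullet_Roll slightly above it and destroys the bullet.
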(event OnComponentBeginOverlap(Box)
  (params (OverlappedComponent :type Primitive%20Component%20Object%20Reference) (OtherActor :type Actor%20Object%20Reference) (OtherComp :type Primitive%20Component%20Object%20Reference) (OtherBodyIndex :type Integer) (bFromSweep :type Boolean) (SweepResult :type Hit%20Result%20Structure%20%28by%20ref%29))
  (bind _returnvalue (Transformation|GetActorLocation))
  (Utilities|Casting|CastToBP_Mesh_Finish OtherActor)
  (Utilities|FlowControl|DoOnce false
    (:Completed
      (Game|SpawnActorfromClass "/Game/Misoten/BP/Misoten_Enemy/Enemy/Boss/BP_BOSSChase_Bullet_Roll.BP_BOSSChase_Bullet_Roll_C" (Math|Transform|MakeTransform (Math|Vector|MakeVector (.x _returnvalue) (.y _returnvalue) (+ (.z _returnvalue) 5e+01)) (Transformation|GetActorRotation) "1.000000,1.000000,1.000000") "Undefined" "MultiplyWithRoot" 0 0)
      (Actor|DestroyActor))))

(event EventBeginPlay
  (bind _returnvalue (Math|Random|RandomIntegerinRange 0 2))
  (Transformation|SetActorRotation (Math|Interpolation|RInterpTo (Transformation|GetActorRotation) (Math|Rotator|FindLookatRotation (Transformation|GetActorLocation) (Transformation|GetActorLocation (Game|GetPlayerCharacter 0))) (Utilities|Time|GetWorldDeltaSeconds) 0.0))
  (bind _returnvalue_2 (Actor|GetActorOfClass "/Game/Misoten/BP/Misoten_Enemy/Enemy/Boss/BP_BOSSChase.BP_BOSSChase_C"))
  (bind _output_get (Variables|Default|SetBP_BOSSChase _returnvalue_2))
  (Variables|Default|SetThrowPosition (Transformation|GetWorldLocation (Variables|/Game/Misoten/BP/Misoten_Enemy/Enemy/Boss/BP_BOSSChase.BP_BOSSChase_C|GetThrowPoint _output_get)))
  (Variables|Default|SetTargetArry (Utilities|Array|MakeArray (Transformation|GetWorldLocation (Variables|/Game/Misoten/BP/Misoten_Enemy/Enemy/Boss/BP_BOSSChase.BP_BOSSChase_C|GetTargetLeft (Variables|Default|GetBP_BOSSChase))) (Transformation|GetWorldLocation (Variables|/Game/Misoten/BP/Misoten_Enemy/Enemy/Boss/BP_BOSSChase.BP_BOSSChase_C|GetTargetMiddle (Variables|Default|GetBP_BOSSChase))) (Transformation|GetWorldLocation (Variables|/Game/Misoten/BP/Misoten_Enemy/Enemy/Boss/BP_BOSSChase.BP_BOSSChase_C|GetTargetRight (Variables|Default|GetBP_BOSSChase)))))
  (Variables|Default|SetTargetPosition (Utilities|Array|Get(acopy) (Variables|Default|GetTargetArry) _returnvalue))
  (Development|PrintString (Utilities|String|ToString(Integer) _returnvalue)))

(event EventTick
  (params (DeltaSeconds :type Float%20%28single-precision%29))
  (Transformation|AddActorWorldOffset (* (Math|Vector|Normalize (- (Variables|Default|GetTargetPosition) (Variables|Default|GetThrowPosition))) (Variables|Default|GetSpeed))))

(fn ConstructionScript)