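; BP_BOSSChase_Bullet_Roll is a boss chase bullet that can be reflected and respects the game's pause.
; Reflection spawns a BP_BOSSChase_Reflection at the bullet's location and destroys the bullet.
; On BeginPlay it binds to the player controller's pause events, which freeze or restore it through CustomTimeDilation and an IsPause flag.
; The graph's force nodes are unconnected, so no movement is driven here.
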(event Custom|Reflection
  (Game|SpawnActorfromClass "/Game/Misoten/BP/Misoten_Enemy/Enemy/Boss/BP_BOSSChase_Reflection.BP_BOSSChase_Reflection_C" (Math|Transform|MakeTransform (Transformation|GetActorLocation) "0, 0, 0" "1.000000,1.000000,1.000000") "Undefined" "MultiplyWithRoot" 0 0)
  (Actor|DestroyActor))

(event Custom|SetCustomTimeDilationZero
  (Variables|Default|SetCustomTimeDilation 0.0)
  (Variables|Default|SetIsPause true))

(event Custom|SetCustomTimeDilationOne
  (Variables|Default|SetCustomTimeDilation 1.0)
  (Variables|Default|SetIsPause false))

(event EventBeginPlay
  (bind _asbp_practise_drift_player_con (Utilities|Casting|CastToBP_PractiseDrift_PlayerCon (Game|GetPlayerController 0)))
  (EventDispatchers|BindEventtoStartPause _asbp_practise_drift_player_con (delegate Custom|SetCustomTimeDilationZero))
  (EventDispatchers|BindEventtoStopPause _asbp_practise_drift_player_con (delegate Custom|SetCustomTimeDilationOne)))

(fn ConstructionScript)