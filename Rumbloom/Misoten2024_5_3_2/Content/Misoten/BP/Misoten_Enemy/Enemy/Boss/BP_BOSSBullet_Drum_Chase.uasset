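; Drum projectile thrown by the chase boss at the player during a chase.
; On spawn it faces the player and takes its start point and speed from BP_BOSSChase, then moves each tick along that fixed direction without delta-time scaling or homing.
; Reflection redirects it from a given point toward its original launch point.
; Overlapping the drift pawn zeroes the player's speed, flags the boss, triggers a hit reaction and destroys the drum.
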(event OnComponentBeginOverlap(Capsule)
  (params (OverlappedComponent :type Primitive%20Component%20Object%20Reference) (OtherActor :type Actor%20Object%20Reference) (OtherComp :type Primitive%20Component%20Object%20Reference) (OtherBodyIndex :type Integer) (bFromSweep :type Boolean) (SweepResult :type Hit%20Result%20Structure%20%28by%20ref%29))
  (bind _asbp_practise_drift_pawn (Utilities|Casting|CastToBP_PractiseDrift_Pawn OtherActor))
  (bind _asbp_practise_drift_player_con (Utilities|Casting|CastToBP_PractiseDrift_PlayerCon (Game|GetPlayerController 0)))
  (Variables|/Game/Misoten/BP/BP_PractiseDrift_PlayerCon.BP_PractiseDrift_PlayerCon_C|SetNowSpeed _asbp_practise_drift_player_con 0.0)
  (bind _returnvalue (Actor|GetActorOfClass "/Game/Misoten/BP/Misoten_Enemy/Enemy/Boss/BP_BOSSChase.BP_BOSSChase_C"))
  (Variables|/Game/Misoten/BP/Misoten_Enemy/Enemy/Boss/BP_BOSSChase.BP_BOSSChase_C|SetHit2Flg _returnvalue true)
  (Default|HitReaction _asbp_practise_drift_pawn)
  (Actor|DestroyActor))

(event Custom|Reflection
  (params (Start :type Vector))
  (Variables|Default|SetTargetLocation (Variables|Default|GetStartLocation))
  (Variables|Default|SetStartLocation Start))

(event EventBeginPlay
  (Variables|Default|SetTargetLocation (Transformation|GetActorLocation (Game|GetPlayerCharacter 0)))
  (bind _returnvalue (Actor|GetActorOfClass "/Game/Misoten/BP/Misoten_Enemy/Enemy/Boss/BP_BOSSChase.BP_BOSSChase_C"))
  (Variables|Default|SetStartLocation (Transformation|GetWorldLocation (Variables|/Game/Misoten/BP/Misoten_Enemy/Enemy/Boss/BP_BOSSChase.BP_BOSSChase_C|GetBullet _returnvalue)))
  (Variables|Default|SetSpeed (Variables|/Game/Misoten/BP/Misoten_Enemy/Enemy/Boss/BP_BOSSChase.BP_BOSSChase_C|GetOut%20Row%20Throwing%20Speed _returnvalue))
  (Transformation|SetActorRotation (Math|Rotator|FindLookatRotation (Transformation|GetActorLocation) (Transformation|GetActorLocation (Game|GetPlayerCharacter 0)))))

(event EventTick
  (params (DeltaSeconds :type Float%20%28single-precision%29))
  (Transformation|AddActorWorldOffset (* (Math|Vector|Normalize (- (Variables|Default|GetTargetLocation) (Variables|Default|GetStartLocation))) (Variables|Default|GetSpeed))))

(fn ConstructionScript)