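; Chase-stage boss, a panda on a bike that races ahead of the player throwing drums.
; Loads stats from a data table, drives forward along its facing, takes yaw from a supplied spline, and otherwise recenters.
; Rams cost HP, add score and slow both racers; a front blocker also slows the player.
; AnimBP flags coordinate attacks, damage, the low-HP pinch phase and the death sequence with camera switch and explosion.
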(event OnComponentHit(Box1)
  (params (HitComponent :type Primitive%20Component%20Object%20Reference) (OtherActor :type Actor%20Object%20Reference) (OtherComp :type Primitive%20Component%20Object%20Reference) (NormalImpulse :type Vector :default "0, 0, 0") (Hit :type Hit%20Result%20Structure%20%28by%20ref%29))
  ;[1 1 1] 前に出ないようにするためのコリジョンにぶつかった時の処理
  (Utilities|Casting|CastToBP_PractiseDrift_Pawn OtherActor)
  (if (not (Variables|Default|GetHitFlg))
    (Variables|Default|SetHit2Flg true)))

(event OnComponentHit(Box)
  (params (HitComponent :type Primitive%20Component%20Object%20Reference) (OtherActor :type Actor%20Object%20Reference) (OtherComp :type Primitive%20Component%20Object%20Reference) (NormalImpulse :type Vector :default "0, 0, 0") (Hit :type Hit%20Result%20Structure%20%28by%20ref%29))
  ;[1 1 1] ボスにヒットした時の処理
  (Utilities|Casting|CastToBP_PractiseDrift_Pawn OtherActor)
  (if (not (Variables|Default|GetHit2Flg))
    (Variables|Default|SetHitFlg true)
    (bind _asabp_bosspanda_chase (Utilities|Casting|CastToABP_BOSSPanda_Chase (Components|SkeletalMesh|GetAnimInstance (Variables|Default|GetBOSSPanda))))
    (Variables|/Game/Misoten/BP/Misoten_Enemy/Enemy/Boss/ABP_BOSSPanda_Chase.ABP_BOSSPanda_Chase_C|SetDamageFlg _asabp_bosspanda_chase true)
    (Variables|/Game/Misoten/BP/Misoten_Enemy/Enemy/Boss/ABP_BOSSPanda_Chase.ABP_BOSSPanda_Chase_C|SetPitchDamageFlg _asabp_bosspanda_chase true)
    (bind _asabp_model_bossbike (Utilities|Casting|CastToABP_Model_BOSSBike (Components|SkeletalMesh|GetAnimInstance (Variables|Character|GetMesh))))
    (Variables|/Game/Misoten/BP/Misoten_Enemy/Enemy/Boss/ABP_Model_BOSSBike.ABP_Model_BOSSBike_C|SetDamageFlg _asabp_model_bossbike true)
    (Variables|/Game/Misoten/BP/Misoten_Enemy/Enemy/Boss/ABP_Model_BOSSBike.ABP_Model_BOSSBike_C|SetPitchDamageFlg _asabp_model_bossbike true)
    (bind _asabp_bosspanda_chase_2 (Utilities|Casting|CastToABP_BOSSPanda_Chase (Components|SkeletalMesh|GetAnimInstance (Variables|Default|GetBOSSPanda))))
    (Variables|/Game/Misoten/BP/Misoten_Enemy/Enemy/Boss/ABP_BOSSPanda_Chase.ABP_BOSSPanda_Chase_C|SetAttackFlg _asabp_bosspanda_chase_2 false)
    (Variables|/Game/Misoten/BP/Misoten_Enemy/Enemy/Boss/ABP_BOSSPanda_Chase.ABP_BOSSPanda_Chase_C|SetBOSSPand_AttackFlg _asabp_bosspanda_chase_2 false)
    (bind _asabp_model_bossbike_2 (Utilities|Casting|CastToABP_Model_BOSSBike (Components|SkeletalMesh|GetAnimInstance (Variables|Character|GetMesh))))
    (Variables|/Game/Misoten/BP/Misoten_Enemy/Enemy/Boss/ABP_Model_BOSSBike.ABP_Model_BOSSBike_C|SetBOSSBikeAttackFlg _asabp_model_bossbike_2 false)
    (Variables|/Game/Misoten/BP/Misoten_Enemy/Enemy/Boss/ABP_Model_BOSSBike.ABP_Model_BOSSBike_C|SetBossBikePitchAttakFlg _asabp_model_bossbike_2 false)
    (Variables|Default|SetNowSpeed 1.4e+02)
    (bind _asbp_practise_drift_pawn (Utilities|Casting|CastToBP_PractiseDrift_Pawn (Game|Player|GetPlayerPawn 0)))
    (Default|AddScoreBOSSEnclose (Variables|/Game/Misoten/BP/BP_PractiseDrift_Pawn.BP_PractiseDrift_Pawn_C|GetBP_PlayerState _asbp_practise_drift_pawn))))

(event Custom|DownSpeedEventLeftLight
  ;[1 1 1] ボスより前に行かないようにする為のコリジョンに当たった時の処理
  (if (Variables|Default|GetHit2Flg)
    (bind _asbp_practise_drift_player_con (Utilities|Casting|CastToBP_PractiseDrift_PlayerCon (Game|GetPlayerController 0)))
    (Math|Float|DecrementFloat (Variables|/Game/Misoten/BP/BP_PractiseDrift_PlayerCon.BP_PractiseDrift_PlayerCon_C|GetNowSpeed _asbp_practise_drift_player_con)
      (:%20%20
        (if (> (Variables|Default|GetCount) 60)
          (Variables|Default|SetHit2Flg false)
          (Variables|Default|SetCount 0)
          (bind _asabp_bosspanda_chase (Utilities|Casting|CastToABP_BOSSPanda_Chase (Components|SkeletalMesh|GetAnimInstance (Variables|Default|GetBOSSPanda))))
          (Variables|/Game/Misoten/BP/Misoten_Enemy/Enemy/Boss/ABP_BOSSPanda_Chase.ABP_BOSSPanda_Chase_C|SetDamageFlg _asabp_bosspanda_chase false)
          (bind _asabp_model_bossbike (Utilities|Casting|CastToABP_Model_BOSSBike (Components|SkeletalMesh|GetAnimInstance (Variables|Character|GetMesh))))
          (Variables|/Game/Misoten/BP/Misoten_Enemy/Enemy/Boss/ABP_Model_BOSSBike.ABP_Model_BOSSBike_C|SetDamageFlg _asabp_model_bossbike false)
          (else
            (Math|Integer|IncrementInt (Variables|Default|GetCount))))))))

(event Custom|SplineSupportStart
  ;[1 1 1] ボスの体力が0になった時の処理
  (bind _returnvalue (Utilities|Time|SetTimerbyEvent (delegate Custom|SplineSupportTimerEvent) (Utilities|Time|GetWorldDeltaSeconds) true))
  (Variables|Default|SetSplineSupportTimerHundle _returnvalue))

(event Custom|SplineSupportTimerEvent
  (bind _returnvalue (Transformation|GetActorRotation))
  (bind _returnvalue_2 (Transformation|GetActorLocation))
  (bind _movesupportsline (Variables|Default|GetMoveSupportSline))
  (bind _returnvalue_3 (Class|SplineComponent|GetDistanceAlongSplineatLocation _movesupportsline _returnvalue_2 "World"))
  ;[1 1 1] ボスの体力が0になった時の処理
  (Utilities|IsValid _movesupportsline
    (:Is%20Valid
      (Variables|Default|SetFrontLine true)
      (Transformation|SetActorRotation (Math|Rotator|MakeRotator (.roll _returnvalue) (.pitch _returnvalue) (.yaw (Spline|GetRotationatDistanceAlongSpline _movesupportsline _returnvalue_3 "World"))))
      (if (Math|Float|NearlyEqual(Float) (Spline|GetSplineLength _movesupportsline) _returnvalue_3 1e-06)
        (Utilities|Time|ClearandInvalidateTimerbyHandle (Variables|Default|GetSplineSupportTimerHundle))
        (Variables|Default|SetFrontLine false)))))

(event Custom|HitDownEvent
  (bind _returnvalue (Game|Player|GetPlayerPawn 0))
  (bind _returnvalue_2 (Transformation|GetActorTransform _returnvalue))
  (bind (_location _rotation) (Math|Transform|BreakTransform _returnvalue_2))
  ;[1 1 1] ボスにヒットした時の詳細な処理
  (if (Variables|Default|GetHitFlg)
    (bind _asbp_practise_drift_player_con (Utilities|Casting|CastToBP_PractiseDrift_PlayerCon (Game|GetPlayerController 0)))
    (Math|Float|DecrementFloat (Variables|/Game/Misoten/BP/BP_PractiseDrift_PlayerCon.BP_PractiseDrift_PlayerCon_C|GetNowSpeed _asbp_practise_drift_player_con)
      (:%20%20
        (if (> (Variables|Default|GetCountHit) 60)
          ;;[1 1 1] 停止時間が終わった時の処理
          (Variables|Default|SetHitFlg false)
          (Variables|Default|SetCountHit 0)
          (bind _asabp_bosspanda_chase (Utilities|Casting|CastToABP_BOSSPanda_Chase (Components|SkeletalMesh|GetAnimInstance (Variables|Default|GetBOSSPanda))))
          (Variables|/Game/Misoten/BP/Misoten_Enemy/Enemy/Boss/ABP_BOSSPanda_Chase.ABP_BOSSPanda_Chase_C|SetDamageFlg _asabp_bosspanda_chase false)
          (Variables|/Game/Misoten/BP/Misoten_Enemy/Enemy/Boss/ABP_BOSSPanda_Chase.ABP_BOSSPanda_Chase_C|SetPitchDamageFlg _asabp_bosspanda_chase false)
          (bind _asabp_model_bossbike (Utilities|Casting|CastToABP_Model_BOSSBike (Components|SkeletalMesh|GetAnimInstance (Variables|Character|GetMesh))))
          (Variables|/Game/Misoten/BP/Misoten_Enemy/Enemy/Boss/ABP_Model_BOSSBike.ABP_Model_BOSSBike_C|SetDamageFlg _asabp_model_bossbike false)
          (Variables|/Game/Misoten/BP/Misoten_Enemy/Enemy/Boss/ABP_Model_BOSSBike.ABP_Model_BOSSBike_C|SetPitchDamageFlg _asabp_model_bossbike false)
          (CallFunction|HitStartEvent)
          (else
            ;;[1 1 1] プレイヤーが停止してる時に行う処理
            (Math|Integer|IncrementInt (Variables|Default|GetCountHit)
              (:%20%20
                (Utilities|FlowControl|DoOnce false
                  (:Completed
                    (bind _result (Math|Float|DecrementFloat (Variables|Default|GetHP))
                      (:%20%20
                        (Variables|Default|SetHP _result)
                        (bind _asbp_practise_drift_player_con_2 (Utilities|Casting|CastToBP_PractiseDrift_PlayerCon (Game|GetPlayerController 0)))
                        (switch int (Variables|/Game/Misoten/BP/BP_PractiseDrift_PlayerCon.BP_PractiseDrift_PlayerCon_C|GetGearStairs _asbp_practise_drift_player_con_2)
                          (:Default
                            (Variables|Default|SetGearFloatFlg 2e+02 :!label _label))
                          (:0
                            (goto _label))
                          (:1
                            (Variables|Default|SetGearFloatFlg 3e+02))
                          (:2
                            (Variables|Default|SetGearFloatFlg 5e+02))
                          (:3
                            (Variables|Default|SetGearFloatFlg 7e+02))
                          (:4
                            (Variables|Default|SetGearFloatFlg 9e+02)))
                        (Niagara|SpawnSystematLocation "/Game/Misoten/Assets/EFF/EFF_Hit_Chase/NS_Hit_Chase.NS_Hit_Chase" (Math|Vector|MakeVector (.x (+ _location (* (Math|Vector|GetForwardVector _rotation) (Variables|Default|GetGearFloatFlg)))) (.y (+ _location (* (Math|Vector|GetForwardVector _rotation) (Variables|Default|GetGearFloatFlg)))) (+ (.z (+ _location (* (Math|Vector|GetForwardVector _rotation) (Variables|Default|GetGearFloatFlg)))) 4e+02)) "0, 0, 0" "9.000000,9.000000,9.000000")
                        (if (<= (Variables|Default|GetHP) 0.0)
                          (Audio|PlaySoundatLocation "/Game/Misoten/BP/Audio/SE/Enemy/BOSS/MS_NomalBikeHit.MS_NomalBikeHit" "0, 0, 0" "0, 0, 0" 1.0 1.0 0.0 0 0 0 0 :!label _label_2)
                          (else
                            (bind _returnvalue_3 (Rendering|Material|CreateDynamicMaterialInstance (Variables|Character|GetMesh) 0 0 "None" :!class /Script/Engine.PrimitiveComponent))
                            (Variables|Default|SetMaterialvariavel _returnvalue_3)
                            (bind _新規track_2 (Timeline|タイムライン PlayFromStart)
                              (:Update
                                (Rendering|Material|SetScalarParameterValue (Variables|Default|GetMaterialvariavel) "BlinkColor_Mult" _新規track_2 :!class /Script/Engine.MaterialInstanceDynamic)
                                (bind _returnvalue_4 (Rendering|Material|CreateDynamicMaterialInstance (Variables|Default|GetBOSSPanda) 1 0 "None" :!class /Script/Engine.PrimitiveComponent))
                                (Variables|Default|SetMaterialvariavel_2 _returnvalue_4)
                                (bind _新規track_2_2 (Timeline|タイムライン_0 PlayFromStart)
                                  (:Update
                                    (Utilities|FlowControl|Sequence
                                      (:then_0
                                        (Utilities|FlowControl|DoOnce false :!label _label_3
                                          (:Completed
                                            (goto _label_2))))
                                      (:then_1
                                        (Rendering|Material|SetScalarParameterValue (Variables|Default|GetMaterialvariavel_2) "BlinkColor_Mult" _新規track_2_2 :!class /Script/Engine.MaterialInstanceDynamic))))
                                  (:Finished
                                    (goto _label_3 Reset)))))))))))))))))))

(event Custom|PitchAttackEvent
  ;[1 1 1] ピンチの時の攻撃イベント
  (Utilities|FlowControl|DoOnce false :!label _label
    (:Completed
      (bind _asabp_bosspanda_chase (Utilities|Casting|CastToABP_BOSSPanda_Chase (Components|SkeletalMesh|GetAnimInstance (Variables|Default|GetBOSSPanda))))
      (Variables|/Game/Misoten/BP/Misoten_Enemy/Enemy/Boss/ABP_BOSSPanda_Chase.ABP_BOSSPanda_Chase_C|SetBOSSPand_AttackFlg _asabp_bosspanda_chase true)
      (bind _asabp_model_bossbike (Utilities|Casting|CastToABP_Model_BOSSBike (Components|SkeletalMesh|GetAnimInstance (Variables|Character|GetMesh))))
      (Variables|/Game/Misoten/BP/Misoten_Enemy/Enemy/Boss/ABP_Model_BOSSBike.ABP_Model_BOSSBike_C|SetBossBikePitchAttakFlg _asabp_model_bossbike true)
      (Timeline|タイムライン_2 PlayFromStart
        (:Finished
          (Game|SpawnActorfromClass "/Game/Misoten/BP/Misoten_Enemy/Enemy/Boss/BP_Drum_Chase.BP_Drum_Chase_C" (Math|Transform|MakeTransform (Transformation|GetWorldLocation (Variables|Default|GetThrowPoint)) "0, 0, 0" "1.000000,1.000000,1.000000") "Undefined" "MultiplyWithRoot" 0 0)
          (goto _label Reset))))))

(event Custom|AttackEvent
  ;[1 1 1] 通常時の攻撃イベント
  (Utilities|FlowControl|DoOnce false :!label _label
    (:Completed
      (bind _asabp_bosspanda_chase (Utilities|Casting|CastToABP_BOSSPanda_Chase (Components|SkeletalMesh|GetAnimInstance (Variables|Default|GetBOSSPanda))))
      (Variables|/Game/Misoten/BP/Misoten_Enemy/Enemy/Boss/ABP_BOSSPanda_Chase.ABP_BOSSPanda_Chase_C|SetAttackFlg _asabp_bosspanda_chase true)
      (bind _asabp_model_bossbike (Utilities|Casting|CastToABP_Model_BOSSBike (Components|SkeletalMesh|GetAnimInstance (Variables|Character|GetMesh))))
      (Variables|/Game/Misoten/BP/Misoten_Enemy/Enemy/Boss/ABP_Model_BOSSBike.ABP_Model_BOSSBike_C|SetBOSSBikeAttackFlg _asabp_model_bossbike true)
      (Timeline|タイムライン_1 PlayFromStart
        (:Finished
          (Components|Activation|Activate (Variables|Default|GetNS_Throw_Before) true)
          (Game|SpawnActorfromClass "/Game/Misoten/BP/Misoten_Enemy/Enemy/Boss/BP_Drum_Chase.BP_Drum_Chase_C" (Math|Transform|MakeTransform (Transformation|GetWorldLocation (Variables|Default|GetThrowPoint)) "0, 0, 0" "1.000000,1.000000,1.000000") "Undefined" "MultiplyWithRoot" 0 0)
          (goto _label Reset))))))

(event Custom|HitStartEvent
  (bind _returnvalue (Game|Player|GetPlayerPawn 0))
  (bind _returnvalue_2 (Transformation|GetActorTransform _returnvalue))
  (bind (_location _rotation) (Math|Transform|BreakTransform _returnvalue_2))
  ;[1 1 1] ボスにヒットした時の詳細な処理
  ;;[1 1 1] プレイヤーが停止してる時に行う処理
  (Utilities|FlowControl|DoOnce false) ; enters at Reset
)

(event Custom|AttackFinishEvent
  ;[1 1 1] ボスが攻撃する時の処理
  (bind _asabp_bosspanda_chase (Utilities|Casting|CastToABP_BOSSPanda_Chase (Components|SkeletalMesh|GetAnimInstance (Variables|Default|GetBOSSPanda))))
  (if (not (Variables|/Game/Misoten/BP/Misoten_Enemy/Enemy/Boss/ABP_BOSSPanda_Chase.ABP_BOSSPanda_Chase_C|GetAttackFlg _asabp_bosspanda_chase))
    (if (not (Variables|/Game/Misoten/BP/Misoten_Enemy/Enemy/Boss/ABP_BOSSPanda_Chase.ABP_BOSSPanda_Chase_C|GetBOSSPand_AttackFlg _asabp_bosspanda_chase))
      (bind _asabp_model_bossbike (Utilities|Casting|CastToABP_Model_BOSSBike (Components|SkeletalMesh|GetAnimInstance (Variables|Character|GetMesh))))
      (if (not (Variables|/Game/Misoten/BP/Misoten_Enemy/Enemy/Boss/ABP_Model_BOSSBike.ABP_Model_BOSSBike_C|GetBOSSBikeAttackFlg _asabp_model_bossbike))
        (if (not (Variables|/Game/Misoten/BP/Misoten_Enemy/Enemy/Boss/ABP_Model_BOSSBike.ABP_Model_BOSSBike_C|GetBossBikePitchAttakFlg _asabp_model_bossbike))
          (bind _asabp_model_bossbike_2 (Utilities|Casting|CastToABP_Model_BOSSBike (Components|SkeletalMesh|GetAnimInstance (Variables|Character|GetMesh))))
          (if (Variables|/Game/Misoten/BP/Misoten_Enemy/Enemy/Boss/ABP_Model_BOSSBike.ABP_Model_BOSSBike_C|GetBOSSBikePitchFlg _asabp_model_bossbike_2)
            ;;[1 1 1] ピンチになってるときの攻撃イベント
            (CallFunction|PitchAttackEvent)
            (else
              ;;[1 1 1] 通常のときの攻撃イベント
              (CallFunction|AttackEvent))))))))

(event Custom|FrontEvent
  (bind _capsulecomponent (Variables|Collision|GetCapsuleComponent))
  (bind _returnvalue (Transformation|GetWorldLocation _capsulecomponent))
  ;[1 1 1] ボスを中心に戻す処理
  (if (not (Variables|Default|GetFrontLine))
    (if (Math|Float|InRange(Float) (.yaw (Transformation|GetWorldRotation (Variables|Collision|GetCapsuleComponent))) -0.001 0.1)
      (Transformation|SetActorLocation (Math|Vector|MakeVector (.x _returnvalue) (Math|Float|Lerp (.y _returnvalue) 0.0 0.02) (.z _returnvalue)) false false))))

(event EventBeginPlay
  ;[1 1 1] データをとってくる処理
  (Utilities|FlowControl|Sequence
    (:then_0
      (bind _returnvalue (Utilities|GetDataTableRow "/Game/Misoten/BP/DataTable/BossChaseStatusDataTable.BossChaseStatusDataTable" "Stage1")
        (:then
          (Variables|Default|SetHP (.hp _returnvalue))
          (Variables|Default|SetAttackTime (.attacktime _returnvalue))
          (Variables|Default|SetOut%20Row%20Throwing%20Speed (.bulletspeed _returnvalue))
          (Variables|Default|SetPitchHP (.pitchhp _returnvalue))
          (Variables|Default|SetNowSpeed 2.1e+02))
        (:RowNotFound
          (Development|PrintString "Error"))))
    (:then_1
      (bind _asabp_model_bossbike (Utilities|Casting|CastToABP_Model_BOSSBike (Components|SkeletalMesh|GetAnimInstance (Variables|Character|GetMesh))))
      (Variables|/Game/Misoten/BP/Misoten_Enemy/Enemy/Boss/ABP_Model_BOSSBike.ABP_Model_BOSSBike_C|SetBOSSBikeDushFlg _asabp_model_bossbike true))))

(event EventTick
  (params (DeltaSeconds :type Float%20%28single-precision%29))
  (if (Variables|Default|GetWigetFlg)
    (Utilities|FlowControl|Sequence
      (:then_0
        (bind _asabp_bosspanda_chase (Utilities|Casting|CastToABP_BOSSPanda_Chase (Components|SkeletalMesh|GetAnimInstance (Variables|Default|GetBOSSPanda))))
        (if (Variables|/Game/Misoten/BP/Misoten_Enemy/Enemy/Boss/ABP_BOSSPanda_Chase.ABP_BOSSPanda_Chase_C|GetLastAnimFinishFlg _asabp_bosspanda_chase)
          (Utilities|FlowControl|DoOnce false
            (:Completed
              (Audio|Components|Audio|Play (Variables|Default|GetMS_SE_ResultExplosion1) 0.0)
              (Audio|Components|Audio|Play (Variables|Default|GetMS_SE_ResultExplosion2_Cue) 0.0)
              ;[1 1 1] 爆発エフェクトを出す
              (Niagara|SpawnSystematLocation "/Game/Misoten/Assets/EFF/EFF_Explosion_v3/NS_Explosion_Toon.NS_Explosion_Toon" (Transformation|GetActorLocation))
              ;[1 1 1] カメラを揺らす
              (Game|Feedback|ClientStartCameraShake (Game|GetPlayerController 0) "/Game/Misoten/BP/BP_BOSSMyCameraShake.BP_BOSSMyCameraShake_C" 1.0 "CameraLocal" "0, 0, 0")))
          (else
            ;[1 1 1] ボスが生きているときの処理
            ;;[1 1 1] スプラインに沿うように移動
            (Transformation|AddActorWorldOffset (* (Transformation|GetActorForwardVector) (Variables|Default|GetNowSpeed)) false true :!label _label)
            (Utilities|FlowControl|DoOnce false
              (:Completed
                ;;[1 1 1] ボスのエンジン音再生
                (Audio|Components|Audio|Play (Variables|Default|GetMS_BossEngine_Cue) 0.0))))))
      (:then_1
        ;[1 1 1] 滑る音を出す処理
        (bind _asabp_bosspanda_chase_2 (Utilities|Casting|CastToABP_BOSSPanda_Chase (Components|SkeletalMesh|GetAnimInstance (Variables|Default|GetBOSSPanda))))
        (if (Variables|/Game/Misoten/BP/Misoten_Enemy/Enemy/Boss/ABP_BOSSPanda_Chase.ABP_BOSSPanda_Chase_C|GetLastStartFlg _asabp_bosspanda_chase_2)
          (Utilities|FlowControl|DoOnce false
            (:Completed
              (Audio|Components|Audio|Play (Variables|Default|GetTitle_Brake) 0.0)))
          (else
            (Audio|Components|Audio|Stop (Variables|Default|GetTitle_Brake)))))
      (:then_2
        ;[1 1 1] 爆発後の炎の音を消す
        (bind _asbp_practise_drift_player_con (Utilities|Casting|CastToBP_PractiseDrift_PlayerCon (Game|GetPlayerController 0)))
        (if (Variables|/Game/Misoten/BP/BP_PractiseDrift_PlayerCon.BP_PractiseDrift_PlayerCon_C|GetResultRankingFlg _asbp_practise_drift_player_con)
          (Audio|Components|Audio|Stop (Variables|Default|GetMS_SE_ResultExplosion2_Cue)))))
    (else
      (Utilities|FlowControl|Sequence
        (:then_0
          ;[1 1 1] ボスがHP死んだか判断
          (bind _asabp_model_bossbike (Utilities|Casting|CastToABP_Model_BOSSBike (Components|SkeletalMesh|GetAnimInstance (Variables|Character|GetMesh))))
          (if (Variables|/Game/Misoten/BP/Misoten_Enemy/Enemy/Boss/ABP_Model_BOSSBike.ABP_Model_BOSSBike_C|GetBOSSBikeFinishFlg _asabp_model_bossbike)
            ;[1 1 1] ボスが死んだときの処理
            ;;[1 1 1] ボスにカメラを向ける
            (Game|Player|SetViewTargetwithBlend (Game|GetPlayerController 0) (Components|GetOwner (Variables|Default|GetCamera)) 0.0 "VTBlend_Linear" 0.0 false)
            ;;;[1 1 1] ウィジェット表示フラグ
            (Variables|Default|SetWigetFlg true)
            (else
              (bind _asabp_bosspanda_chase_3 (Utilities|Casting|CastToABP_BOSSPanda_Chase (Components|SkeletalMesh|GetAnimInstance (Variables|Default|GetBOSSPanda))))
              (if (not (Variables|/Game/Misoten/BP/Misoten_Enemy/Enemy/Boss/ABP_BOSSPanda_Chase.ABP_BOSSPanda_Chase_C|GetLastAnimFinishFlg _asabp_bosspanda_chase_3))
                (goto _label)))))
        (:then_1
          ;[1 1 1] 攻撃してよいか判断
          (bind _asabp_model_bossbike_2 (Utilities|Casting|CastToABP_Model_BOSSBike (Components|SkeletalMesh|GetAnimInstance (Variables|Character|GetMesh))))
          (if (not (Variables|/Game/Misoten/BP/Misoten_Enemy/Enemy/Boss/ABP_Model_BOSSBike.ABP_Model_BOSSBike_C|GetDamageFlg _asabp_model_bossbike_2))
            (if (Variables|/Game/Misoten/BP/Misoten_Enemy/Enemy/Boss/ABP_Model_BOSSBike.ABP_Model_BOSSBike_C|GetBOSSBikeDushFlg _asabp_model_bossbike_2)
              (CallFunction|AttackFinishEvent))))
        (:then_2
          ;[1 1 1] ピンチになるか判断
          ;;[1 1 1] 現在ピンチか判断
          (if (<= (Variables|Default|GetHP) (Variables|Default|GetPitchHP))
            (bind _asabp_bosspanda_chase_4 (Utilities|Casting|CastToABP_BOSSPanda_Chase (Components|SkeletalMesh|GetAnimInstance (Variables|Default|GetBOSSPanda))))
            (if (not (Variables|/Game/Misoten/BP/Misoten_Enemy/Enemy/Boss/ABP_BOSSPanda_Chase.ABP_BOSSPanda_Chase_C|GetDamageFlg _asabp_bosspanda_chase_4))
              (if (not (Variables|/Game/Misoten/BP/Misoten_Enemy/Enemy/Boss/ABP_BOSSPanda_Chase.ABP_BOSSPanda_Chase_C|GetPitchDamageFlg _asabp_bosspanda_chase_4))
                (Utilities|FlowControl|DoOnce false
                  (:Completed
                    (bind _asabp_model_bossbike_3 (Utilities|Casting|CastToABP_Model_BOSSBike (Components|SkeletalMesh|GetAnimInstance (Variables|Character|GetMesh))))
                    (Variables|/Game/Misoten/BP/Misoten_Enemy/Enemy/Boss/ABP_Model_BOSSBike.ABP_Model_BOSSBike_C|SetBOSSBikePitchFlg _asabp_model_bossbike_3 true)
                    (bind _asabp_bosspanda_chase_5 (Utilities|Casting|CastToABP_BOSSPanda_Chase (Components|SkeletalMesh|GetAnimInstance (Variables|Default|GetBOSSPanda))))
                    (Variables|/Game/Misoten/BP/Misoten_Enemy/Enemy/Boss/ABP_BOSSPanda_Chase.ABP_BOSSPanda_Chase_C|SetPintchFlg _asabp_bosspanda_chase_5 true)
                    ;;[1 1 1] ボスのバイクのエンジン音を変える為停止
                    (Audio|Components|Audio|Stop (Variables|Default|GetMS_BossEngine_Cue))
                    (Components|Activation|SetActive (Variables|Default|GetNS_BikeStagger) true true)))))))
        (:then_3
          ;[1 1 1] ボスの体力が0になった時の処理
          (if (<= (Variables|Default|GetHP) 0.0)
            (Utilities|FlowControl|DoOnce false
              (:Completed
                (bind _asabp_model_bossbike_4 (Utilities|Casting|CastToABP_Model_BOSSBike (Components|SkeletalMesh|GetAnimInstance (Variables|Character|GetMesh))))
                (Variables|/Game/Misoten/BP/Misoten_Enemy/Enemy/Boss/ABP_Model_BOSSBike.ABP_Model_BOSSBike_C|SetPitchDamageFlg _asabp_model_bossbike_4 false)
                (Variables|/Game/Misoten/BP/Misoten_Enemy/Enemy/Boss/ABP_Model_BOSSBike.ABP_Model_BOSSBike_C|SetBOSSBikeFinishFlg _asabp_model_bossbike_4 true)
                (bind _asabp_bosspanda_chase_6 (Utilities|Casting|CastToABP_BOSSPanda_Chase (Components|SkeletalMesh|GetAnimInstance (Variables|Default|GetBOSSPanda))))
                (Variables|/Game/Misoten/BP/Misoten_Enemy/Enemy/Boss/ABP_BOSSPanda_Chase.ABP_BOSSPanda_Chase_C|SetFinishFlg _asabp_bosspanda_chase_6 true)
                (Variables|/Game/Misoten/BP/Misoten_Enemy/Enemy/Boss/ABP_BOSSPanda_Chase.ABP_BOSSPanda_Chase_C|SetPitchDamageFlg _asabp_bosspanda_chase_6 false)))))
        (:then_4
          (CallFunction|DownSpeedEventLEFTLIGHT)
          (CallFunction|HitDownEvent)
          ;[1 1 1] プレイヤーの速度がなくなった時にフラグ解除する処理
          (bind _asbp_practise_drift_player_con_2 (Utilities|Casting|CastToBP_PractiseDrift_PlayerCon (Game|GetPlayerController 0)))
          (if (< (Variables|/Game/Misoten/BP/BP_PractiseDrift_PlayerCon.BP_PractiseDrift_PlayerCon_C|GetNowSpeed _asbp_practise_drift_player_con_2) 0.0)
            (Variables|Default|SetHit2Flg false)
            (Variables|Default|SetCount 0)
            (Variables|Default|SetHitFlg false)
            (Variables|Default|SetCountHit 0)
            (bind _asabp_bosspanda_chase_7 (Utilities|Casting|CastToABP_BOSSPanda_Chase (Components|SkeletalMesh|GetAnimInstance (Variables|Default|GetBOSSPanda))))
            (Variables|/Game/Misoten/BP/Misoten_Enemy/Enemy/Boss/ABP_BOSSPanda_Chase.ABP_BOSSPanda_Chase_C|SetDamageFlg _asabp_bosspanda_chase_7 false)
            (Variables|/Game/Misoten/BP/Misoten_Enemy/Enemy/Boss/ABP_BOSSPanda_Chase.ABP_BOSSPanda_Chase_C|SetPitchDamageFlg _asabp_bosspanda_chase_7 false)
            (bind _asabp_model_bossbike_5 (Utilities|Casting|CastToABP_Model_BOSSBike (Components|SkeletalMesh|GetAnimInstance (Variables|Character|GetMesh))))
            (Variables|/Game/Misoten/BP/Misoten_Enemy/Enemy/Boss/ABP_Model_BOSSBike.ABP_Model_BOSSBike_C|SetDamageFlg _asabp_model_bossbike_5 false)
            (Variables|/Game/Misoten/BP/Misoten_Enemy/Enemy/Boss/ABP_Model_BOSSBike.ABP_Model_BOSSBike_C|SetPitchDamageFlg _asabp_model_bossbike_5 false)
            (CallFunction|HitStartEvent)))
        (:then_5
          ;[1 1 1] 徐々に元の速度に戻す
          (if (not (<= (Variables|Default|GetNowSpeed) 9e+01))
            (bind _result (Math|Float|DecrementFloat (Variables|Default|GetNowSpeed))
              (:%20%20
                (Variables|Default|SetNowSpeed _result)))))
        (:then_6
          ;[1 1 1] 中心にボスを戻すイベント
          (CallFunction|FrontEvent))))))

(fn ConstructionScript)

(fn StartMoveSupportSpline
  (params (Input :type Spline%20Component%20Object%20Reference))
  (Variables|Default|SetMoveSupportSline Input)
  (CallFunction|SplineSupportStart))