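; BP_Drum_Chase is a hittable drum that the drift player's pawn can knock away to score points.
; Its first unpaused box overlap with the pawn adds drum score and applies speed-scaled impulses, blending pawn heading with direction to the drum.
; The overlap also plays a drum sound through a DoOnce that Tick re-arms after a delay.
; Player controller pause events freeze its time dilation and block hits.
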(event OnComponentBeginOverlap(Box)
  (params (OverlappedComponent :type Primitive%20Component%20Object%20Reference) (OtherActor :type Actor%20Object%20Reference) (OtherComp :type Primitive%20Component%20Object%20Reference) (OtherBodyIndex :type Integer) (bFromSweep :type Boolean) (SweepResult :type Hit%20Result%20Structure%20%28by%20ref%29))
  (bind _staticmesh (Variables|Default|GetStaticMesh))
  (if (not (Variables|Default|GetIsHit))
    (if (not (Variables|Default|GetIsPause))
      (bind _asbp_practise_drift_pawn (Utilities|Casting|CastToBP_PractiseDrift_Pawn OtherActor))
      (Utilities|FlowControl|Sequence
        (:then_0
          (Default|AddScoreDrum (Variables|/Game/Misoten/BP/BP_PractiseDrift_Pawn.BP_PractiseDrift_Pawn_C|GetBP_PlayerState _asbp_practise_drift_pawn))
          (Variables|Default|SetIsHit true)
          (bind _asbp_practise_drift_player_con (Utilities|Casting|CastToBP_PractiseDrift_PlayerCon (Game|GetPlayerController 0)))
          (Variables|Default|SetImpactPoint (Math|Transform|InverseTransformLocation (Transformation|GetActorTransform) (.ImpactPoint (Collision|BreakHitResult SweepResult))))
          (Variables|Default|SetImpulse (* (Math|Vector|Lerp(Vector) (Transformation|GetActorForwardVector _asbp_practise_drift_pawn) (Math|Vector|Normalize (- (Transformation|GetActorLocation) (Transformation|GetActorLocation _asbp_practise_drift_pawn))) (Variables|Default|GetAlpha)) (* (Variables|/Game/Misoten/BP/BP_PractiseDrift_PlayerCon.BP_PractiseDrift_PlayerCon_C|GetNowSpeed _asbp_practise_drift_player_con) (Variables|Default|GetValue))))
          (Variables|Default|SetForce (* (Math|Vector|Lerp(Vector) (Transformation|GetActorForwardVector _asbp_practise_drift_pawn) (Math|Vector|Normalize (- (Transformation|GetActorLocation) (Transformation|GetActorLocation _asbp_practise_drift_pawn))) (Variables|Default|GetAlpha)) (* (Variables|/Game/Misoten/BP/BP_PractiseDrift_PlayerCon.BP_PractiseDrift_PlayerCon_C|GetNowSpeed _asbp_practise_drift_player_con) (Variables|Default|GetValue))))
          (Physics|AddImpulse _staticmesh (Variables|Default|GetImpulse) "None" false)
          (Physics|AddImpulseatLocation _staticmesh (Variables|Default|GetImpulse) (Variables|Default|GetImpactPoint) "None"))
        (:then_1
          (Utilities|FlowControl|DoOnce false
            (:Completed
              (Audio|PlaySoundatLocation "/Game/Misoten/BP/Audio/SE/MS_Drum_Cue.MS_Drum_Cue" (Transformation|GetActorLocation) "0, 0, 0" 0.35 1.0 0.0 0 0 0 0))))))))

(event Custom|SetCustomTimeDilationZero
  (Variables|Default|SetCustomTimeDilation 0.0)
  (Variables|Default|SetIsPause true))

(event Custom|SetCustomTimeDilationOne
  (Variables|Default|SetCustomTimeDilation 1.0)
  (Variables|Default|SetIsPause false))

(event EventBeginPlay
  (bind _asbp_practise_drift_player_con (Utilities|Casting|CastToBP_PractiseDrift_PlayerCon (Game|GetPlayerController 0)))
  (EventDispatchers|BindEventtoStartPause _asbp_practise_drift_player_con (delegate Custom|SetCustomTimeDilationZero))
  (EventDispatchers|BindEventtoStopPause _asbp_practise_drift_player_con (delegate Custom|SetCustomTimeDilationOne)))

(event EventTick
  (params (DeltaSeconds :type Float%20%28single-precision%29))
  (Utilities|FlowControl|Delay 1.0)
  (Utilities|FlowControl|DoOnce false) ; enters at Reset
)

(fn ConstructionScript)