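; BP_BOSSBullet_ColorCone is a projectile for BP_BOSS that flies in a straight line toward where the player was when it spawned.
; On BeginPlay it stores a point slightly above the player, the boss's BulletLocation and its OutRowThrowingSpeed.
; Tick moves it along that direction without sweep or delta-time scaling.
; The Reflection event sends it back by making the old start the target and the supplied point the new start.
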(event Custom|Reflection
  (params (Start :type Vector))
  (Variables|Default|SetTargetLocation (Variables|Default|GetStartLocation))
  (Variables|Default|SetStartLocation Start))

(event EventBeginPlay
  (bind _returnvalue (Game|GetPlayerCharacter 0))
  (bind _returnvalue_2 (Transformation|GetActorLocation _returnvalue))
  (Variables|Default|SetTargetLocation (Math|Vector|MakeVector (.x _returnvalue_2) (.y _returnvalue_2) (+ (.z _returnvalue_2) 5e+01)))
  (bind _returnvalue_3 (Actor|GetActorOfClass "/Game/Misoten/BP/Misoten_Enemy/Enemy/Boss/BP_BOSS.BP_BOSS_C"))
  (Variables|Default|SetStartLocation (Transformation|GetWorldLocation (Variables|/Game/Misoten/BP/Misoten_Enemy/Enemy/Boss/BP_BOSS.BP_BOSS_C|GetBulletLocation _returnvalue_3)))
  (Variables|Default|SetSpeed (Variables|/Game/Misoten/BP/Misoten_Enemy/Enemy/Boss/BP_BOSS.BP_BOSS_C|GetOut%20Row%20Throwing%20Speed _returnvalue_3)))

(event EventTick
  (params (DeltaSeconds :type Float%20%28single-precision%29))
  (Transformation|AddActorWorldOffset (* (Math|Vector|Normalize (- (Variables|Default|GetTargetLocation) (Variables|Default|GetStartLocation))) (Variables|Default|GetSpeed))))

(fn ConstructionScript)