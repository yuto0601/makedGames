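; BP_BOSSChase_Reflection is a projectile in the boss chase that travels toward the ReflectionPoint on BP_BOSSChase, apparently as a reflected attack.
; BeginPlay captures both positions and applies one RInterpTo step toward the target.
; Tick moves it along that fixed direction by Speed each frame, without delta-time scaling or sweep.
; Overlapping BP_Mesh_Finish replaces it with a BP_BOSSChase_Drum, while hitting the boss only prints a debug message.
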(event OnComponentBeginOverlap(Box)
  (params (OverlappedComponent :type Primitive%20Component%20Object%20Reference) (OtherActor :type Actor%20Object%20Reference) (OtherComp :type Primitive%20Component%20Object%20Reference) (OtherBodyIndex :type Integer) (bFromSweep :type Boolean) (SweepResult :type Hit%20Result%20Structure%20%28by%20ref%29))
  (Utilities|FlowControl|Sequence
    (:then_0
      (Utilities|Casting|CastToBP_Mesh_Finish OtherActor)
      (Utilities|FlowControl|DoOnce false
        (:Completed
          (Game|SpawnActorfromClass "/Game/Misoten/BP/Misoten_Enemy/Enemy/Boss/BP_BOSSChase_Drum.BP_BOSSChase_Drum_C" (Math|Transform|MakeTransform (Transformation|GetActorLocation) (Transformation|GetActorRotation) "1.000000,1.000000,1.000000") "Undefined" "MultiplyWithRoot" 0 0)
          (Actor|DestroyActor))))
    (:then_1
      (Utilities|Casting|CastToBP_BOSSChase OtherActor)
      (Utilities|FlowControl|DoOnce false
        (:Completed
          (Development|PrintString "ボスにヒット"))))))

(event EventBeginPlay
  (Variables|Default|SetReflectionLocation (Transformation|GetActorLocation))
  (bind _returnvalue (Actor|GetActorOfClass "/Game/Misoten/BP/Misoten_Enemy/Enemy/Boss/BP_BOSSChase.BP_BOSSChase_C"))
  (Variables|Default|SetTargetLocation (Transformation|GetWorldLocation (Variables|/Game/Misoten/BP/Misoten_Enemy/Enemy/Boss/BP_BOSSChase.BP_BOSSChase_C|GetReflectionPoint _returnvalue)))
  (Transformation|SetActorRotation (Math|Interpolation|RInterpTo (Transformation|GetActorRotation) (Math|Rotator|FindLookatRotation (Transformation|GetActorLocation) (Transformation|GetWorldLocation (Variables|/Game/Misoten/BP/Misoten_Enemy/Enemy/Boss/BP_BOSSChase.BP_BOSSChase_C|GetReflectionPoint _returnvalue))) (Utilities|Time|GetWorldDeltaSeconds) 0.0)))

(event EventTick
  (params (DeltaSeconds :type Float%20%28single-precision%29))
  (Transformation|AddActorWorldOffset (* (Math|Vector|Normalize (- (Variables|Default|GetTargetLocation) (Variables|Default|GetReflectionLocation))) (Variables|Default|GetSpeed))))

(fn ConstructionScript)