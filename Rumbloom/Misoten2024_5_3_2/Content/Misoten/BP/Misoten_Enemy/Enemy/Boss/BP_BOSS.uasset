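; Panda boss that drops in at its spawner, loads data-table stats, and faces the player, slamming or throwing by distance on a timer.
; While it is stunned, the player's drift spline encloses it if the summed signed angles around it reach a full turn.
; Completed enclosure scores and revives it from stun.
; Events also handle three cycling minion waves, hit blinking, pause via time dilation, and death into a chase sequence.
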(event OnComponentHit(Box)
  (params (HitComponent :type Primitive%20Component%20Object%20Reference) (OtherActor :type Actor%20Object%20Reference) (OtherComp :type Primitive%20Component%20Object%20Reference) (NormalImpulse :type Vector :default "0, 0, 0") (Hit :type Hit%20Result%20Structure%20%28by%20ref%29))
  ;[1 1 1] プレイヤーとボスが当たった時
  (bind _asbp_practise_drift_pawn (Utilities|Casting|CastToBP_PractiseDrift_Pawn OtherActor))
  (Default|HitReaction _asbp_practise_drift_pawn))

(event Custom|SpawnEnemy
  ;[1 1 1] 雑魚敵のスポーン
  (if (== 1.0 (Variables|Default|GetWaveCount))
    (Variables|Default|SetWaveCount (+ (Variables|Default|GetWaveCount) 1.0))
    (bind _outactors (Actor|GetAllActorsOfClass "/Game/Misoten/BP/Misoten_Enemy/Enemy/Boss/BP_Sponer1.BP_Sponer1_C"))
    (for _array_element _outactors
      (Niagara|SpawnSystematLocation "/Game/Misoten/Assets/EFF/EFF_Enemy_Spawn/NS_Enemy_Spawn.NS_Enemy_Spawn" (Transformation|GetActorLocation _array_element) "0, 0, 0" "2.000000,2.000000,2.000000")
      (Game|SpawnActorfromClass "/Game/Misoten/BP/Misoten_Enemy/Enemy/Boss/BP_BOSSEnemy.BP_BOSSEnemy_C" (Math|Transform|MakeTransform (Transformation|GetActorLocation _array_element) "0.000000,180.000000,0.000000" "1.000000,1.000000,1.000000") "Undefined" "MultiplyWithRoot" 0 0))
    (elif (== 2.0 (Variables|Default|GetWaveCount))
      (Variables|Default|SetWaveCount (+ (Variables|Default|GetWaveCount) 1.0))
      (bind _outactors_2 (Actor|GetAllActorsOfClass "/Game/Misoten/BP/Misoten_Enemy/Enemy/Boss/BP_Sponer2.BP_Sponer2_C"))
      (for _array_element_2 _outactors_2
        (Niagara|SpawnSystematLocation "/Game/Misoten/Assets/EFF/EFF_Enemy_Spawn/NS_Enemy_Spawn.NS_Enemy_Spawn" (Transformation|GetActorLocation _array_element_2) "0, 0, 0" "2.000000,2.000000,2.000000")
        (Game|SpawnActorfromClass "/Game/Misoten/BP/Misoten_Enemy/Enemy/Boss/BP_BOSSEnemy.BP_BOSSEnemy_C" (Math|Transform|MakeTransform (Transformation|GetActorLocation _array_element_2) "0.000000,180.000000,0.000000" "1.000000,1.000000,1.000000") "Undefined" "MultiplyWithRoot" 0 0))
      (elif (== 3.0 (Variables|Default|GetWaveCount))
        (Variables|Default|SetWaveCount 1.0)
        (bind _outactors_3 (Actor|GetAllActorsOfClass "/Game/Misoten/BP/Misoten_Enemy/Enemy/Boss/BP_Sponer3.BP_Sponer3_C"))
        (for _array_element_3 _outactors_3
          (Niagara|SpawnSystematLocation "/Game/Misoten/Assets/EFF/EFF_Enemy_Spawn/NS_Enemy_Spawn.NS_Enemy_Spawn" (Transformation|GetActorLocation _array_element_3) "0, 0, 0" "2.000000,2.000000,2.000000")
          (Game|SpawnActorfromClass "/Game/Misoten/BP/Misoten_Enemy/Enemy/Boss/BP_BOSSEnemy.BP_BOSSEnemy_C" (Math|Transform|MakeTransform (Transformation|GetActorLocation _array_element_3) "0.000000,180.000000,0.000000" "1.000000,1.000000,1.000000") "Undefined" "MultiplyWithRoot" 0 0))))))

(event Custom|ShockWave
  ;[1 1 1] 攻撃
  (Animation|Montage|PlayMontage (Variables|Character|GetMesh) "/Game/Misoten/Assets/Models/BossPanda/Anim_BossPanda/Anim_BossPanda_SlamAttack_Montage.Anim_BossPanda_SlamAttack_Montage"))

(event Custom|Revival
  ;[1 1 1] 囲まれたとき
  (Animation|Montage|PlayMontage (Variables|Character|GetMesh) "/Game/Misoten/Assets/Models/BossPanda/Anim_BossPanda/Anim_BossPanda_Stan_Out_Montage.Anim_BossPanda_Stan_Out_Montage"))

(event Custom|Death
  ;[1 1 1] ３回囲まれた時
  (CallFunction|ChaseSequence)
  (Actor|DestroyActor))

(event Custom|ApplyColor
  ;[1 1 1] はじき返された弾に当たった時
  (bind _returnvalue (Rendering|Material|CreateDynamicMaterialInstance (Variables|Character|GetMesh) 1 "/Game/Misoten/Assets/Models/BossPanda/M_BossPanda_First.M_BossPanda_First" "None" :!class /Script/Engine.PrimitiveComponent))
  (bind _新規track_2 (Timeline|タイムライン PlayFromStart)
    (:Update
      (Rendering|Material|SetScalarParameterValue _returnvalue "BlinkColor_Mult" _新規track_2 :!class /Script/Engine.MaterialInstanceDynamic))))

(event Custom|BOSSEncloseCompleted
  (if (Variables|Default|GetEnclosed)
    (CallFunction|Revival)
    (Variables|Default|SetEnclosed false)
    (Components|Activation|SetActive (Variables|Default|GetChargeEFF) false false)
    (bind _asbp_practise_drift_pawn (Utilities|Casting|CastToBP_PractiseDrift_Pawn (Game|Player|GetPlayerPawn 0)))
    (Default|AddScoreBOSSEnclose (Variables|/Game/Misoten/BP/BP_PractiseDrift_Pawn.BP_PractiseDrift_Pawn_C|GetBP_PlayerState _asbp_practise_drift_pawn))))

(event Custom|EncloseEvent
  (Variables|Default|SetEnclosed true)
  (Default|BOSSEncloseEvent (Variables|Default|GetAs%20BP%20Practise%20Drift%20Player%20Con))
  (Components|Activation|SetActive (Variables|Default|GetChargeEFF) true false))

(event Custom|EncloseCompulsionStop
  (Variables|Default|SetEnclosed false)
  (Components|Activation|SetActive (Variables|Default|GetChargeEFF) false false)
  (Default|EncloseCompulsionStop (Variables|Default|GetAs%20BP%20Practise%20Drift%20Player%20Con)))

(event Custom|Attack
  ;[1 1 1] 攻撃
  (Audio|PlaySound2D "/Game/Misoten/BP/Audio/SE/Enemy/BOSS/MS_BossAttack.MS_BossAttack" 0.8 1.0 0.0 0 0)
  (bind _returndistance (CallFunction|Distance))
  (if (<= _returndistance (Variables|Default|GetOut%20Row%20Attack%20Range))
    (CallFunction|ShockWave)
    (else
      (CallFunction|Throw))))

(event Custom|Stan
  ;[1 1 1] はじき返された弾に当たった時
  (Animation|Montage|PlayMontage (Variables|Character|GetMesh) "/Game/Misoten/Assets/Models/BossPanda/Anim_BossPanda/Anim_BossPanda_Stun_Montage.Anim_BossPanda_Stun_Montage"
    (:then
      (Variables|Default|SetisStanNaw true))))

(event Custom|EncloseJudgeEvent
  (params (SplineObject :type Spline%20Component%20Object%20Reference))
  ;[1 1 1] 囲まれたとき
  (if (<= (Math|Vector|VectorLength (- (Transformation|GetActorLocation (Variables|Default|GetAs%20BP%20Practise%20Drift%20Pawn)) (Transformation|GetActorLocation))) (Variables|Default|GetEffectiveDistance))
    (Utilities|IsValid SplineObject
      (:Is%20Valid
        (bind _resultout (CallFunction|InternalandExternalJudgments SplineObject))
        (if (and (>= _resultout (* (Math|Trig|GetPI) 2.0)) (Variables|Default|GetisStanNaw))
          (CallFunction|EncloseEvent))))))

(event Custom|Throw
  ;[1 1 1] 攻撃
  (Animation|Montage|PlayMontage (Variables|Character|GetMesh) "/Game/Misoten/Assets/Models/BossPanda/Anim_BossPanda/Anim_BossPanda_ThrowAttack_Montage.Anim_BossPanda_ThrowAttack_Montage"))

(event Custom|BulletDamage
  ;[1 1 1] はじき返された弾に当たった時
  (CallFunction|ApplyColor))

(event Custom|EnablePause
  (Variables|Default|SetIsPause true)
  (Variables|Default|SetCustomTimeDilation 0.0))

(event Custom|DisablePause
  (Variables|Default|SetIsPause false)
  (Variables|Default|SetCustomTimeDilation 1.0))

(event Custom|ChaseSequence
  ;[1 1 1] ３回囲まれた時
  (bind _returnvalue (Sequencer|Player|CreateLevelSequencePlayer "/Game/Misoten/Assets/Seqence/Sequence/Go_To_Chase_Sequence.Go_To_Chase_Sequence"))
  (Sequencer|Player|Play _returnvalue :!class /Script/MovieScene.MovieSceneSequencePlayer))

(event EventBeginPlay
  (Variables|Default|SetBOSSStageNaw true)
  (Utilities|FlowControl|Sequence
    (:then_0
      (|Data)
      (Animation|Montage|PlayMontage (Variables|Character|GetMesh) "/Game/Misoten/Assets/Models/BossPanda/Anim_BossPanda/Anim_BossPanda_Roar_Montage.Anim_BossPanda_Roar_Montage"
        (:then
          (bind _asbp_practise_drift_pawn (Utilities|Casting|CastToBP_PractiseDrift_Pawn (Game|Player|GetPlayerPawn 0)))
          (Variables|Default|SetAs%20BP%20Practise%20Drift%20Pawn _asbp_practise_drift_pawn)
          (EventDispatchers|BindEventtoEncloseJudge (Variables|Default|GetAs%20BP%20Practise%20Drift%20Pawn) (delegate Custom|EncloseJudgeEvent))
          (EventDispatchers|BindEventtoEncloseCompleted (Variables|Default|GetAs%20BP%20Practise%20Drift%20Pawn) (delegate Custom|BOSSEncloseCompleted))
          (Variables|Default|SetBOSSPandaMesh (Variables|Character|GetMesh))
          (bind _asbp_practise_drift_player_con (Utilities|Casting|CastToBP_PractiseDrift_PlayerCon (Game|GetPlayerController 0)))
          (bind _output_get (Variables|Default|SetAs%20BP%20Practise%20Drift%20Player%20Con _asbp_practise_drift_player_con))
          (EventDispatchers|BindEventtoStartPause _output_get (delegate Custom|EnablePause))
          (EventDispatchers|BindEventtoStopPause _output_get (delegate Custom|DisablePause)))))
    (:then_1
      (bind _returnvalue (Actor|GetActorOfClass "/Game/Misoten/BP/Misoten_Enemy/Enemy/Boss/BP_SponerBOSS.BP_SponerBOSS_C"))
      (bind _新規track_0 (Timeline|タイムライン_0 Play)
        (:Update
          (Transformation|SetActorLocation (Math|Vector|Lerp(Vector) (Transformation|GetActorLocation) (Transformation|GetActorLocation _returnvalue) _新規track_0) false false))
        (:Finished
          (Components|Activation|SetActive (Variables|Default|GetNS_PandaLanding) true false))))))

(event EventTick
  (params (DeltaSeconds :type Float%20%28single-precision%29))
  (bind _returnvalue (Transformation|GetActorLocation))
  (bind _returnvalue_2 (Game|GetPlayerCharacter 0))
  (bind _returnvalue_3 (Transformation|GetActorRotation))
  (bind _returnvalue_4 (Utilities|Time|GetWorldDeltaSeconds))
  (bind _out_row_attack_interval (Variables|Default|GetOut%20Row%20Attack%20Interval))
  (bind _returnvalue_5 (Transformation|GetActorLocation _returnvalue_2))
  (bind _returnvalue_6 (Math|Rotator|FindLookatRotation _returnvalue _returnvalue_5))
  (bind _returnvalue_7 (Math|Interpolation|RInterpTo _returnvalue_3 _returnvalue_6 _returnvalue_4 0.0))
  (if (not (Variables|Default|GetIsPause))
    (if (not (Variables|Default|GetisStanNaw))
      ;[1 1 1] プレイヤーのほうを向く
      (Transformation|SetActorRotation (Math|Rotator|MakeRotator (.roll _returnvalue_7) 0.0 (.yaw _returnvalue_7)))
      ;[1 1 1] 攻撃
      (if (Variables|Default|GetinGame)
        (bind _output_get (Variables|Default|SetElapsedTime (+ (Variables|Default|GetElapsedTime) (Utilities|Time|GetWorldDeltaSeconds))))
        (if (>= _output_get _out_row_attack_interval)
          (Variables|Default|SetElapsedTime (- _output_get _out_row_attack_interval))
          (CallFunction|Attack))))))

(fn ConstructionScript)

(fn Distance
  (bind _returnvalue (Game|GetPlayerCharacter 0))
  (Utilities|IsValid _returnvalue
    (:Is%20Valid
      (return (Math|Vector|VectorLength (- (Transformation|GetActorLocation) (Transformation|GetActorLocation _returnvalue)))))))

(fn InternalandExternalJudgments
  (params (Spline :type Spline%20Component%20Object%20Reference))
  (bind _returnvalue (Transformation|GetActorLocation))
  (LocalVariables|SetSplineObject Spline)
  (LocalVariables|SetResult 0.0)
  (bind _index (Utilities|FlowControl|ForLoopwithBreak 0 (- (Class|SplineComponent|GetNumberOfSplineSegments (LocalVariables|GetSplineObject)) 2) :!label _label)
    (:LoopBody
      (Utilities|IsValid (LocalVariables|GetSplineObject)
        (:Is%20Valid
          (if (< (Math|Vector|DotProduct (Math|Vector|CrossProduct (- (.Location (Spline|GetLocationandTangentatSplinePoint (LocalVariables|GetSplineObject) _index "World")) _returnvalue) (- (.Location (Spline|GetLocationandTangentatSplinePoint (LocalVariables|GetSplineObject) (+ _index 1) "World")) _returnvalue)) (Math|Vector|MakeVector 0.0 0.0 1.0)) 0.0)
            (LocalVariables|SetResult (+ (Math|Trig|Acos(Degrees) (/ (Math|Vector|DotProduct (- (.Location (Spline|GetLocationandTangentatSplinePoint (LocalVariables|GetSplineObject) _index "World")) _returnvalue) (- (.Location (Spline|GetLocationandTangentatSplinePoint (LocalVariables|GetSplineObject) (+ _index 1) "World")) _returnvalue)) (* (Math|Vector|VectorLength (- (.Location (Spline|GetLocationandTangentatSplinePoint (LocalVariables|GetSplineObject) _index "World")) _returnvalue)) (Math|Vector|VectorLength (- (.Location (Spline|GetLocationandTangentatSplinePoint (LocalVariables|GetSplineObject) (+ _index 1) "World")) _returnvalue))))) (LocalVariables|GetResult)))
            (else
              (LocalVariables|SetResult (+ (* (Math|Trig|Acos(Degrees) (/ (Math|Vector|DotProduct (- (.Location (Spline|GetLocationandTangentatSplinePoint (LocalVariables|GetSplineObject) _index "World")) _returnvalue) (- (.Location (Spline|GetLocationandTangentatSplinePoint (LocalVariables|GetSplineObject) (+ _index 1) "World")) _returnvalue)) (* (Math|Vector|VectorLength (- (.Location (Spline|GetLocationandTangentatSplinePoint (LocalVariables|GetSplineObject) _index "World")) _returnvalue)) (Math|Vector|VectorLength (- (.Location (Spline|GetLocationandTangentatSplinePoint (LocalVariables|GetSplineObject) (+ _index 1) "World")) _returnvalue))))) -1.0) (LocalVariables|GetResult))))))
        (:Is%20Not%20Valid
          (goto _label Break))))
    (:Completed
      (return (Math|Float|Absolute(Float) (LocalVariables|GetResult))))))