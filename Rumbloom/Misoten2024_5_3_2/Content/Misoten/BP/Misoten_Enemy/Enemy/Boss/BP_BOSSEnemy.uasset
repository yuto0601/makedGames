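; BP_BOSSEnemy is an enemy Blueprint for the boss fight that reports its count to BP_BOSS.
; On BeginPlay it runs the parent logic, then disables collision on its Sphere component.
; EnemyCountUP and EnemyCountDown find BP_BOSS via GetActorOfClass and adjust its EnemyCount by one.
; When the count drops to zero, EnemyCountDown calls SpawnEnemy on the boss.
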(event Custom|EnemyCountUP
  (bind _returnvalue (Actor|GetActorOfClass "/Game/Misoten/BP/Misoten_Enemy/Enemy/Boss/BP_BOSS.BP_BOSS_C"))
  (Variables|/Game/Misoten/BP/Misoten_Enemy/Enemy/Boss/BP_BOSS.BP_BOSS_C|SetEnemyCount _returnvalue (+ (Variables|/Game/Misoten/BP/Misoten_Enemy/Enemy/Boss/BP_BOSS.BP_BOSS_C|GetEnemyCount _returnvalue) 1.0)))

(event Custom|EnemyCountDown
  (bind _returnvalue (Actor|GetActorOfClass "/Game/Misoten/BP/Misoten_Enemy/Enemy/Boss/BP_BOSS.BP_BOSS_C"))
  (bind _output_get (Variables|/Game/Misoten/BP/Misoten_Enemy/Enemy/Boss/BP_BOSS.BP_BOSS_C|SetEnemyCount _returnvalue (+ (Variables|/Game/Misoten/BP/Misoten_Enemy/Enemy/Boss/BP_BOSS.BP_BOSS_C|GetEnemyCount _returnvalue) -1.0)))
  (if (== _output_get 0.0)
    (Default|SpawnEnemy _returnvalue)))

(event EventBeginPlay
  (|CallParentFunction)
  (Collision|SetCollisionEnabled (Variables|Default|GetSphere) "NoCollision"))

(event Collision|EventActorBeginOverlap
  (params (OtherActor :type Actor%20Object%20Reference)))

(event EventTick
  (params (DeltaSeconds :type Float%20%28single-precision%29))
  (|CallParentFunction DeltaSeconds) ; このノードは無効になっているため呼び出せません。\n機能をビルドするにはピンをドラッグしてください。
)

(fn ConstructionScript
  (|CallParentFunction))