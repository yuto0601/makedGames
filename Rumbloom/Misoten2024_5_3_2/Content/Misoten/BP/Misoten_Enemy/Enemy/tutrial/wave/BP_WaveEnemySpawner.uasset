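; Wave-based enemy spawner in the tutorial folder that opens the Area C fence once every wave is defeated.
; BeginPlay records placed enemies' classes and transforms, then destroys them as templates for waves sized by EnemyCount.
; After firstSpawn, Tick prunes dead enemies and spawns the next wave when none remain.
; After the last, a pause-aware timer spawns a death box and plays the opening sequence; Sequence_FanceOpen removes the wall.
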(event Custom|firstSpawn
  (Utilities|FlowControl|DoOnce false
    (:Completed
      ;[1 1 1] 1wave目の敵のスポーン
      (for _index (range 0 (- (Utilities|Array|Get(acopy) (Variables|Default|GetenemyCount)) 1))
        (Niagara|SpawnSystematLocation "/Game/Misoten/Assets/EFF/EFF_Enemy_Spawn/NS_Enemy_Spawn.NS_Enemy_Spawn" (.Location (Math|Transform|BreakTransform (Math|Transform|MakeTransform (.location (.transform (Utilities|Array|Get(acopy) (Variables|Default|GetWaveenemy) _index))) (.rotation (.transform (Utilities|Array|Get(acopy) (Variables|Default|GetWaveenemy) _index))) (/ (.scale (.transform (Utilities|Array|Get(acopy) (Variables|Default|GetWaveenemy) _index))) 2)))) (.Rotation (Math|Transform|BreakTransform (Math|Transform|MakeTransform (.location (.transform (Utilities|Array|Get(acopy) (Variables|Default|GetWaveenemy) _index))) (.rotation (.transform (Utilities|Array|Get(acopy) (Variables|Default|GetWaveenemy) _index))) (/ (.scale (.transform (Utilities|Array|Get(acopy) (Variables|Default|GetWaveenemy) _index))) 2)))) (.Scale (Math|Transform|BreakTransform (Math|Transform|MakeTransform (.location (.transform (Utilities|Array|Get(acopy) (Variables|Default|GetWaveenemy) _index))) (.rotation (.transform (Utilities|Array|Get(acopy) (Variables|Default|GetWaveenemy) _index))) (/ (.scale (.transform (Utilities|Array|Get(acopy) (Variables|Default|GetWaveenemy) _index))) 2)))))
        (bind _returnvalue (Game|SpawnActorfromClass (.actorclass (Utilities|Array|Get(acopy) (Variables|Default|GetWaveenemy) _index)) (Math|Transform|MakeTransform (.location (.transform (Utilities|Array|Get(acopy) (Variables|Default|GetWaveenemy) _index))) (.rotation (.transform (Utilities|Array|Get(acopy) (Variables|Default|GetWaveenemy) _index))) (/ (.scale (.transform (Utilities|Array|Get(acopy) (Variables|Default|GetWaveenemy) _index))) 2)) "AlwaysSpawn" "MultiplyWithRoot" 0 0))
        ;[1 1 1] 計算しやすくするために敵の中にself追加
        (bind _asbp_enemy_base (Utilities|Casting|CastToBP_Enemy_Base _returnvalue))
        (Variables|/Game/Misoten/BP/BP_Enemy_Base.BP_Enemy_Base_C|Setparent _asbp_enemy_base self)
        ;[1 1 1] 敵の配列に追加
        (Utilities|Array|Add (Variables|Default|Getnow%20Enemy%20Obj) _returnvalue)
        ;[1 1 1] スポーン数にプラス
        (Math|Integer|IncrementInt (Variables|Default|GetspawnedEnemyTotal)))
      (Math|Integer|IncrementInt (Variables|Default|GetnowWave)
        (:%20%20
          (Variables|Default|Setspawned true))))))

(event Custom|FenceOpen
  (Utilities|FlowControl|DoOnce false
    (:Completed
      (Utilities|Time|SetTimerbyEvent (delegate Custom|カスタムイベント) 1.0))))

(event Custom|Sequence_FanceOpen
  (Components|Activation|SetActive (Variables|Default|GetNS_Enemy_Spawn) true false)
  (Components|DestroyComponent (Variables|Default|Getwall1))
  (Components|DestroyComponent (Variables|Default|GetBox))
  (Variables|Default|SetIsFinish true))

(event Custom|カスタムイベント
  (bind _asbp_practise_drift_player_con (Utilities|Casting|CastToBP_PractiseDrift_PlayerCon (Game|GetPlayerController 0) :!label _label))
  (if (Variables|/Game/Misoten/BP/BP_PractiseDrift_PlayerCon.BP_PractiseDrift_PlayerCon_C|GetIsPause _asbp_practise_drift_player_con)
    (Utilities|FlowControl|DelayUntilNextTick)
    (goto _label)
    (else
      (Game|SpawnActorfromClass "/Game/Misoten/BP/BP_AreaC_DeathBox.BP_AreaC_DeathBox_C" (Math|Transform|MakeTransform "106513.362027,0.000000,0.000000" "0, 0, 0" "1.000000,1.000000,1.000000") "Undefined" "MultiplyWithRoot" 0 0)
      (bind _returnvalue (Sequencer|Player|CreateLevelSequencePlayer "/Game/Misoten/Assets/Seqence/Sequence/Area_C_Open_SequenceMaster.Area_C_Open_SequenceMaster" (Utilities|Struct|MakeMovieSceneSequencePlaybackSettings false "(Value=0)")))
      (Sequencer|Player|Play _returnvalue :!class /Script/MovieScene.MovieSceneSequencePlayer))))

(event EventBeginPlay
  (for _array_element (Variables|Default|GetenemiesTransform)
    (Utilities|Array|Add (Variables|Default|GetWaveenemy) (Utilities|Struct|MakeWaveEnemy (Utilities|GetClass _array_element) (Transformation|GetActorTransform _array_element)))
    (Actor|DestroyActor _array_element))
  (Variables|Default|SetwaveCount (Utilities|Array|Length (Variables|Default|GetenemyCount))) ; wave数の計算
)

(event EventTick
  (params (DeltaSeconds :type Float%20%28single-precision%29))
  (if (not (Variables|Default|GetIsFinish))
    (CallFunction|ArrayConfirm)))

(fn ConstructionScript)

(fn SpawnNextWave
  ;[1 1 1] 今のウェーブがウェーブ総数のとき削除
  (if (>= (Variables|Default|GetnowWave) (Variables|Default|GetwaveCount))
    (CallFunction|FenceOpen)
    (else
      (bind _output_get (LocalVariables|SetNewLocalVar (- (+ (Variables|Default|GetspawnedEnemyTotal) (Utilities|Array|Get(acopy) (Variables|Default|GetenemyCount) (Variables|Default|GetnowWave))) 1)))
      (for _index (range (Variables|Default|GetspawnedEnemyTotal) _output_get)
        ;[1 1 1] 一度目と同じ処理
        (Niagara|SpawnSystematLocation "/Game/Misoten/Assets/EFF/EFF_Enemy_Spawn/NS_Enemy_Spawn.NS_Enemy_Spawn" (.location (.transform (Utilities|Array|Get(acopy) (Variables|Default|GetWaveenemy) _index))) (.rotation (.transform (Utilities|Array|Get(acopy) (Variables|Default|GetWaveenemy) _index))) (.scale (.transform (Utilities|Array|Get(acopy) (Variables|Default|GetWaveenemy) _index))))
        (bind _returnvalue (Game|SpawnActorfromClass (.actorclass (Utilities|Array|Get(acopy) (Variables|Default|GetWaveenemy) _index)) (Math|Transform|MakeTransform (.location (.transform (Utilities|Array|Get(acopy) (Variables|Default|GetWaveenemy) _index))) (.rotation (.transform (Utilities|Array|Get(acopy) (Variables|Default|GetWaveenemy) _index))) (/ (.scale (.transform (Utilities|Array|Get(acopy) (Variables|Default|GetWaveenemy) _index))) 2)) "Undefined" "MultiplyWithRoot" 0 0))
        (Utilities|Array|Add (Variables|Default|Getnow%20Enemy%20Obj) _returnvalue)
        (Math|Integer|IncrementInt (Variables|Default|GetspawnedEnemyTotal)
          (:%20%20
            (bind _asbp_enemy_base (Utilities|Casting|CastToBP_Enemy_Base _returnvalue))
            (Variables|/Game/Misoten/BP/BP_Enemy_Base.BP_Enemy_Base_C|Setparent _asbp_enemy_base self))))
      (if (not (== (Variables|Default|GetnowWave) (Variables|Default|GetwaveCount)))
        (Math|Integer|IncrementInt (Variables|Default|GetnowWave))))))

(fn ArrayConfirm
  (bind _now_enemy_obj (Variables|Default|Getnow%20Enemy%20Obj))
  (bind (_arrayindex _arrayelement) (Utilities|Array|ReverseforEachLoop _now_enemy_obj)
    (:LoopBody
      (Utilities|Casting|CastToBP_Enemy_Base _arrayelement
        (:CastFailed
          (Utilities|Array|RemoveIndex _now_enemy_obj _arrayindex))))
    (:Completed
      (if (Utilities|Array|IsEmpty _now_enemy_obj)
        (if (Variables|Default|Getspawned)
          (CallFunction|SpawnNextWave))))))