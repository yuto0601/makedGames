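; Tutorial-wave enemy Blueprint that circles endlessly around the point where it starts, facing its direction of travel.
; BeginPlay stores the start location as the orbit center and the initial yaw as the starting angle.
; Each Tick adds Speed to that angle without DeltaSeconds scaling, computes the XY point at Radius, turns toward it through LookatVector, then moves there without sweep.
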(event EventBeginPlay
  (|CallParentFunction)
  (Variables|Default|SetPointO (Transformation|GetActorLocation))
  (Variables|Default|Setacceleration (.yaw (Transformation|GetActorRotation))))

(event Collision|EventActorBeginOverlap
  (params (OtherActor :type Actor%20Object%20Reference)))

(event EventTick
  (params (DeltaSeconds :type Float%20%28single-precision%29))
  (|CallParentFunction DeltaSeconds)
  (Variables|Default|Setacceleration (+ (Variables|Default|Getspeed) (Variables|Default|Getacceleration)))
  (bind _returnvalue (CallFunction|Calclation))
  (CallFunction|LookatVector (Math|Conversions|RotationFromXVector (- _returnvalue (Transformation|GetActorLocation))) 0.0)
  (Transformation|SetActorLocation _returnvalue false false))

(fn ConstructionScript
  (|CallParentFunction))

(fn Calclation
  (bind _pointo (Variables|Default|GetPointO))
  (return (Math|Vector|MakeVector (+ (* (Variables|Default|GetRadius) (Math|Trig|Cos(Degrees) (Variables|Default|Getacceleration))) (.x _pointo)) (+ (.y _pointo) (* (Variables|Default|GetRadius) (Math|Trig|Sin(Degrees) (Variables|Default|Getacceleration)))) (.z _pointo))))