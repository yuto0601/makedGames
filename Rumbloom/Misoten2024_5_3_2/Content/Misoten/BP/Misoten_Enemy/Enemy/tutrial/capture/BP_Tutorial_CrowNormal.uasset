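; BP_Tutorial_CrowNormal is a tutorial crow enemy that must be defeated by enclosing it to open a linked wall.
; BeginPlay sets HP to 1 and saves the crow's transform as the respawn point.
; The Death override destroys the Wall if enclosed, otherwise spawns a replacement slightly above that point carrying the same Wall, then calls parent Death with both flags false.
; Debug keys clear IsCap or force a non-enclosed death.
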(event Custom|respawn
  (bind _respawn_point (Variables|Default|Getrespawn_point))
  ;[1 1 1] リスポーン用の処理
  (Game|SpawnActorfromClass "BP_Tutorial_CrowNormal_C" (Math|Transform|MakeTransform (Math|Vector|MakeVector (.x (.location _respawn_point)) (.y (.location _respawn_point)) (+ (.z (.location _respawn_point)) 5e+01)) (.rotation _respawn_point) "1.000000,1.000000,1.000000") "Undefined" "MultiplyWithRoot" 0 (Variables|Default|Getwall) 0))

(event Custom|break%20wall
  ;[1 1 1] 壁の破壊イベント
  (Actor|DestroyActor (Variables|Default|Getwall)))

(event EventBeginPlay
  ;[1 1 1] 開始時にリスポーン位置として初期位置を保存する処理
  (Variables|Default|SetHP 1.0)
  (|CallParentFunction)
  (Variables|Default|Setrespawn_point (Transformation|GetWorldTransform (Variables|Default|GetCrow)))
  ;[1 1 1] テスト用
  (Input|EnableInput (Game|GetPlayerController 0)) ; デバッグ用
)

(event Input|KeyboardEvents|DebugKeyO
  (params (Key :type Key%20Structure :default "None") (ActionValue :type Input%20Action%20Value%20Structure))
  ;[1 1 1] テスト用
  (:Pressed
    (CallFunction|Death false false)
    (Development|PrintString "deathed!!!")))

(event Input|KeyboardEvents|DebugKeyI
  (params (Key :type Key%20Structure :default "None") (ActionValue :type Input%20Action%20Value%20Structure))
  ;[1 1 1] テスト用
  (:Pressed
    (Utilities|FlowControl|DoOnce false :!label _label
      (:Completed
        (Variables|Default|SetisCap false))))
  (:Released
    (Variables|Default|SetisCap false)
    (goto _label Reset)))

(fn ConstructionScript
  (|CallParentFunction))

(fn Death
  (params (isEnclose :type Boolean) (IsDeath :type Boolean))
  ;[1 1 1] 倒されたときのイベント
  (if isEnclose ; どのように倒されたのか\n(今回は囲まれたときにtrue)
    (CallFunction|BreakWall) ; 壁(指定したオブジェクト)を破壊するイベント
    (else
      (CallFunction|Respawn) ; 初期位置にリスポーンさせる処理
    ))
  (|CallParentFunction false false))