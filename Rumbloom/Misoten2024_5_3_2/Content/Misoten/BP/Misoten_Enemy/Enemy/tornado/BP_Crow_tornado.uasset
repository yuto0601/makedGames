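; Crow enemy, tornado variant, that turns to face the player and fires bullets while inside the player's camera view.
; Tick tests a 50-degree cone around camera forward, calls LookPlayer, waits AttackInterval, then rechecks the cone before calling Attack.
; Attack runs the parent attack and spawns a Bullet at the Crow component, rotated along the player-to-crow direction.
; Both rotations offset yaw by 90 degrees to correct the forward vector.
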(event EventBeginPlay)

(event Collision|EventActorBeginOverlap
  (params (OtherActor :type Actor%20Object%20Reference)))

(event EventTick
  (params (DeltaSeconds :type Float%20%28single-precision%29))
  (bind _returnvalue (Game|GetPlayerCameraManager 0))
  (bind _returnvalue_2 (Transformation|GetActorLocation))
  (bind _returnvalue_3 (Math|Float|MakeLiteralFloat 5e+01))
  (bind _returnvalue_4 (Transformation|GetActorLocation _returnvalue))
  (bind _transformcomponent (Variables|/Script/Engine.PlayerCameraManager|GetTransformComponent _returnvalue))
  (bind _returnvalue_5 (Math|Vector|GetForwardVector _transformcomponent))
  (bind _returnvalue_6 (Math|Rotator|FindLookatRotation _returnvalue_4 _returnvalue_2))
  (bind _returnvalue_7 (Math|Vector|GetForwardVector _returnvalue_6))
  (bind _returnvalue_8 (Math|Vector|DotProduct _returnvalue_5 _returnvalue_7))
  (bind _returnvalue_9 (Class|KismetMathLibrary|DegAcos _returnvalue_8))
  (bind _returnvalue_10 (< _returnvalue_9 _returnvalue_3))
  (if _returnvalue_10
    (CallFunction|LookPlayer)
    (Utilities|FlowControl|Delay (Variables|Default|GetattackInterval))
    (if _returnvalue_10
      (Development|PrintString "attack!")
      (CallFunction|Attack))))

(fn ConstructionScript)

(fn Attack
  (bind _returnvalue (Game|Player|GetPlayerPawn 0))
  (bind _crow (Variables|Default|GetCrow))
  (bind _returnvalue_2 (Transformation|GetWorldTransform _crow))
  (bind _returnvalue_3 (Transformation|GetActorTransform _returnvalue))
  (bind _returnvalue_4 (Math|Rotator|FindLookatRotation (.location _returnvalue_3) (.location _returnvalue_2)))
  (|CallParentFunction)
  (bind _returnvalue_5 (Game|SpawnActorfromClass "/Game/Misoten/BP/Misoten_Enemy/Enemy/tornado/bullet.bullet_C" (Math|Transform|MakeTransform (.location _returnvalue_2) (Math|Rotator|MakeRotator (.roll _returnvalue_4) (.pitch _returnvalue_4) (- (.yaw _returnvalue_4) 9e+01)) "1.000000,1.000000,1.000000") "Undefined" "OverrideRootScale" 0 0)))

(fn LookPlayer
  (bind _returnvalue (Game|Player|GetPlayerPawn 0))
  (bind _crow (Variables|Default|GetCrow))
  (bind _returnvalue_2 (Transformation|GetWorldLocation _crow))
  (bind _returnvalue_3 (Transformation|GetActorLocation _returnvalue))
  (bind _returnvalue_4 (Math|Rotator|FindLookatRotation _returnvalue_2 _returnvalue_3))
  (bind (_roll _pitch _yaw) (Math|Rotator|BreakRotator _returnvalue_4))
  (Transformation|SetActorRotation (Math|Rotator|MakeRotator _roll _pitch (- _yaw 9e+01)) true))