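; Thunder boss enemy that looks at the player and, on a cooldown made by a Delay in Tick, randomly picks one of two lightning attacks.
; Attack1 builds a grid of positions toward the player and spawns Thunder row by row through a custom delayed ForLoop macro.
; Attack2 repeatedly spawns Thunder ahead of the player a random number of times.
; Debug keys adjust the grid's row count and width.
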(event EventBeginPlay
  (|CallParentFunction)
  (Input|EnableInput (Game|GetPlayerController 0)))

(event Collision|EventActorBeginOverlap
  (params (OtherActor :type Actor%20Object%20Reference)))

(event EventTick
  (params (DeltaSeconds :type Float%20%28single-precision%29))
  (|CallParentFunction DeltaSeconds)
  (CallFunction|LookatTarget (Game|Player|GetPlayerPawn 0))
  (Utilities|FlowControl|Delay (Variables|Default|GetCoolTime))
  (if (Math|Random|RandomBool)
    (|Attack1)
    (else
      (Utilities|ForLoop 0 (Math|Random|RandomIntegerinRange (- (Variables|Default|Getattack2Min) 1) (Variables|Default|Getattack2Max)) (Variables|Default|GetAttack2Interval)
        (:LoopBody
          (CallFunction|Attack2))))))

(event Input|KeyboardEvents|DebugKeyL
  (params (Key :type Key%20Structure) (ActionValue :type Input%20Action%20Value%20Structure))
  (:Pressed
    (Math|Integer|DecrementInt (Variables|Default|GetthunderCount))))

(event Input|KeyboardEvents|DebugKeyP
  (params (Key :type Key%20Structure) (ActionValue :type Input%20Action%20Value%20Structure))
  (:Pressed
    (Math|Integer|IncrementInt (Variables|Default|GetthunderCount))))

(event Input|KeyboardEvents|DebugKeyO
  (params (Key :type Key%20Structure) (ActionValue :type Input%20Action%20Value%20Structure))
  (bind _thunderwidth (Variables|Default|GetthunderWidth))
  (:Pressed
    (Math|Integer|IncrementInt _thunderwidth
      (:%20%20
        (Math|Integer|IncrementInt _thunderwidth)))))

(event Input|KeyboardEvents|DebugKeyK
  (params (Key :type Key%20Structure) (ActionValue :type Input%20Action%20Value%20Structure))
  (bind _thunderwidth (Variables|Default|GetthunderWidth))
  (:Pressed
    (Math|Integer|DecrementInt _thunderwidth
      (:%20%20
        (Math|Integer|DecrementInt _thunderwidth)))))

(fn ConstructionScript
  (|CallParentFunction))

(fn MakePositions
  (CallFunction|CalcPlayerVec)
  (for _index (range 0 (Variables|Default|GetthunderCount))
    (for _index_2 (range 1 (Variables|Default|GetthunderWidth))
      ;[1 1 1] 値の偶奇判定
      (if (== (Math|Integer|%(Integer) _index_2 2) 1)
        (Utilities|Array|Add (Variables|Default|GetspawnPos) (Math|Conversions|ToTransform(Vector) (.ReturnValue (|calcRow (.Location (Math|Transform|BreakTransform (|calclationcolumm (Transformation|GetActorLocation) _index))) _index_2))))
        (else
          (Utilities|Array|Add (Variables|Default|GetspawnPos) (Math|Conversions|ToTransform(Vector) (.ReturnValue2 (|calcRow (.Location (Math|Transform|BreakTransform (|calclationcolumm (Transformation|GetActorLocation) _index))) _index_2)))))))))

(fn MakeThunderObj
  (params (Attack%20row :type Integer))
  (bind _thunderwidth (Variables|Default|GetthunderWidth))
  (bind _returnvalue (* Attack%20row _thunderwidth))
  (for _index (range _returnvalue (- (+ _thunderwidth _returnvalue) 1))
    (bind _returnvalue_2 (Game|SpawnActorfromClass "/Game/Misoten/BP/Misoten_Enemy/Enemy/Thunder/Thunder.Thunder_C" (Utilities|Array|Get(acopy) (Variables|Default|GetspawnPos) _index) "Undefined" "OverrideRootScale" 0 0))
    (Development|PrintString (Utilities|String|ToString(Vector) (Transformation|GetActorLocation _returnvalue_2)))))

(fn Attack
  (|CallParentFunction))

(fn CalcPlayerVec
  (bind _output_get (Variables|Default|SetatPlayerVec (- (Transformation|GetActorLocation (Game|GetPlayerCharacter 0)) (Transformation|GetActorLocation))))
  (Development|PrintString (Utilities|String|ToString(Float) (Math|Vector|VectorLength _output_get)) true true "(R=1.000000,G=0.064799,B=0.000000,A=1.000000)"))

(fn Attack2
  (Game|SpawnActorfromClass "/Game/Misoten/BP/Misoten_Enemy/Enemy/Thunder/Thunder.Thunder_C" (Math|Conversions|ToTransform(Vector) (+ (* (Transformation|GetActorForwardVector (Game|GetPlayerCharacter 0)) (Variables|Default|GetAttack2%20dist)) (Transformation|GetActorLocation (Game|Player|GetPlayerPawn 0)))) "Undefined" "MultiplyWithRoot" 0 0))

(fn Death
  (params (isEnclose :type Boolean) (IsDeath :type Boolean))
  (|CallParentFunction isEnclose IsDeath))