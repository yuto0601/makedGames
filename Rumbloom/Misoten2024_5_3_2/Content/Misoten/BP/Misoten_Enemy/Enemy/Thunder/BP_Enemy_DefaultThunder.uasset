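; Thunder enemy that repeatedly attacks by spawning a line of Thunder actors in front of the player.
; Tick runs through a Delay to call Attack periodically, which calls the parent attack, builds spawn positions, then spawns an actor at each.
; Positions center ahead of the player at the enemy's height, with a FlipFlop fanning extra ones left and right by Space, up to ThunderCount.
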(event EventTick
  (params (DeltaSeconds :type Float%20%28single-precision%29))
  (Utilities|FlowControl|Delay 2.0)
  (CallFunction|Attack))

(fn ConstructionScript)

(fn MakeThunderObj
  (for _array_element (Variables|Default|GetspawnPos)
    (Game|SpawnActorfromClass "/Game/Misoten/BP/Misoten_Enemy/Enemy/Thunder/Thunder.Thunder_C" _array_element "Undefined" "OverrideRootScale" 0 0)))

(fn MakePositions
  (bind _returnvalue (Game|GetPlayerCharacter 0))
  (bind _returnvalue_2 (Transformation|GetActorLocation))
  (bind _returnvalue_3 (Game|GetPlayerCharacter 0))
  (bind _returnvalue_4 (Transformation|GetActorLocation _returnvalue))
  (bind _returnvalue_5 (Transformation|GetActorForwardVector _returnvalue_3))
  (bind _returnvalue_6 (* _returnvalue_5 1e+03))
  (bind _returnvalue_7 (+ (Math|Vector|MakeVector (.x _returnvalue_4) (.y _returnvalue_4) 0.0) (Math|Vector|MakeVector (.x _returnvalue_6) (.y _returnvalue_6) (.z _returnvalue_2))))
  (Variables|Default|SetspawnPos (Utilities|Array|MakeArray (Math|Conversions|ToTransform(Vector) _returnvalue_7)))
  (for _index (range 2 (Variables|Default|GetthunderCount))
    (Utilities|FlowControl|FlipFlop
      (:A
        (Utilities|Array|Add (Variables|Default|GetspawnPos) (Math|Conversions|ToTransform(Vector) (+ _returnvalue_7 (* (/ _index 2) (* (Transformation|GetActorRightVector _returnvalue_3) (Variables|Default|Getspace)))))))
      (:B
        (Utilities|Array|Add (Variables|Default|GetspawnPos) (Math|Conversions|ToTransform(Vector) (- _returnvalue_7 (* (/ _index 2) (* (Transformation|GetActorRightVector _returnvalue_3) (Variables|Default|Getspace))))))))))

(fn Attack
  (|CallParentFunction)
  (CallFunction|MakePositions)
  (CallFunction|MakeThunderObj))