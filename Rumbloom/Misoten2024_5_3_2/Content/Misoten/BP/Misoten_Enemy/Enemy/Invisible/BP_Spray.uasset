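; BP_Spray is a short-lived spray effect actor that triggers the spray attack on the invisible enemy, Enemy_Invisible.
; On BeginPlay it registers itself as its Niagara system's callback object, and the first exported particle data event calls SprayAttack on that enemy, gated by DoOnce.
; After four seconds it clears the enemy's SprayNaw flag and destroys itself.
; The enemy is found with GetActorOfClass rather than a stored reference.
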(event EventBeginPlay
  (Class|NiagaraComponent|SetVariableObject (Variables|Default|GetNiagara) "BPCallback" self)
  (Utilities|FlowControl|Delay 4.0)
  (bind _returnvalue (Actor|GetActorOfClass "/Game/Misoten/BP/Misoten_Enemy/Enemy/Invisible/Enemy_Invisible.Enemy_Invisible_C"))
  (Variables|/Game/Misoten/BP/Misoten_Enemy/Enemy/Invisible/Enemy_Invisible.Enemy_Invisible_C|SetSprayNaw _returnvalue false)
  (Actor|DestroyActor))

(event EventParticleData
  (params (Data :type Array%20of%20Basic%20Particle%20Data%20Structures) (NiagaraSystem :type Niagara%20System%20Object%20Reference) (SimulationPositionOffset :type Vector%20%28by%20ref%29 :default "0, 0, 0"))
  (Utilities|FlowControl|DoOnce false
    (:Completed
      (bind _returnvalue (Actor|GetActorOfClass "/Game/Misoten/BP/Misoten_Enemy/Enemy/Invisible/Enemy_Invisible.Enemy_Invisible_C"))
      (Default|SprayAttack _returnvalue))))

(fn ConstructionScript)