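; BP_GameClear is an actor that runs the game clear screen.
; On BeginPlay it creates the WBP_GameClearwight widget and adds it to the viewport.
; Pressing A or the gamepad bottom face button fires once, playing a sound and waiting briefly.
; It then sets the finish flag and scene variable on BP_Gameinstance and calls ChangeSceneEvent to switch scenes.
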(event EventBeginPlay
  ;[1 1 1] 初期処理
  ;;[1 1 1] ゲームクリア画像生成
  (bind _returnvalue (UserInterface|CreateWidget "/Game/Misoten/BP/nomurafolder/WBP_GameClearwight.WBP_GameClearwight_C"))
  (UserInterface|Viewport|AddtoViewport _returnvalue 0))

(event Collision|EventActorBeginOverlap
  (params (OtherActor :type Actor%20Object%20Reference)))

(event EventTick
  (params (DeltaSeconds :type Float%20%28single-precision%29)))

(event Input|GamepadEvents|GamepadFaceButtonBottom
  (params (Key :type Key%20Structure :default "None"))
  ;[1 1 1] Aボタンを押したときの処理
  (:Pressed
    (Utilities|FlowControl|DoOnce false
      (:Completed
        (Audio|PlaySoundatLocation "/Game/Misoten/BP/Audio/BGM/Title/11_16/DEMO3.DEMO3" "0, 0, 0" "0, 0, 0" 1.0 1.0 0.0 0 0 0 0)
        (Utilities|FlowControl|Delay 2.0)
        (bind _asbp_gameinstance (Utilities|Casting|CastToBP_Gameinstance (Game|GetGameInstance)))
        (Variables|/Game/Misoten/BP/nomurafolder/BP_Gameinstance.BP_Gameinstance_C|SetGameFinishFlg _asbp_gameinstance true)
        (Variables|/Game/Misoten/BP/nomurafolder/BP_Gameinstance.BP_Gameinstance_C|SetSceneVariable _asbp_gameinstance 2)
        (Default|ChangeSceneEvent _asbp_gameinstance)))))

(event Input|KeyboardEvents|A
  (params (Key :type Key%20Structure :default "None"))
  ;[1 1 1] Aボタンを押したときの処理
  (:Pressed
    (Utilities|FlowControl|DoOnce false
      (:Completed
        (Audio|PlaySoundatLocation "/Game/Misoten/BP/Audio/BGM/Title/11_16/DEMO3.DEMO3" "0, 0, 0" "0, 0, 0" 1.0 1.0 0.0 0 0 0 0)
        (Utilities|FlowControl|Delay 2.0)
        (bind _asbp_gameinstance (Utilities|Casting|CastToBP_Gameinstance (Game|GetGameInstance)))
        (Variables|/Game/Misoten/BP/nomurafolder/BP_Gameinstance.BP_Gameinstance_C|SetGameFinishFlg _asbp_gameinstance true)
        (Variables|/Game/Misoten/BP/nomurafolder/BP_Gameinstance.BP_Gameinstance_C|SetSceneVariable _asbp_gameinstance 2)
        (Default|ChangeSceneEvent _asbp_gameinstance)))))

(fn ConstructionScript)