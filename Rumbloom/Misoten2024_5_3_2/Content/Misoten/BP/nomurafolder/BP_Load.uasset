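; BP_Load is the loading-screen actor that shows a loading widget and then moves the game on to the next scene.
; On BeginPlay it adds WBP_Loadwigit to the viewport, then triggers the transition after a three-second delay or when A or the gamepad bottom face button is pressed.
; The transition reads GameFinishFlg from BP_Gameinstance to choose the scene number, clearing the flag if set, and calls ChangeSceneEvent.
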(event EventBeginPlay
  ;[1 1 1] 初期処理
  (Utilities|FlowControl|Sequence
    (:then_0
      ;;[1 1 1] ロード画面画像生成
      (bind _returnvalue (UserInterface|CreateWidget "/Game/Misoten/BP/nomurafolder/WBP_Loadwigit.WBP_Loadwigit_C"))
      (UserInterface|Viewport|AddtoViewport _returnvalue 0))
    (:then_1
      (Utilities|FlowControl|Delay 3.0)
      ;;[1 1 1] ゲームが終わったか判断
      (bind _asbp_gameinstance (Utilities|Casting|CastToBP_Gameinstance (Game|GetGameInstance)))
      (if (Variables|/Game/Misoten/BP/nomurafolder/BP_Gameinstance.BP_Gameinstance_C|GetGameFinishFlg _asbp_gameinstance)
        ;;[1 1 1] ゲームが終わっているかつAボタンを押したときか3秒以上たった時の処理
        (bind _asbp_gameinstance_2 (Utilities|Casting|CastToBP_Gameinstance (Game|GetGameInstance)))
        (Variables|/Game/Misoten/BP/nomurafolder/BP_Gameinstance.BP_Gameinstance_C|SetGameFinishFlg _asbp_gameinstance_2 false)
        (Variables|/Game/Misoten/BP/nomurafolder/BP_Gameinstance.BP_Gameinstance_C|SetSceneVariable _asbp_gameinstance_2 1)
        (Default|ChangeSceneEvent _asbp_gameinstance_2)
        (else
          ;;[1 1 1] ゲームが終わっていないかつAボタンを押したときか3秒以上たった時の処理
          (bind _asbp_gameinstance_3 (Utilities|Casting|CastToBP_Gameinstance (Game|GetGameInstance)))
          (Variables|/Game/Misoten/BP/nomurafolder/BP_Gameinstance.BP_Gameinstance_C|SetSceneVariable _asbp_gameinstance_3 3)
          (Default|ChangeSceneEvent _asbp_gameinstance_3))))))

(event Collision|EventActorBeginOverlap
  (params (OtherActor :type Actor%20Object%20Reference)))

(event EventTick
  (params (DeltaSeconds :type Float%20%28single-precision%29))
  ;[1 1 1] 初期処理
)

(event Input|GamepadEvents|GamepadFaceButtonBottom
  (params (Key :type Key%20Structure))
  ;[1 1 1] 初期処理
  ;;[1 1 1] 入力処理
  (:Pressed
    ;;[1 1 1] ゲームが終わったか判断
    (bind _asbp_gameinstance (Utilities|Casting|CastToBP_Gameinstance (Game|GetGameInstance)))
    (if (Variables|/Game/Misoten/BP/nomurafolder/BP_Gameinstance.BP_Gameinstance_C|GetGameFinishFlg _asbp_gameinstance)
      ;;[1 1 1] ゲームが終わっているかつAボタンを押したときか3秒以上たった時の処理
      (bind _asbp_gameinstance_2 (Utilities|Casting|CastToBP_Gameinstance (Game|GetGameInstance)))
      (Variables|/Game/Misoten/BP/nomurafolder/BP_Gameinstance.BP_Gameinstance_C|SetGameFinishFlg _asbp_gameinstance_2 false)
      (Variables|/Game/Misoten/BP/nomurafolder/BP_Gameinstance.BP_Gameinstance_C|SetSceneVariable _asbp_gameinstance_2 1)
      (Default|ChangeSceneEvent _asbp_gameinstance_2)
      (else
        ;;[1 1 1] ゲームが終わっていないかつAボタンを押したときか3秒以上たった時の処理
        (bind _asbp_gameinstance_3 (Utilities|Casting|CastToBP_Gameinstance (Game|GetGameInstance)))
        (Variables|/Game/Misoten/BP/nomurafolder/BP_Gameinstance.BP_Gameinstance_C|SetSceneVariable _asbp_gameinstance_3 3)
        (Default|ChangeSceneEvent _asbp_gameinstance_3)))))

(event Input|KeyboardEvents|A
  (params (Key :type Key%20Structure))
  ;[1 1 1] 初期処理
  ;;[1 1 1] 入力処理
  (:Pressed
    ;;[1 1 1] ゲームが終わったか判断
    (bind _asbp_gameinstance (Utilities|Casting|CastToBP_Gameinstance (Game|GetGameInstance)))
    (if (Variables|/Game/Misoten/BP/nomurafolder/BP_Gameinstance.BP_Gameinstance_C|GetGameFinishFlg _asbp_gameinstance)
      ;;[1 1 1] ゲームが終わっているかつAボタンを押したときか3秒以上たった時の処理
      (bind _asbp_gameinstance_2 (Utilities|Casting|CastToBP_Gameinstance (Game|GetGameInstance)))
      (Variables|/Game/Misoten/BP/nomurafolder/BP_Gameinstance.BP_Gameinstance_C|SetGameFinishFlg _asbp_gameinstance_2 false)
      (Variables|/Game/Misoten/BP/nomurafolder/BP_Gameinstance.BP_Gameinstance_C|SetSceneVariable _asbp_gameinstance_2 1)
      (Default|ChangeSceneEvent _asbp_gameinstance_2)
      (else
        ;;[1 1 1] ゲームが終わっていないかつAボタンを押したときか3秒以上たった時の処理
        (bind _asbp_gameinstance_3 (Utilities|Casting|CastToBP_Gameinstance (Game|GetGameInstance)))
        (Variables|/Game/Misoten/BP/nomurafolder/BP_Gameinstance.BP_Gameinstance_C|SetSceneVariable _asbp_gameinstance_3 3)
        (Default|ChangeSceneEvent _asbp_gameinstance_3)))))

(fn ConstructionScript)