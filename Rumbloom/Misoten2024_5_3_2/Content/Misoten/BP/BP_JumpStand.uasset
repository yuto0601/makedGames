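; Jump ramp gimmick that boosts the drift pawn's speed, score, audio and rumble as it drives on and launches off.
; Entering the box adds acceleration score, speeds up the player and rumbles; leaving it airborne boosts again and switches to the jump engine sound.
; Tick watches for that jump to land, then plays the landing cue.
; The construction script reads both boost values from the gimmick status data table.
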(event OnComponentBeginOverlap(Box)
  (params (OverlappedComponent :type Primitive%20Component%20Object%20Reference) (OtherActor :type Actor%20Object%20Reference) (OtherComp :type Primitive%20Component%20Object%20Reference) (OtherBodyIndex :type Integer) (bFromSweep :type Boolean) (SweepResult :type Hit%20Result%20Structure%20%28by%20ref%29))
  (bind _asbp_practise_drift_pawn (Utilities|Casting|CastToBP_PractiseDrift_Pawn OtherActor))
  (Default|AddScoreAcceleration (Variables|/Game/Misoten/BP/BP_PractiseDrift_Pawn.BP_PractiseDrift_Pawn_C|GetBP_PlayerState _asbp_practise_drift_pawn))
  (bind _asbp_practise_drift_player_con (Utilities|Casting|CastToBP_PractiseDrift_PlayerCon (Game|GetPlayerController 0)))
  (if (Variables|/Game/Misoten/BP/BP_PractiseDrift_Pawn.BP_PractiseDrift_Pawn_C|GetIsGround _asbp_practise_drift_pawn)
    _
    (else
      _))
  (Default|CallSpeedUp _asbp_practise_drift_player_con (Variables|Default|GetBegineSpeedUpValue))
  (Game|Feedback|ClientPlayForceFeedback _asbp_practise_drift_player_con "/Game/Misoten/BP/FFE/FFE_PlayerPhase3.FFE_PlayerPhase3" "None" false false false))

(event OnComponentEndOverlap(Box)
  (params (OverlappedComponent :type Primitive%20Component%20Object%20Reference) (OtherActor :type Actor%20Object%20Reference) (OtherComp :type Primitive%20Component%20Object%20Reference) (OtherBodyIndex :type Integer))
  (bind _asbp_practise_drift_pawn (Utilities|Casting|CastToBP_PractiseDrift_Pawn OtherActor))
  (Default|AddScoreAcceleration (Variables|/Game/Misoten/BP/BP_PractiseDrift_Pawn.BP_PractiseDrift_Pawn_C|GetBP_PlayerState _asbp_practise_drift_pawn))
  (bind _asbp_practise_drift_player_con (Utilities|Casting|CastToBP_PractiseDrift_PlayerCon (Game|GetPlayerController 0)))
  (if (not (Variables|/Game/Misoten/BP/BP_PractiseDrift_Pawn.BP_PractiseDrift_Pawn_C|GetIsGround _asbp_practise_drift_pawn))
    (Default|CallSpeedUp _asbp_practise_drift_player_con (Variables|Default|GetEndSpeedUpValue))
    (Variables|Default|SetKasokuJumpFlg true)
    (Audio|Components|Audio|Play (Variables|Default|GetMS_NomalJumpEngine_Cue) 0.0)
    (Audio|Components|Audio|FadeOut (Variables|Default|GetMS_NomalJumpUp_Cue) 0.5 0.0 "Linear" :!class /Script/Engine.AudioComponent)
    (Game|Feedback|ClientPlayForceFeedback _asbp_practise_drift_player_con "/Game/Misoten/BP/FFE/FFE_PlayerPhase3.FFE_PlayerPhase3" "None" false false false)))

(event OnComponentHit(SM_TestFloor)
  (params (HitComponent :type Primitive%20Component%20Object%20Reference) (OtherActor :type Actor%20Object%20Reference) (OtherComp :type Primitive%20Component%20Object%20Reference) (NormalImpulse :type Vector :default "0, 0, 0") (Hit :type Hit%20Result%20Structure%20%28by%20ref%29))
  (bind _asbp_practise_drift_pawn (Utilities|Casting|CastToBP_PractiseDrift_Pawn OtherActor))
  (Utilities|Casting|CastToBP_PractiseDrift_PlayerCon (Game|GetPlayerController 0))
  (if (Variables|/Game/Misoten/BP/BP_PractiseDrift_Pawn.BP_PractiseDrift_Pawn_C|GetIsGround _asbp_practise_drift_pawn)
    (Audio|Components|Audio|Play (Variables|Default|GetMS_NomalJumpUp_Cue) 0.0)))

(event EventBeginPlay)

(event Collision|EventActorBeginOverlap
  (params (OtherActor :type Actor%20Object%20Reference)))

(event EventTick
  (params (DeltaSeconds :type Float%20%28single-precision%29))
  (if (Variables|Default|GetKasokuJumpFlg)
    (bind _asbp_practise_drift_pawn (Utilities|Casting|CastToBP_PractiseDrift_Pawn (Game|Player|GetPlayerPawn 0)))
    (if (Variables|/Game/Misoten/BP/BP_PractiseDrift_Pawn.BP_PractiseDrift_Pawn_C|GetIsGround _asbp_practise_drift_pawn)
      (Audio|Components|Audio|Play (Variables|Default|GetMS_NomalJumpDown_Cue) 0.0)
      (Audio|Components|Audio|Stop (Variables|Default|GetMS_NomalJumpEngine_Cue))
      (Variables|Default|SetKasokuJumpFlg false))))

(fn ConstructionScript
  (bind _returnvalue (Utilities|GetDataTableRow "/Game/Misoten/BP/DataTable/GimmickStatusDataTable.GimmickStatusDataTable" "JampStand")
    (:then
      (Variables|Default|SetBegineSpeedUpValue (.BeginSpeedUpValue (Utilities|Struct|BreakGimmickStatusStruct _returnvalue)))
      (Variables|Default|SetEndSpeedUpValue (.EndSpeedUpValue (Utilities|Struct|BreakGimmickStatusStruct _returnvalue))))))