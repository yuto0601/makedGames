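; BP_SpeedUpRing is a ring gimmick that speeds up the drift player when they exit its sphere trigger.
; The construction script loads begin and end speed-up values from the "Ring" row of the gimmick status DataTable.
; End overlap adds acceleration score, then passes only the end value to player controller 0's CallSpeedUp.
; It also plays a ring sound, activates the clear Niagara effect and triggers force feedback.
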(event OnComponentEndOverlap(Sphere)
  (params (OverlappedComponent :type Primitive%20Component%20Object%20Reference) (OtherActor :type Actor%20Object%20Reference) (OtherComp :type Primitive%20Component%20Object%20Reference) (OtherBodyIndex :type Integer))
  (bind _asbp_practise_drift_pawn (Utilities|Casting|CastToBP_PractiseDrift_Pawn OtherActor))
  (Default|AddScoreAcceleration (Variables|/Game/Misoten/BP/BP_PractiseDrift_Pawn.BP_PractiseDrift_Pawn_C|GetBP_PlayerState _asbp_practise_drift_pawn))
  (bind _asbp_practise_drift_player_con (Utilities|Casting|CastToBP_PractiseDrift_PlayerCon (Game|GetPlayerController 0)))
  (if (Variables|/Game/Misoten/BP/BP_PractiseDrift_Pawn.BP_PractiseDrift_Pawn_C|GetIsGround _asbp_practise_drift_pawn)
    _
    (else
      _))
  (Default|CallSpeedUp _asbp_practise_drift_player_con (Variables|Default|GetEndSpeedUpValue))
  (Audio|PlaySoundatLocation "/Game/Misoten/BP/Audio/SE/MS_Ring.MS_Ring" (Transformation|GetActorLocation) "0, 0, 0" 0.6 1.0 0.0 0 0 0 0)
  (Components|Activation|SetActive (Variables|Default|GetNS_RingClear) true false)
  (Game|Feedback|ClientPlayForceFeedback _asbp_practise_drift_player_con "/Game/Misoten/BP/FFE/FFE_PlayerPhase3.FFE_PlayerPhase3" "None" false false false))

(event EventBeginPlay)

(event Collision|EventActorBeginOverlap
  (params (OtherActor :type Actor%20Object%20Reference)))

(event EventTick
  (params (DeltaSeconds :type Float%20%28single-precision%29)))

(fn ConstructionScript
  (bind _returnvalue (Utilities|GetDataTableRow "/Game/Misoten/BP/DataTable/GimmickStatusDataTable.GimmickStatusDataTable" "Ring")
    (:then
      (Variables|Default|SetBegineSpeedUpValue (.BeginSpeedUpValue (Utilities|Struct|BreakGimmickStatusStruct _returnvalue)))
      (Variables|Default|SetEndSpeedUpValue (.EndSpeedUpValue (Utilities|Struct|BreakGimmickStatusStruct _returnvalue))))))