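; BP_SpeedUpStand is a speed-up pad gimmick for the drift pawn.
; The construction script reads its begin and end boost values from the "SpeedUpStand" row of the gimmick status data table.
; Box overlap adds an acceleration score to the pawn's player state, then, only if grounded, calls speed-up on player controller 0 with boost sound and force feedback.
; The end value is stored but unused in these graphs.
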(event OnComponentBeginOverlap(Box)
  (params (OverlappedComponent :type Primitive%20Component%20Object%20Reference) (OtherActor :type Actor%20Object%20Reference) (OtherComp :type Primitive%20Component%20Object%20Reference) (OtherBodyIndex :type Integer) (bFromSweep :type Boolean) (SweepResult :type Hit%20Result%20Structure%20%28by%20ref%29))
  (bind _asbp_practise_drift_pawn (Utilities|Casting|CastToBP_PractiseDrift_Pawn OtherActor))
  (Default|AddScoreAcceleration (Variables|/Game/Misoten/BP/BP_PractiseDrift_Pawn.BP_PractiseDrift_Pawn_C|GetBP_PlayerState _asbp_practise_drift_pawn))
  (bind _asbp_practise_drift_player_con (Utilities|Casting|CastToBP_PractiseDrift_PlayerCon (Game|GetPlayerController 0)))
  (if (Variables|/Game/Misoten/BP/BP_PractiseDrift_Pawn.BP_PractiseDrift_Pawn_C|GetIsGround _asbp_practise_drift_pawn)
    (Default|CallSpeedUp _asbp_practise_drift_player_con (Variables|Default|GetBegineSpeedUpValue))
    (Audio|PlaySoundatLocation "/Game/Misoten/BP/Audio/SE/Player/MS_NomalBoost_Cue.MS_NomalBoost_Cue" (Transformation|GetActorLocation (Game|GetPlayerCharacter 0)) "0, 0, 0" 0.4 1.0 0.0 0 0 0 0)
    (Game|Feedback|ClientPlayForceFeedback _asbp_practise_drift_player_con "/Game/Misoten/BP/FFE/FFE_PlayerPhase3.FFE_PlayerPhase3" "None" false false false)))

(event EventBeginPlay)

(event Collision|EventActorBeginOverlap
  (params (OtherActor :type Actor%20Object%20Reference)))

(event EventTick
  (params (DeltaSeconds :type Float%20%28single-precision%29)))

(fn ConstructionScript
  (bind _returnvalue (Utilities|GetDataTableRow "/Game/Misoten/BP/DataTable/GimmickStatusDataTable.GimmickStatusDataTable" "SpeedUpStand")
    (:then
      (Variables|Default|SetBegineSpeedUpValue (.BeginSpeedUpValue (Utilities|Struct|BreakGimmickStatusStruct _returnvalue)))
      (Variables|Default|SetEndSpeedUpValue (.EndSpeedUpValue (Utilities|Struct|BreakGimmickStatusStruct _returnvalue))))))