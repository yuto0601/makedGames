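; BP_MoveSupportSpline is a spline actor with a trigger box that supplies a movement-assist path to the player and the chasing boss.
; The construction script builds a collision-free spline mesh along each segment, matching local point locations and tangents.
; When BP_PractiseDrift_Pawn enters the box, the spline is passed to player controller 0 via SetMoveSupportSpline.
; Otherwise, an entering BP_BOSSChase receives it through StartMoveSupportSpline.
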(event OnComponentBeginOverlap(Box)
  (params (OverlappedComponent :type Primitive%20Component%20Object%20Reference) (OtherActor :type Actor%20Object%20Reference) (OtherComp :type Primitive%20Component%20Object%20Reference) (OtherBodyIndex :type Integer) (bFromSweep :type Boolean) (SweepResult :type Hit%20Result%20Structure%20%28by%20ref%29))
  (Utilities|Casting|CastToBP_PractiseDrift_Pawn OtherActor
    (:then
      (bind _asbp_practise_drift_player_con (Utilities|Casting|CastToBP_PractiseDrift_PlayerCon (Game|GetPlayerController 0)))
      (Default|SetMoveSupportSpline _asbp_practise_drift_player_con (Variables|Default|GetSpline)))
    (:CastFailed
      (bind _asbp_bosschase (Utilities|Casting|CastToBP_BOSSChase OtherActor))
      (Default|StartMoveSupportSpline _asbp_bosschase (Variables|Default|GetSpline)))))

(event EventBeginPlay)

(event Collision|EventActorBeginOverlap
  (params (OtherActor :type Actor%20Object%20Reference)))

(event EventTick
  (params (DeltaSeconds :type Float%20%28single-precision%29)))

(fn ConstructionScript
  (bind _spline (Variables|Default|GetSpline))
  (for _index (range 0 (- (Class|SplineComponent|GetNumberOfSplineSegments (Variables|Default|GetSpline)) 1))
    (bind _returnvalue (AddComponent|AddSplineMeshComponent false))
    (SplineMesh|SetStartandEnd _returnvalue (.Location (Spline|GetLocationandTangentatSplinePoint _spline _index "Local")) (.Tangent (Spline|GetLocationandTangentatSplinePoint _spline _index "Local")) (.Location (Spline|GetLocationandTangentatSplinePoint _spline (+ _index 1) "Local")) (.Tangent (Spline|GetLocationandTangentatSplinePoint _spline (+ _index 1) "Local")) true :!class /Script/Engine.SplineMeshComponent)
    (Collision|SetCollisionEnabled _returnvalue "NoCollision")))