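; BP_DriftLeftCamera is a camera actor for the left-drift view of the practise drift pawn.
; On BeginPlay it caches player 0's BP_PractiseDrift_Pawn, then each Tick snaps its transform to that pawn's DriftLeftCameraPos component.
; Two custom events switch its SpeedLine2 effect on and off.
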(event Custom|InactiveSpeedLine
  (Components|Activation|SetActive (Variables|Default|GetSpeedLine2) false false))

(event Custom|ActiveSpeedLine
  (Components|Activation|SetActive (Variables|Default|GetSpeedLine2) true false))

(event EventBeginPlay
  (bind _asbp_practise_drift_pawn (Utilities|Casting|CastToBP_PractiseDrift_Pawn (Game|Player|GetPlayerPawn 0)))
  (Variables|Default|SetAs%20BP%20Practise%20Drift%20Pawn _asbp_practise_drift_pawn))

(event EventTick
  (params (DeltaSeconds :type Float%20%28single-precision%29))
  (Transformation|SetActorTransform (Transformation|GetWorldTransform (Variables|/Game/Misoten/BP/BP_PractiseDrift_Pawn.BP_PractiseDrift_Pawn_C|GetDriftLeftCameraPos (Variables|Default|GetAs%20BP%20Practise%20Drift%20Pawn)))))

(fn ConstructionScript)