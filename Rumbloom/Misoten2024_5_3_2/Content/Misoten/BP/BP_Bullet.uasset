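; Bullet actor that the drift-driving player smashes away on contact, with hit stop and toon effects.
; Launch direction follows camera rotation and drift or wheelie state; player speed, clamped, sets its velocity.
; Swept Tick movement mirrors it off BP_Floor, multiplying speed for limited bounces and re-arming the smash; other bullets deflect it.
; EncloseJudge destroys it when summed signed angles to spline points show the spline encircles it.
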(event OnComponentBeginOverlap(Sphere)
  (params (OverlappedComponent :type Primitive%20Component%20Object%20Reference) (OtherActor :type Actor%20Object%20Reference) (OtherComp :type Primitive%20Component%20Object%20Reference) (OtherBodyIndex :type Integer) (bFromSweep :type Boolean) (SweepResult :type Hit%20Result%20Structure%20%28by%20ref%29))
  (bind _returnvalue (Game|GetPlayerCameraManager 0))
  (bind _as_bp_practise_drift_pawn (Variables|Default|GetAs%20BP%20Practise%20Drift%20Pawn))
  (bind _as_bp_practise_drift_player_con (Variables|Default|GetAs%20BP%20Practise%20Drift%20Player%20Con))
  (bind _returnvalue_2 (Transformation|GetActorRotation _returnvalue))
  (bind _returnvalue_3 (Transformation|GetActorForwardVector _returnvalue))
  (bind _returnvalue_4 (Transformation|GetActorRightVector _returnvalue))
  (bind _nowspeed (Variables|/Game/Misoten/BP/BP_PractiseDrift_PlayerCon.BP_PractiseDrift_PlayerCon_C|GetNowSpeed _as_bp_practise_drift_player_con))
  (bind _returnvalue_5 (Math|Rotator|FindLookatRotation _returnvalue_3 _returnvalue_4))
  (bind _returnvalue_6 (+ (.pitch _returnvalue_2) 3e+01))
  (bind _returnvalue_7 (Math|Rotator|MakeRotator (.roll _returnvalue_2) _returnvalue_6 (.yaw _returnvalue_2)))
  (bind _asbp_practise_drift_pawn (Utilities|Casting|CastToBP_PractiseDrift_Pawn OtherActor)
    (:then
      (bind _actor (Default|GetLockonTarget _asbp_practise_drift_pawn))
      (if (== _actor self)
        (Default|LockonRelease _asbp_practise_drift_pawn))
      (Utilities|FlowControl|DoOnce false
        (:Completed
          (bind _returnvalue_8 (Niagara|SpawnSystematLocation "/Game/Misoten/Assets/EFF/Toon_Hit/NS_ToonHit.NS_ToonHit" (Transformation|GetWorldLocation (Variables|Default|GetStaticMesh))))
          (Rendering|SetRenderCustomDepth _returnvalue_8 true)
          (if (Variables|/Game/Misoten/BP/BP_PractiseDrift_Pawn.BP_PractiseDrift_Pawn_C|GetIsDriftRight _as_bp_practise_drift_pawn)
            (Default|CallSmashBullet (Math|Rotator|CombineRotators _returnvalue_7 _returnvalue_5) _nowspeed)
            (elif (Variables|/Game/Misoten/BP/BP_PractiseDrift_Pawn.BP_PractiseDrift_Pawn_C|GetIsDriftLeft _as_bp_practise_drift_pawn)
              (Default|CallSmashBullet (Math|Rotator|CombineRotators (* _returnvalue_7 -1.0) _returnvalue_5) _nowspeed)
              (elif (Variables|/Game/Misoten/BP/BP_PractiseDrift_PlayerCon.BP_PractiseDrift_PlayerCon_C|GetIsWiley (Variables|Default|GetAs%20BP%20Practise%20Drift%20Player%20Con))
                (Default|CallSmashBullet (Math|Rotator|CombineRotators _returnvalue_7 (Math|Rotator|FindLookatRotation _returnvalue_3 (Transformation|GetActorUpVector _returnvalue))) _nowspeed)
                (else
                  (Default|CallSmashBullet _returnvalue_7 _nowspeed)))))
          (Utilities|HitStop 0.2 0.3))))
    (:CastFailed
      (bind _asbp_bullet (Utilities|Casting|CastToBP_Bullet OtherActor))
      (CallFunction|Reflection _asbp_bullet))))

(event Custom|LookatTarget
  (params (TargetActor :type Actor%20Object%20Reference))
  (Transformation|SetWorldRotation (Variables|Default|GetStaticMesh) (Math|Rotator|FindLookatRotation (Transformation|GetActorLocation) (Transformation|GetActorLocation TargetActor)) false false))

(event Custom|SmashBulletEvent
  (params (Rotator :type Rotator) (SmashSpeed :type Float%20%28double-precision%29))
  (bind _maxspeed (Variables|Default|GetMaxSpeed))
  (bind _minspeed (Variables|Default|GetMinSpeed))
  (if (>= SmashSpeed _maxspeed)
    (Variables|Default|SetNowSpeed _maxspeed)
    (elif (<= SmashSpeed _minspeed)
      (Variables|Default|SetNowSpeed _minspeed)
      (else
        (Variables|Default|SetNowSpeed SmashSpeed)))))

(event Custom|Reflection
  (params (TargetActor :type Actor%20Object%20Reference))
  (Transformation|SetWorldRotation (Variables|Default|GetStaticMesh) (* (Math|Rotator|FindLookatRotation (Transformation|GetActorLocation) (Transformation|GetActorLocation TargetActor)) -1.0) false false))

(event Custom|LookatVector
  (params (Rotator :type Rotator) (SmashSpeed :type Float%20%28double-precision%29))
  (Transformation|SetWorldRotation (Variables|Default|GetStaticMesh) Rotator false false))

(event Custom|EncloseJudge
  (params (SplineObject :type Spline%20Component%20Object%20Reference))
  (bind _resultout (CallFunction|InternalandExternalJudgments SplineObject))
  (if (>= _resultout (* (Math|Trig|GetPI) 2.0))
    (CallFunction|EncloseEvent)))

(event Custom|EncloseEvent
  (Actor|DestroyActor))

(event Custom|HitFloor_Event
  (bind _returnvalue (Game|GetPlayerCameraManager 0))
  (bind _as_bp_practise_drift_pawn (Variables|Default|GetAs%20BP%20Practise%20Drift%20Pawn))
  (bind _as_bp_practise_drift_player_con (Variables|Default|GetAs%20BP%20Practise%20Drift%20Player%20Con))
  (bind _returnvalue_2 (Transformation|GetActorRotation _returnvalue))
  (bind _returnvalue_3 (Transformation|GetActorForwardVector _returnvalue))
  (bind _returnvalue_4 (Transformation|GetActorRightVector _returnvalue))
  (bind _nowspeed (Variables|/Game/Misoten/BP/BP_PractiseDrift_PlayerCon.BP_PractiseDrift_PlayerCon_C|GetNowSpeed _as_bp_practise_drift_player_con))
  (bind _returnvalue_5 (Math|Rotator|FindLookatRotation _returnvalue_3 _returnvalue_4))
  (bind _returnvalue_6 (+ (.pitch _returnvalue_2) 3e+01))
  (bind _returnvalue_7 (Math|Rotator|MakeRotator (.roll _returnvalue_2) _returnvalue_6 (.yaw _returnvalue_2)))
  (Utilities|FlowControl|DoOnce false) ; enters at Reset
)

(event EventBeginPlay
  (EventDispatchers|BindEventtoSmashBullet (delegate Custom|SmashBulletEvent))
  (EventDispatchers|BindEventtoSmashBullet (delegate Custom|LookatVector))
  (bind _asbp_practise_drift_pawn (Utilities|Casting|CastToBP_PractiseDrift_Pawn (Game|Player|GetPlayerPawn 0)))
  (Variables|Default|SetAs%20BP%20Practise%20Drift%20Pawn _asbp_practise_drift_pawn)
  (bind _asbp_practise_drift_player_con (Utilities|Casting|CastToBP_PractiseDrift_PlayerCon (Game|GetPlayerController 0)))
  (Variables|Default|SetAs%20BP%20Practise%20Drift%20Player%20Con _asbp_practise_drift_player_con)
  (EventDispatchers|BindEventtoHitFloor (delegate Custom|HitFloor_Event)))

(event EventTick
  (params (DeltaSeconds :type Float%20%28single-precision%29))
  (Utilities|FlowControl|Sequence
    (:then_0
      (bind _sweephitresult (Transformation|AddActorWorldOffset (* (Transformation|GetActorForwardVector) (Variables|Default|GetNowSpeed)) true))
      (bind _asbp_floor (Utilities|Casting|CastToBP_Floor (.HitActor (Collision|BreakHitResult _sweephitresult)))
        (:then
          (Transformation|SetWorldRotation (Variables|Default|GetStaticMesh) (Math|Conversions|RotationFromXVector (Math|Vector|MirrorVectorbyNormal (Transformation|GetActorForwardVector) (Math|Vector|GetForwardVector (Variables|/Game/Misoten/BP/BP_Floor.BP_Floor_C|GetArrow _asbp_floor)))) false false)
          (Transformation|AddActorWorldOffset (* (Transformation|GetActorForwardVector) (Variables|Default|GetNowSpeed)))
          (Default|CallHitFloor)
          (Niagara|SpawnSystematLocation "/Game/Misoten/Assets/EFF/Toon_Shockwave/NS_ToonShockwave.NS_ToonShockwave" (Transformation|GetWorldLocation (Variables|Default|GetStaticMesh)) (Transformation|GetActorRotation _asbp_floor) "3.000000,3.000000,3.000000")
          (if (not (>= (Variables|Default|GetHitFloorNum) (Variables|Default|GetMaxHitFloorNum)))
            (bind _output_get (Variables|Default|SetHitFloorNum (+ (Variables|Default|GetHitFloorNum) 1)))
            (Variables|Default|SetNowSpeed (* _output_get (Variables|Default|GetNowSpeed)))))
        (:CastFailed
          (if (.bBlockingHit (Collision|BreakHitResult _sweephitresult))
            (Transformation|AddActorWorldOffset (* (Transformation|GetActorForwardVector) (Variables|Default|GetNowSpeed)))))))))

(fn ConstructionScript)

(fn GetIsMove
  (if (Math|Float|NearlyEqual(Float) (Variables|Default|GetNowSpeed) 0.0 1e-06)
    (return false)
    (else
      (return true))))

(fn InternalandExternalJudgments
  (params (Spline :type Spline%20Component%20Object%20Reference))
  (bind _returnvalue (Transformation|GetActorLocation))
  (LocalVariables|SetSplineObject Spline)
  (LocalVariables|Setresult 0.0)
  (for _index (range 0 (- (Class|SplineComponent|GetNumberOfSplineSegments (LocalVariables|GetSplineObject)) 2))
    (if (< (Math|Vector|DotProduct (Math|Vector|CrossProduct (- (.Location (Spline|GetLocationandTangentatSplinePoint (LocalVariables|GetSplineObject) _index "World")) _returnvalue) (- (.Location (Spline|GetLocationandTangentatSplinePoint (LocalVariables|GetSplineObject) (+ _index 1) "World")) _returnvalue)) (Math|Vector|MakeVector 0.0 0.0 1.0)) 0.0)
      (LocalVariables|Setresult (+ (Math|Trig|Acos(Degrees) (/ (Math|Vector|DotProduct (- (.Location (Spline|GetLocationandTangentatSplinePoint (LocalVariables|GetSplineObject) _index "World")) _returnvalue) (- (.Location (Spline|GetLocationandTangentatSplinePoint (LocalVariables|GetSplineObject) (+ _index 1) "World")) _returnvalue)) (* (Math|Vector|VectorLength (- (.Location (Spline|GetLocationandTangentatSplinePoint (LocalVariables|GetSplineObject) _index "World")) _returnvalue)) (Math|Vector|VectorLength (- (.Location (Spline|GetLocationandTangentatSplinePoint (LocalVariables|GetSplineObject) (+ _index 1) "World")) _returnvalue))))) (LocalVariables|Getresult)))
      (else
        (LocalVariables|Setresult (+ (* (Math|Trig|Acos(Degrees) (/ (Math|Vector|DotProduct (- (.Location (Spline|GetLocationandTangentatSplinePoint (LocalVariables|GetSplineObject) _index "World")) _returnvalue) (- (.Location (Spline|GetLocationandTangentatSplinePoint (LocalVariables|GetSplineObject) (+ _index 1) "World")) _returnvalue)) (* (Math|Vector|VectorLength (- (.Location (Spline|GetLocationandTangentatSplinePoint (LocalVariables|GetSplineObject) _index "World")) _returnvalue)) (Math|Vector|VectorLength (- (.Location (Spline|GetLocationandTangentatSplinePoint (LocalVariables|GetSplineObject) (+ _index 1) "World")) _returnvalue))))) -1.0) (LocalVariables|Getresult))))))
  (return (LocalVariables|Getresult)))