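; Player state Blueprint that keeps the player's score in the drift game.
; One function per scoring reason, such as props, tricks, acceleration, encloses or reflection, adds that reason's preset points and sends the amount and name to the main UI widget, cached from BP_PractiseDrift_PlayerCon on BeginPlay.
; Trick scores are flagged as non-combo, while clear-time bonuses come from a rank-indexed list and skip the popup; the score can also be reset and read.
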(event EventBeginPlay
  (Variables|Default|SetEncloseAttackValue 5.0)
  (bind _asbp_practise_drift_player_con (Utilities|Casting|CastToBP_PractiseDrift_PlayerCon (Game|GetPlayerController 0)))
  (Variables|Default|SetMain%20UI%20Widget (Variables|/Game/Misoten/BP/BP_PractiseDrift_PlayerCon.BP_PractiseDrift_PlayerCon_C|GetMain%20UI%20Widget _asbp_practise_drift_player_con)))

(event EventTick
  (params (DeltaSeconds :type Float%20%28single-precision%29)))

(fn AddScoreDrum
  (bind _drumscore (Variables|Default|GetDrumScore))
  (Variables|Default|SetScore (+ (Variables|Default|GetScore) (.score _drumscore)))
  (Default|ScoreUpInput (Variables|Default|GetMain%20UI%20Widget) (.score _drumscore) (.name _drumscore) 0 false))

(fn AddScoreCardboard
  (bind _cardboardscore (Variables|Default|GetCardboardScore))
  (Variables|Default|SetScore (+ (Variables|Default|GetScore) (.score _cardboardscore)))
  (Default|ScoreUpInput (Variables|Default|GetMain%20UI%20Widget) (.score _cardboardscore) (.name _cardboardscore) 0 false))

(fn AddScoreSpray
  (bind _sprayscore (Variables|Default|GetSprayScore))
  (Variables|Default|SetScore (+ (Variables|Default|GetScore) (.score _sprayscore)))
  (Default|ScoreUpInput (Variables|Default|GetMain%20UI%20Widget) (.score _sprayscore) (.name _sprayscore) 0 false))

(fn AddScoreTrick
  (bind _trickscore (Variables|Default|GetTrickScore))
  (Variables|Default|SetScore (+ (Variables|Default|GetScore) (.score _trickscore)))
  (Default|ScoreUpInput (Variables|Default|GetMain%20UI%20Widget) (.score _trickscore) (.name _trickscore) 0 true))

(fn AddScoreAcceleration
  (bind _accelerationscore (Variables|Default|GetAccelerationScore))
  (Variables|Default|SetScore (+ (Variables|Default|GetScore) (.score _accelerationscore)))
  (Default|ScoreUpInput (Variables|Default|GetMain%20UI%20Widget) (.score _accelerationscore) (.name _accelerationscore) 0 false))

(fn AddScoreEnclose
  (bind _enclosescore (Variables|Default|GetEncloseScore))
  (Variables|Default|SetScore (+ (Variables|Default|GetScore) (.score _enclosescore)))
  (Default|ScoreUpInput (Variables|Default|GetMain%20UI%20Widget) (.score _enclosescore) (.name _enclosescore) 0 false))

(fn AddScoreCharge
  (bind _chargescore (Variables|Default|GetChargeScore))
  (Variables|Default|SetScore (+ (Variables|Default|GetScore) (.score _chargescore)))
  (Default|ScoreUpInput (Variables|Default|GetMain%20UI%20Widget) (.score _chargescore) (.name _chargescore) 0 false))

(fn AddScoreClearTime
  (params (ClierRank :type Integer))
  (Variables|Default|SetScore (+ (Utilities|Array|Get(acopy) (Variables|Default|GetClearTimeScoreList) ClierRank) (Variables|Default|GetScore))))

(fn ResetScore
  (Variables|Default|SetScore 0))

(fn GetScore
  (return (Variables|Default|GetScore)))

(fn AddScoreReflection
  (bind _reflection_score (Variables|Default|GetReflection_Score))
  (Variables|Default|SetScore (+ (Variables|Default|GetScore) (.score _reflection_score)))
  (Default|ScoreUpInput (Variables|Default|GetMain%20UI%20Widget) (.score _reflection_score) (.name _reflection_score) 0 false))

(fn AddScoreBOSSEnclose
  (bind _bossenclose_score (Variables|Default|GetBossEnclose_Score))
  (Variables|Default|SetScore (+ (Variables|Default|GetScore) (.score _bossenclose_score)))
  (Default|ScoreUpInput (Variables|Default|GetMain%20UI%20Widget) (.score _bossenclose_score) (.name _bossenclose_score) 0 false))