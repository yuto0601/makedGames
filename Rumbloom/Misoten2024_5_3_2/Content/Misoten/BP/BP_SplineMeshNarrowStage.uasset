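; Spline-driven stage builder that lays out a narrow course with a raised piece along each side, judging by its name and layout.
; The construction script adds three collision-enabled spline meshes per segment: one on the spline and two side pieces scaled taller in Z.
; Side pieces are offset by normalized tangents rotated 90 degrees either way, at slightly unequal distances, and reuse the center tangents.
; The event graph has no runtime logic.
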(event EventBeginPlay)

(event Collision|EventActorBeginOverlap
  (params (OtherActor :type Actor%20Object%20Reference)))

(event EventTick
  (params (DeltaSeconds :type Float%20%28single-precision%29)))

(fn ConstructionScript
  (bind _spline (Variables|Default|GetSpline))
  (for _index (range 0 (- (Class|SplineComponent|GetNumberOfSplineSegments _spline) 1))
    (bind _returnvalue (AddComponent|AddSplineMeshComponent false))
    (SplineMesh|SetStartandEnd _returnvalue (.Location (Spline|GetLocationandTangentatSplinePoint _spline _index "Local")) (.Tangent (Spline|GetLocationandTangentatSplinePoint _spline _index "Local")) (.Location (Spline|GetLocationandTangentatSplinePoint _spline (+ _index 1) "Local")) (.Tangent (Spline|GetLocationandTangentatSplinePoint _spline (+ _index 1) "Local")) true :!class /Script/Engine.SplineMeshComponent)
    (Collision|SetCollisionEnabled _returnvalue "QueryAndPhysics")
    (bind _returnvalue_2 (AddComponent|AddSplineMeshComponent false (Math|Transform|MakeTransform "0, 0, 0" "0, 0, 0" "1,1,3.000000")))
    (SplineMesh|SetStartandEnd _returnvalue_2 (+ (* (Math|Vector|RotateVector (Math|Vector|Normalize (.Tangent (Spline|GetLocationandTangentatSplinePoint _spline _index "Local"))) "0,90.000000, 0") 9.5e+02) (.Location (Spline|GetLocationandTangentatSplinePoint _spline _index "Local"))) (.Tangent (Spline|GetLocationandTangentatSplinePoint _spline _index "Local")) (+ (* (Math|Vector|RotateVector (Math|Vector|Normalize (.Tangent (Spline|GetLocationandTangentatSplinePoint _spline (+ _index 1) "Local"))) "0,90.000000, 0") 9.5e+02) (.Location (Spline|GetLocationandTangentatSplinePoint _spline (+ _index 1) "Local"))) (.Tangent (Spline|GetLocationandTangentatSplinePoint _spline (+ _index 1) "Local")) true :!class /Script/Engine.SplineMeshComponent)
    (Collision|SetCollisionEnabled _returnvalue_2 "QueryAndPhysics")
    (bind _returnvalue_3 (AddComponent|AddSplineMeshComponent false (Math|Transform|MakeTransform "0, 0, 0" "0, 0, 0" "1,1,3.000000")))
    (SplineMesh|SetStartandEnd _returnvalue_3 (+ (* (Math|Vector|RotateVector (Math|Vector|Normalize (.Tangent (Spline|GetLocationandTangentatSplinePoint _spline _index "Local"))) "0,-90.000000, 0") 9e+02) (.Location (Spline|GetLocationandTangentatSplinePoint _spline _index "Local"))) (.Tangent (Spline|GetLocationandTangentatSplinePoint _spline _index "Local")) (+ (* (Math|Vector|RotateVector (Math|Vector|Normalize (.Tangent (Spline|GetLocationandTangentatSplinePoint _spline (+ _index 1) "Local"))) "0,-90.000000, 0") 9e+02) (.Location (Spline|GetLocationandTangentatSplinePoint _spline (+ _index 1) "Local"))) (.Tangent (Spline|GetLocationandTangentatSplinePoint _spline (+ _index 1) "Local")) true :!class /Script/Engine.SplineMeshComponent)
    (Collision|SetCollisionEnabled _returnvalue_3 "QueryAndPhysics")))