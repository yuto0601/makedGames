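; Blueprint that saves and loads the game's score through an SD_ScoreSave slot; a note says it has all been ported to the Game Instance.
; BeginPlay runs Dataload, which caches and returns the stored score or creates a blank save if none exists.
; SaveName is copied from SaveFile only after that load.
; DataSave writes the given score into a fresh save object, overwriting the slot.
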(event EventBeginPlay
  ;[1 1 1] ゲームインスタンスにすべて移植済み
  (CallFunction|Dataload)
  (Variables|Default|SetSaveName (Variables|/Game/Misoten/BP/SaveData/SD_ScoreSave.SD_ScoreSave_C|GetSaveName (Variables|Default|GetSaveFile))))

(event EventTick
  (params (DeltaSeconds :type Float%20%28single-precision%29)))

(fn DataSave
  (params (SaveScore :type Array%20of%20Integers))
  (bind _returnvalue (SaveGame|CreateSaveGameObject "/Game/Misoten/BP/SaveData/SD_ScoreSave.SD_ScoreSave_C"))
  (Variables|/Game/Misoten/BP/SaveData/SD_ScoreSave.SD_ScoreSave_C|SetScore _returnvalue SaveScore)
  (SaveGame|SaveGametoSlot _returnvalue (Variables|Default|GetSaveName) (Variables|/Game/Misoten/BP/SaveData/SD_ScoreSave.SD_ScoreSave_C|GetUserIndex _returnvalue)))

(fn Dataload
  ;[1 1 1] データが残っているか
  (bind _returnvalue (SaveGame|DoesSaveGameExist (Variables|Default|GetSaveName)))
  (if _returnvalue
    ;[1 1 1] データをロードし格納
    (bind _returnvalue_2 (SaveGame|LoadGamefromSlot (Variables|Default|GetSaveName)))
    (bind _assd_score_save (Utilities|Casting|CastToSD_ScoreSave _returnvalue_2))
    (bind _output_get (Variables|Default|SetSaveFile _assd_score_save))
    ;[1 1 1] スコアデータを出力
    (return (Variables|/Game/Misoten/BP/SaveData/SD_ScoreSave.SD_ScoreSave_C|GetScore _output_get))
    (else
      (CallFunction|DataCreate&init) ; データの新規作成
    )))

(fn DataCreate&init
  (bind _returnvalue (SaveGame|CreateSaveGameObject "/Game/Misoten/BP/SaveData/SD_ScoreSave.SD_ScoreSave_C"))
  (SaveGame|SaveGametoSlot _returnvalue (Variables|Default|GetSaveName) (Variables|/Game/Misoten/BP/SaveData/SD_ScoreSave.SD_ScoreSave_C|GetUserIndex _returnvalue)))